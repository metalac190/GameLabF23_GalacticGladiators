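; BP_IceHazard is an ice hazard that leaves a BP_IcePatch where it impacts.
; It derives from a parent hazard class, and its SetSpeedAndSize override forwards the size but always passes zero speed to the parent.
; Its Impact function spawns the patch at the actor's location with zero rotation, scaled by HazardSize, without calling a parent implementation.
; The event graph holds only disabled default events.
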(event EventBeginPlay
  (|CallParentFunction) ; This node is disabled and will not be called.\nDrag off pins to build functionality.
)

(event Collision|EventActorBeginOverlap
  (params (OtherActor :type Actor%20Object%20Reference))
  (|CallParentFunction OtherActor) ; This node is disabled and will not be called.\nDrag off pins to build functionality.
)

(event EventTick
  (params (DeltaSeconds :type Float%20%28single-precision%29))
  (|CallParentFunction DeltaSeconds) ; This node is disabled and will not be called.\nDrag off pins to build functionality.
)

(fn ConstructionScript
  (|CallParentFunction))

(fn SetSpeedandSize
  (params (speed :type Float%20%28double-precision%29) (size :type Float%20%28double-precision%29))
  (|CallParentFunction 0.0 size))

(fn Impact
  (Game|SpawnActorfromClass "/Game/GameMode1/Programming/BP_IcePatch.BP_IcePatch_C" (Math|Transform|MakeTransform (Transformation|GetActorLocation) "0, 0, 0" (Math|Conversions|ToVector(Float) (Variables|Default|GetHazard%20Size))) "Undefined" "MultiplyWithRoot" 0 0))