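; GM_GM1 is the game mode for a local multiplayer arena match with a crown, player scores and a time limit.
; Setup creates local players and has each possess an input receiver at a start point, sharing one camera; SpawnPlayer later swaps in real pawns.
; StartGame requires minimum players, then creates the crown HUD, binds scoring and starts the end timer.
; It also configures a selected or random stage hazard: meteors, bumpers or shrinking ice.
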(event EventBeginPlay
  (CallFunction|DoSetupGame))

(event EventHandleStartingNewPlayer
  (params (NewPlayer :type Player%20Controller%20Object%20Reference))
  ;[1 1 1] Possible Work Around
  (|CallParentFunction NewPlayer)
  (Input|AddMappingContext (PlayerController|LocalPlayerSubsystems|GetEnhancedInputLocalPlayerSubsystem NewPlayer) "/Game/GameMode1/Programming/Player/Input/IMC_GM1.IMC_GM1" 0 "(bIgnoreAllPressedKeysUntilRelease=True,bForceImmediately=False)"))

(event EventOnRestartPlayer
  (params (NewPlayer :type Controller%20Object%20Reference))
  (|CallParentFunction NewPlayer))

(fn ConstructionScript)

(fn GetPlayerStartPoints
  (bind _outactors (Actor|GetAllActorsOfClass "/Game/GameMode1/Programming/Systems/BP_GM1_PlayerStart.BP_GM1_PlayerStart_C"))
  (Variables|Player|SetPlayerStarts _outactors))

(fn SpawnInputRecievers
  (for (_ _array_index) (Variables|Player|GetPlayerStarts)
    (bind _output_get (LocalVariables|SetIndex _array_index))
    (Utilities|IsValid (Game|GetPlayerController _output_get)
      (:Is%20Valid
        (Utilities|IsValid (PlayerController|LocalPlayerSubsystems|GetEnhancedInputLocalPlayerSubsystem (Game|GetPlayerController (LocalVariables|GetIndex)))
          (:Is%20Valid
            ;[0 0 0 0.5] Assign IMCs
            (Input|AddMappingContext (PlayerController|LocalPlayerSubsystems|GetEnhancedInputLocalPlayerSubsystem (Game|GetPlayerController (LocalVariables|GetIndex))) "/Game/GameMode1/Programming/Player/Input/IMC_GM1.IMC_GM1" 0 "(bIgnoreAllPressedKeysUntilRelease=True,bForceImmediately=False)"))))
      (:Is%20Not%20Valid
        ;[0 0 0 0.5] Setup Local Players
        (bind _returnvalue (Class|GameplayStatics|CreatePlayer (LocalVariables|GetIndex))) ; -1 Auto Increment doesn't work in UE5 :D
        (Utilities|IsValid (PlayerController|LocalPlayerSubsystems|GetEnhancedInputLocalPlayerSubsystem _returnvalue)
          (:Is%20Valid
            (Input|AddMappingContext (PlayerController|LocalPlayerSubsystems|GetEnhancedInputLocalPlayerSubsystem _returnvalue) "/Game/GameMode1/Programming/Player/Input/IMC_GM1.IMC_GM1" 0 "(bIgnoreAllPressedKeysUntilRelease=True,bForceImmediately=False)")))))
    ;[0 0 0 0.5] Spawn Input Recievers
    (bind _returnvalue_2 (Game|SpawnActorfromClass "/Game/GameMode1/Programming/Player/Blueprints/BP_InputReciever.BP_InputReciever_C" (Transformation|GetActorTransform (Utilities|Array|Get(acopy) (Variables|Player|GetPlayerStarts) (LocalVariables|GetIndex))) "Undefined" "MultiplyWithRoot" 0 (LocalVariables|GetIndex) 0))
    ;[0 0 0 0.5] Possess Pawn
    (Utilities|Array|AddUnique (Variables|Player|GetPlayerInputRecievers) _returnvalue_2)
    (Pawn|Possess (Class|GameplayStatics|GetPlayerControllerfromID (LocalVariables|GetIndex)) _returnvalue_2)
    (Utilities|Array|AddUnique (Variables|Player|GetPlayerControllers) (Class|GameplayStatics|GetPlayerControllerfromID (LocalVariables|GetIndex)))
    (Game|Player|SetViewTargetwithBlend (Game|GetPlayerController (LocalVariables|GetIndex)) (Variables|Camera|GetCameraRef) 0.0 "VTBlend_Linear" 0.0 false))
  (CallFunction|RemoveUnusedCameras))

(fn GameStarted
  (Variables|Player|SetisInGame true)
  (Default|GameStarted (Variables|Camera|GetCameraRef) (Variables|Player|GetPlayers))
  (bind _returnvalue (Actor|GetActorOfClass "/Game/GameMode1/Programming/BP_Crown.BP_Crown_C"))
  (bind _returnvalue_2 (UserInterface|CreateWidget "/Game/GameMode1/UI/WBP_GM1_CrownMode.WBP_GM1_CrownMode_C" 0 _returnvalue))
  (bind _output_get (Variables|Default|SetHUDWidget _returnvalue_2))
  (UserInterface|Viewport|AddtoViewport _output_get 0)
  (for _array_element (Variables|Player|GetPlayers)
    (EventDispatchers|BindEventtoOnAdjustPlayerScore _array_element (EventDispatchers|CreateEvent :!event AdjustPlayerScore)))
  (Utilities|Time|SetTimerbyFunctionName 0 "GameEnded" (Math|Conversions|ToFloat(Integer) (Variables|/Game/GameMode1/Programming/Gameplay/Data/PDA_Gameplay.PDA_Gameplay_C|GetgameDurationInSeconds (Variables|Default|GetGameplayData))))
  (Development|PrintString "GameStarted"))

(fn GameEnded
  (Variables|Player|SetisInGame false)
  (Default|CallOnEndGame)
  (Development|PrintString "GameEnded"))

(fn RemoveUnusedCameras
  (bind _outactors (Actor|GetAllActorsOfClass "/Script/Engine.CameraActor"))
  (for _array_element _outactors
    (Actor|DestroyActor _array_element)))

(fn DoSetupGame
  (bind _outactors (Actor|GetAllActorsOfClass "/Game/GameMode1/Programming/Camera/CM_GM1.CM_GM1_C"))
  (Variables|Camera|SetCameraRef (Utilities|Array|Get(acopy) _outactors))
  ;[0 0 0 0.5] Basic Start
  (CallFunction|GetPlayerStartPoints)
  (CallFunction|SpawnInputRecievers))

(fn ShouldReset
  (params (ActorToReset :type Actor%20Object%20Reference))
  (return false))

(fn GetActivePlayers
  (bind _players (Variables|Player|GetPlayers))
  (return _players (Utilities|Array|Length _players)))

(fn SelectStageHazard
  (bind _returnvalue (Math|Transform|MakeTransform "0.000000,0.000000,25.000000"))
  (bind _output_get (Variables|Default|SetCurrentStageHazard (Variables|/Game/GameMode1/Programming/Gameplay/Data/PDA_Gameplay.PDA_Gameplay_C|GetstageHazard (Variables|Default|GetGameplayData))))
  (switch Utilities|FlowControl|Switch|SwitchonE_StageHazardType _output_get :!label _label
    (:NewEnumerator1
      (Game|SpawnActorfromClass "/Game/Freelance/Programming/LevelHazards/BP_GM1_MeteorSpawner.BP_GM1_MeteorSpawner_C" _returnvalue "Undefined" "MultiplyWithRoot" 0 (Variables|StageHazardData|GetIceMeteorData) 0))
    (:NewEnumerator2
      (Game|SpawnActorfromClass "/Game/Freelance/Programming/LevelHazards/BP_GM1_MeteorSpawner.BP_GM1_MeteorSpawner_C" _returnvalue "Undefined" "MultiplyWithRoot" 0 (Variables|StageHazardData|GetKnockbackMeteorData) 0))
    (:NewEnumerator4
      (bind _outactors (Actor|GetAllActorsOfClass "/Game/GameMode1/Programming/Hazards/BP_Bumper1.BP_Bumper1_C"))
      (for _array_element _outactors
        (Actor|DestroyActor _array_element))
      (for _array_element_2 (Variables|/Game/GameMode1/Programming/Hazards/Data/PDA_BumperHazard.PDA_BumperHazard_C|GetBumperLocations (Variables|StageHazardData|GetBumperHazardData))
        (bind _returnvalue_2 (Game|SpawnActorfromClass "/Game/GameMode1/Programming/Hazards/BP_Bumper1.BP_Bumper1_C" (Math|Conversions|ToTransform(Vector) _array_element_2) "AlwaysSpawn" "MultiplyWithRoot" 0 0 0))
        (Default|RegisterasStageHazard _returnvalue_2)))
    (:NewEnumerator5
      (bind _returnvalue_3 (Actor|GetActorOfClass "/Game/GameMode1/Programming/Hazards/BP_Arena.BP_Arena_C"))
      (Default|RegisterasStageHazard _returnvalue_3))
    (:NewEnumerator3
      ;[0 0 0] If stage hazard is set to random, get a random stage hazard and then go back through the switch to finish any set up.
      (Variables|Default|SetCurrentStageHazard (Utilities|Select :Index (Math|Random|RandomIntegerinRange 0 3) :Option%200 "NewEnumerator1" :Option%201 "NewEnumerator2" :Option%202 "NewEnumerator4" :Option%203 "NewEnumerator5"))
      (goto _label))))

(fn StartStageHazard
  (Default|CallOnStageHazardStart))

(fn AdjustPlayerScore
  (params (player :type BP%20Player%20GM1%20Object%20Reference) (amount :type Integer))
  (Default|AdjustPlayerScore (Variables|Default|GetHUDWidget) (Variables|/Game/GameMode1/Programming/Player/Blueprints/BP_Player_GM1.BP_Player_GM1_C|GetIndex player) amount))

(fn FreePlayerCast
  (return 0))

(fn GetIsinGame
  (return (Variables|Player|GetisInGame)))

(fn RemovePlayer
  (params (PlayerToRemove :type BP%20Player%20GM1%20Object%20Reference))
  (Default|RemoveTrackedTarget (Variables|Camera|GetCameraRef) PlayerToRemove)
  (return false))

(fn ResetGame
  (bind _playerstarts (Variables|Player|GetPlayerStarts))
  (bind _playerinputrecievers (Variables|Player|GetPlayerInputRecievers))
  (bind _playercontrollers (Variables|Player|GetPlayerControllers))
  (bind _players (Variables|Player|GetPlayers))
  (bind _returnvalue (Utilities|Array|Length _playerinputrecievers))
  (bind _returnvalue_2 (Utilities|Array|Length _playerstarts))
  (bind _returnvalue_3 (Utilities|Array|Length _players))
  (bind _returnvalue_4 (Utilities|Array|Length _playercontrollers))
  (bind _result (Utilities|Text|FormatText "starts {s} 
players {p} 
inputs {i} 
controllers {c}" _returnvalue_2 _returnvalue_3 _returnvalue _returnvalue_4))
  (Utilities|FlowControl|DoOnce false
    (:Completed
      (Development|PrintText _result)
      (Class|GameMode|RestartGame)
      (CallFunction|DoSetupGame)
      (Development|PrintText _result)
      (return true))))

(fn SpawnPlayer
  (params (CurrentPlayerIndex :type Integer) (InputReciever :type BP%20Input%20Reciever%20Object%20Reference))
  ;[0 0 0 0.5] Spawn Player Pawn and Possess
  (bind _returnvalue (Game|SpawnActorfromClass "/Game/GameMode1/Programming/Player/Blueprints/BP_Player_GM1.BP_Player_GM1_C" (Transformation|GetActorTransform InputReciever) "Undefined" "MultiplyWithRoot" 0 CurrentPlayerIndex 0))
  (Utilities|Array|Add (Variables|Player|GetPlayers) _returnvalue)
  (Pawn|Possess (Game|GetPlayerController CurrentPlayerIndex) _returnvalue)
  (Game|Player|SetViewTargetwithBlend (Game|GetPlayerController CurrentPlayerIndex) (Variables|Camera|GetCameraRef) 0.0 "VTBlend_Linear" 0.0 false)
  (return false))

(fn StartGame
  (if (>= (Utilities|Array|Length (Variables|Player|GetPlayers)) (Variables|Player|GetMinPlayers))
    (CallFunction|GameStarted)
    (Default|CallOnStartGame)
    (return false)))