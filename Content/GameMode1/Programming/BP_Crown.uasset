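; BP_Crown is a floating crown pickup for GameMode1 that a player can take and carry above their head.
; On overlap while unowned, it asks an eligible BP_Player_GM1 to take it through GiveCrown; ClearControl releases the owner.
; Every tick it spins and sine-bobs its Cube, lerping toward a point above its owner or, when unowned, back to a default float height.
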(event EventBeginPlay)

(event Collision|EventActorBeginOverlap
  (params (OtherActor :type Actor%20Object%20Reference))
  (Utilities|IsValid (Variables|Default|GetControlling%20Player)
    (:Is%20Not%20Valid
      (bind _asbp_player_gm1 (Utilities|Casting|CastToBP_Player_GM1 OtherActor))
      (if (Variables|/Game/GameMode1/Programming/Player/Blueprints/BP_Player_GM1.BP_Player_GM1_C|GetbCanHaveCrown _asbp_player_gm1)
        (Default|GiveCrown _asbp_player_gm1 self)))))

(event EventTick
  (params (DeltaSeconds :type Float%20%28single-precision%29))
  (bind _returnvalue (Transformation|GetActorLocation))
  (bind _controlling_player (Variables|Default|GetControlling%20Player))
  (bind (_x _y) (Math|Vector|BreakVector _returnvalue))
  (CallFunction|BobandSpin)
  (Utilities|IsValid _controlling_player
    (:Is%20Valid
      (Transformation|SetActorLocation (Math|Vector|Lerp(Vector) (Transformation|GetActorLocation) (+ (Transformation|GetActorLocation _controlling_player) (Math|Vector|MakeVector 0.0 0.0 (Variables|Default|GetverticalOffset))) (Variables|Default|GetfollowLerpSpeed)) false false))
    (:Is%20Not%20Valid
      (Transformation|SetActorLocation (Math|Vector|Lerp(Vector) (Transformation|GetActorLocation) (Math|Vector|MakeVector _x _y (Variables|Default|GetdefaultFloatHeight)) (Variables|Default|GetfollowLerpSpeed)) false false))))

(fn ConstructionScript)

(fn BobandSpin
  (Transformation|SetWorldRotation (Variables|Default|GetCube) (Math|Rotator|CombineRotators (Transformation|GetWorldRotation (Variables|Default|GetCube)) (Math|Rotator|MakeRotator 0.0 0.0 (* (Utilities|Time|GetWorldDeltaSeconds) 135.0))) false false)
  (Transformation|AddWorldOffset (Variables|Default|GetCube) (Math|Vector|MakeVector 0.0 0.0 (Math|Trig|Sin(Degrees) (* (Utilities|Time|GetTimeSeconds) 9e+01))) false false))

(fn ClearControl
  (Variables|Default|SetControlling%20Player 0))