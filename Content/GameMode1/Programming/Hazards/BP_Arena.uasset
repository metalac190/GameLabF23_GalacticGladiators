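; GameMode1 arena that tilts and acts as an ice-ring stage hazard.
; On GM_GM1's hazard start, it flashes a glow overlay, then a timeline rescales the ground and dynamic ice-ring decal together.
; Tick drives either Programmed tilt (random targets or sine/cosine oscillation, continuous or timed intervals) or Dynamic tilt.
; Dynamic tilt sums overlapping players' offsets, clamps them to the arena radius and eases rotation by that combined position.
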(event Custom|RegisterAsStageHazard
  (EventDispatchers|BindEventtoOnStageHazardStart (.AsGM%20GM1 (Utilities|Casting|CastToGM_GM1 (Game|GetGameMode))) (delegate Custom|Start%20Ice%20Grow)))

(event Custom|Start%20Ice%20Grow
  (Rendering|Material|SetMaterial (Variables|Default|GetGroundCollision) 0 "/Game/GameMode1/Art/Materials/MI_OverlayGlow.MI_OverlayGlow")
  (Utilities|FlowControl|Delay 3.0)
  (Rendering|Material|SetMaterial (Variables|Default|GetGroundCollision) 0 "/Game/GameMode1/Art/LevelPrototyping/MI_Whitebox.MI_Whitebox")
  (bind _alpha (Timeline|Timeline PlayFromStart)
    (:Update
      (Transformation|SetRelativeScale3D (Variables|Default|GetGround) (Math|Vector|MakeVector (Math|Float|Lerp 1.0 (Variables|/Game/GameMode1/Programming/Hazards/Data/PDA_IceHazard.PDA_IceHazard_C|GetEndScale (Variables|Default|GetStageHazardData)) _alpha) (Math|Float|Lerp 1.0 (Variables|/Game/GameMode1/Programming/Hazards/Data/PDA_IceHazard.PDA_IceHazard_C|GetEndScale (Variables|Default|GetStageHazardData)) _alpha) (.Z (Math|Vector|BreakVector (Variables|/Script/Engine.SceneComponent|GetRelativeScale3D (Variables|Default|GetGround))))))
      (Rendering|Material|SetScalarParameterValue (Variables|Default|GetIceRingMaterial) "InnerRingSize" (Math|Float|Lerp 1.0 (Variables|/Game/GameMode1/Programming/Hazards/Data/PDA_IceHazard.PDA_IceHazard_C|GetEndScale (Variables|Default|GetStageHazardData)) _alpha) :!class /Script/Engine.MaterialInstanceDynamic))))

(event EventTick
  (params (DeltaSeconds :type Float%20%28single-precision%29))
  (if (Variables|Tilt|GetIsTilting)
    (switch Utilities|FlowControl|Switch|SwitchonE_ArenaTiltType (Variables|/Game/GameMode1/Programming/Hazards/Data/PDA_ArenaTilt.PDA_ArenaTilt_C|GetTiltType (Variables|Tilt|GetArenaTiltData))
      (:NewEnumerator0
        (CallFunction|ProgrammedTilt))
      (:NewEnumerator2
        (CallFunction|DynamicTilt)))))

(event EventBeginPlay
  (Rendering|Material|SetScalarParameterValue (Variables|Default|GetIceRingMaterial) "InnerRingSize" 1.0 :!class /Script/Engine.MaterialInstanceDynamic)
  (Components|DestroyComponent (Variables|Default|GetIndicator))
  (CallFunction|StartTilt))

(fn ConstructionScript
  (bind _stagehazarddata (Variables|Default|GetStageHazardData))
  (bind _returnvalue (Rendering|Material|CreateDynamicMaterialInstance "/Game/GameMode1/Art/Decals/GM1/MI_GM1_SurfaceDecal_IceRing.MI_GM1_SurfaceDecal_IceRing" "None" "None" :!class /Script/Engine.KismetMaterialLibrary))
  (Rendering|Components|Decal|SetDecalMaterial (Variables|Default|GetIceVisuals) _returnvalue)
  (bind _output_get (Variables|Default|SetIceRingMaterial _returnvalue))
  (Rendering|Material|SetScalarParameterValue _output_get "InnerRingSize" (Variables|/Game/GameMode1/Programming/Hazards/Data/PDA_IceHazard.PDA_IceHazard_C|GetEndScale _stagehazarddata) :!class /Script/Engine.MaterialInstanceDynamic)
  (Transformation|SetRelativeScale3D (Variables|Default|GetShrinkingGround) (Math|Conversions|ToVector(Float) (Variables|/Game/GameMode1/Programming/Hazards/Data/PDA_IceHazard.PDA_IceHazard_C|GetStartScale _stagehazarddata))))

(fn StartTilt
  (bind _arenatiltdata (Variables|Tilt|GetArenaTiltData))
  (Variables|Tilt|SetIsTilting true)
  (switch Utilities|FlowControl|Switch|SwitchonE_ArenaTiltType (Variables|/Game/GameMode1/Programming/Hazards/Data/PDA_ArenaTilt.PDA_ArenaTilt_C|GetTiltType (Variables|Tilt|GetArenaTiltData))
    (:NewEnumerator0
      (if (or (Variables|/Game/GameMode1/Programming/Hazards/Data/PDA_ArenaTilt.PDA_ArenaTilt_C|GetRandom%20Rotate _arenatiltdata) (not (Variables|/Game/GameMode1/Programming/Hazards/Data/PDA_ArenaTilt.PDA_ArenaTilt_C|GetContinuous%20Rotate _arenatiltdata)))
        (CallFunction|GenerateNewTargetRotation)))))

(fn ProgrammedTilt
  (bind _arenatiltdata (Variables|Tilt|GetArenaTiltData))
  (bind _rotatetime (Variables|ProgrammedTilt|GetRotateTime))
  (bind _arenatiltdata_2 (Variables|Tilt|GetArenaTiltData))
  (bind _arenatiltdata_3 (Variables|Tilt|GetArenaTiltData))
  (bind _maxtilt (Variables|/Game/GameMode1/Programming/Hazards/Data/PDA_ArenaTilt.PDA_ArenaTilt_C|GetMaxTilt _arenatiltdata_3))
  (bind _tiltspeed (Variables|/Game/GameMode1/Programming/Hazards/Data/PDA_ArenaTilt.PDA_ArenaTilt_C|GetTiltSpeed _arenatiltdata))
  (bind (_x _y _z) (Math|Vector|BreakVector _maxtilt))
  (bind _returnvalue (* _tiltspeed _rotatetime))
  (bind _returnvalue_2 (Math|Trig|Sin(Degrees) _returnvalue))
  (if (Utilities|InRotation)
    (if (Variables|/Game/GameMode1/Programming/Hazards/Data/PDA_ArenaTilt.PDA_ArenaTilt_C|GetRandom%20Rotate (Variables|Tilt|GetArenaTiltData))
      (Transformation|SetActorRotation (Class|KismetMathLibrary|RInterptoConstant (Transformation|GetActorRotation) (Variables|Tilt|GetTargetRotation) (Utilities|Time|GetWorldDeltaSeconds) (Variables|/Game/GameMode1/Programming/Hazards/Data/PDA_ArenaTilt.PDA_ArenaTilt_C|GetTiltSpeed (Variables|Tilt|GetArenaTiltData))))
      (if (Math|Boolean|ANDBoolean (Variables|/Game/GameMode1/Programming/Hazards/Data/PDA_ArenaTilt.PDA_ArenaTilt_C|GetContinuous%20Rotate _arenatiltdata_2) (Variables|/Game/GameMode1/Programming/Hazards/Data/PDA_ArenaTilt.PDA_ArenaTilt_C|GetRandom%20Rotate _arenatiltdata_2) (Utilities|Operators|EqualEqual (Transformation|GetActorRotation) (Variables|Tilt|GetTargetRotation) 0.05))
        (CallFunction|GenerateNewTargetRotation))
      (else
        (Utilities|PlusEqualsFloat (Variables|ProgrammedTilt|GetRotateTime) (Utilities|Time|GetWorldDeltaSeconds)
          (:%20%20
            (Transformation|SetActorRotation (Math|Rotator|MakeRotator (* _x _returnvalue_2) (* _y (Math|Trig|Cos(Degrees) _returnvalue)) (* _z _returnvalue_2)))))))))

(fn GenerateNewTargetRotation
  (bind _arenatiltdata (Variables|Tilt|GetArenaTiltData))
  (bind _arenatiltdata_2 (Variables|Tilt|GetArenaTiltData))
  (bind _rotateduration (Variables|/Game/GameMode1/Programming/Hazards/Data/PDA_ArenaTilt.PDA_ArenaTilt_C|GetRotateDuration _arenatiltdata_2))
  (if (Variables|/Game/GameMode1/Programming/Hazards/Data/PDA_ArenaTilt.PDA_ArenaTilt_C|GetRandom%20Rotate _arenatiltdata)
    (bind _tilt (Default|GetRandomTilt (Variables|Tilt|GetArenaTiltData)))
    (Variables|Tilt|SetTargetRotation _tilt))
  (if (not (Variables|/Game/GameMode1/Programming/Hazards/Data/PDA_ArenaTilt.PDA_ArenaTilt_C|GetContinuous%20Rotate _arenatiltdata))
    (Variables|ProgrammedTilt|SetIsInInterval true)
    (Utilities|Time|SetTimerbyFunctionName 0 "EndInterval" _rotateduration)
    (bind _random (Default|GetRandomInterval (Variables|Tilt|GetArenaTiltData)))
    (Utilities|Time|SetTimerbyFunctionName 0 "Generate New Target Rotation" (+ _random _rotateduration))))

(fn EndInterval
  (Variables|ProgrammedTilt|SetIsInInterval false))

(fn DynamicTilt
  (bind _x (Utilities|GetRadiusinUnits))
  (bind _scale (Utilities|GetScaleinUnits))
  (bind _arenatiltdata (Variables|Tilt|GetArenaTiltData))
  (bind _arenatiltdata_2 (Variables|Tilt|GetArenaTiltData))
  (bind (_x_2 _y) (Math|Vector|BreakVector _scale))
  (bind _maxtilt (Variables|/Game/GameMode1/Programming/Hazards/Data/PDA_ArenaTilt.PDA_ArenaTilt_C|GetMaxTilt _arenatiltdata))
  (bind (_x_3 _y_2) (Math|Vector|BreakVector _maxtilt))
  (LocalVariables|Setplayers (Collision|GetOverlappingActors (Variables|Default|GetPlayerCheck) "/Game/GameMode1/Programming/Player/Blueprints/BP_Player_GM1.BP_Player_GM1_C" :!class /Script/Engine.PrimitiveComponent))
  (Variables|DynamicTilt|SetcurrentTiltSpeed (Math|Interpolation|FInterpTo (Variables|DynamicTilt|GetcurrentTiltSpeed) (Math|Float|SelectFloat 0.0 (Variables|/Game/GameMode1/Programming/Hazards/Data/PDA_ArenaTilt.PDA_ArenaTilt_C|GetTiltSpeed _arenatiltdata_2) (Utilities|Operators|EqualEqual (Variables|Tilt|GetTargetRotation) (Transformation|GetActorRotation) 0.05)) (Utilities|Time|GetWorldDeltaSeconds) (Variables|/Game/GameMode1/Programming/Hazards/Data/PDA_ArenaTilt.PDA_ArenaTilt_C|GetTiltAcceleration _arenatiltdata_2)))
  (Transformation|SetActorRotation (Class|KismetMathLibrary|RInterptoConstant (Transformation|GetActorRotation) (Variables|Tilt|GetTargetRotation) (Utilities|Time|GetWorldDeltaSeconds) (Variables|DynamicTilt|GetcurrentTiltSpeed)))
  (Utilities|Array|Clear (LocalVariables|GetplayerDistances))
  (for _array_element (LocalVariables|Getplayers)
    (Utilities|Array|Add (LocalVariables|GetplayerDistances) (- (Transformation|GetActorLocation _array_element) (Transformation|GetActorLocation))))
  (LocalVariables|SetplayerDistanceSum "0, 0, 0")
  (for _array_element_2 (LocalVariables|GetplayerDistances)
    (LocalVariables|SetplayerDistanceSum (+ (LocalVariables|GetplayerDistanceSum) _array_element_2)))
  (LocalVariables|SetplayerDistanceSum (Math|Vector|SelectVector (* (Math|Vector|Normalize (LocalVariables|GetplayerDistanceSum)) _x) (LocalVariables|GetplayerDistanceSum) (> (Math|Vector|VectorLength (LocalVariables|GetplayerDistanceSum)) _x)))
  (Variables|DynamicTilt|SettiltDirection (Math|Interpolation|VInterpTo (Variables|DynamicTilt|GettiltDirection) (LocalVariables|GetplayerDistanceSum) (Utilities|Time|GetWorldDeltaSeconds) (Variables|/Game/GameMode1/Programming/Hazards/Data/PDA_ArenaTilt.PDA_ArenaTilt_C|GetTiltAcceleration (Variables|Tilt|GetArenaTiltData))))
  (Variables|Tilt|SetTargetRotation (Math|Rotator|MakeRotator (* (/ (.Y (Math|Vector|BreakVector (Variables|DynamicTilt|GettiltDirection))) _y) _y_2) (* (/ (.X (Math|Vector|BreakVector (Variables|DynamicTilt|GettiltDirection))) _x_2) _x_3 -1.0) 0.0)))