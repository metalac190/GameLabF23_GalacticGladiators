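; BP_Bumper is a GameMode1 bumper that bounces BP_Player_GM1 away when they hit it.
; On Hit, it reflects the player's velocity across the inverted hit normal and passes that direction to Bump.
; Bump normalizes the direction, scales it by BounceVelocity, launches the character with only X and Y overridden, and plays a 2D bumper sound.
; An author comment notes that Bump appears to fire twice per hit without apparent issues.
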(event EventBeginPlay)

(event Collision|EventActorBeginOverlap
  (params (OtherActor :type Actor%20Object%20Reference)))

(event EventTick
  (params (DeltaSeconds :type Float%20%28single-precision%29)))

(event Collision|EventHit
  (params (MyComp :type Primitive%20Component%20Object%20Reference) (Other :type Actor%20Object%20Reference) (OtherComp :type Primitive%20Component%20Object%20Reference) (bSelfMoved :type Boolean) (HitLocation :type Vector :default "0, 0, 0") (HitNormal :type Vector :default "0, 0, 0") (NormalImpulse :type Vector :default "0, 0, 0") (Hit :type Hit%20Result%20Structure%20%28by%20ref%29))
  (bind _asbp_player_gm1 (Utilities|Casting|CastToBP_Player_GM1 Other))
  (CallFunction|Bump _asbp_player_gm1 (Math|Vector|GetReflectionVector (Transformation|GetVelocity Other) (* HitNormal -1.0))) ; Bump seems to trigger twice on every hit, but it doesn't seem to cause any issues yet. This is less expensive, so it's better for now
)

(fn ConstructionScript)

(fn Bump
  (params (player :type BP%20Player%20GM1%20Object%20Reference) (direction :type Vector))
  (bind _returnvalue (Math|Vector|Normalize direction))
  (bind _bouncevelocity (Variables|Default|GetbounceVelocity))
  (bind _returnvalue_2 (* _returnvalue _bouncevelocity))
  (bind (_x _y) (Math|Vector|BreakVector _returnvalue_2))
  (Character|LaunchCharacter player (Math|Vector|MakeVector _x _y 0.0) true false)
  (Audio|PlaySound2D "/Game/GameMode1/Audio/Placeholder/Q_Bumper.Q_Bumper" 1.0 1.0 0.0 0 0))