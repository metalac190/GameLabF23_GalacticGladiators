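; Game mode for GM1, a local multiplayer mode where all players share one CM_GM1 camera.
; On BeginPlay it creates a local player per player start, adds the input mapping, possesses a BP_InputReciever and removes stray CameraActors.
; SpawnPlayer swaps a receiver's controller onto a new BP_Player_GM1.
; StartGame requires MinPlayers before notifying the camera and firing OnStartGame, while ResetGame restarts the level.
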(event EventBeginPlay
  (bind _outactors (Actor|GetAllActorsOfClass "/Game/GameMode1/Programming/Player/Systems/CM_GM1.CM_GM1_C"))
  (Variables|Camera|SetCameraRef (Utilities|Array|Get(acopy) _outactors))
  ;[0 0 0 0.5] Basic Start
  (CallFunction|GetPlayerStartPoints)
  (CallFunction|SpawnInputRecievers))

(event EventHandleStartingNewPlayer
  (params (NewPlayer :type Player%20Controller%20Object%20Reference))
  ;[1 1 1] Possible Work Around
  (|CallParentFunction NewPlayer)
  (Input|AddMappingContext (PlayerController|LocalPlayerSubsystems|GetEnhancedInputLocalPlayerSubsystem NewPlayer) "/Game/GameMode1/Programming/Player/Input/IMC_GM1.IMC_GM1" 0 "(bIgnoreAllPressedKeysUntilRelease=True,bForceImmediately=False)"))

(fn ConstructionScript)

(fn GetPlayerStartPoints
  (bind _outactors (Actor|GetAllActorsOfClass "/Game/GameMode1/Programming/Player/Systems/BP_GM1_PlayerStart.BP_GM1_PlayerStart_C"))
  (Variables|Player|SetPlayerStarts _outactors))

(fn SpawnInputRecievers
  (bind _returnvalue (Class|GameplayStatics|GetPlayerControllerfromID))
  (bind _returnvalue_2 (Game|GetPlayerController 0))
  (bind _returnvalue_3 (PlayerController|LocalPlayerSubsystems|GetEnhancedInputLocalPlayerSubsystem _returnvalue_2))
  (for (_ _array_index) (Variables|Player|GetPlayerStarts)
    (LocalVariables|SetIndex _array_index)
    ;[0 0 0 0.5] Setup Local Players and Assign IMCs
    (bind _returnvalue_4 (Class|GameplayStatics|CreatePlayer (LocalVariables|GetIndex))) ; -1 Auto Increment doesn't work in UE5 :D
    (if (> (LocalVariables|GetIndex) 0)
      (Utilities|IsValid (PlayerController|LocalPlayerSubsystems|GetEnhancedInputLocalPlayerSubsystem _returnvalue_4)
        (:Is%20Valid
          ;[0 0 0 0.5] Spawn Input Recievers
          (Input|AddMappingContext (PlayerController|LocalPlayerSubsystems|GetEnhancedInputLocalPlayerSubsystem _returnvalue_4) "/Game/GameMode1/Programming/Player/Input/IMC_GM1.IMC_GM1" 0 "(bIgnoreAllPressedKeysUntilRelease=True,bForceImmediately=False)")
          (bind _returnvalue_5 (Game|SpawnActorfromClass "/Game/GameMode1/Programming/Player/Blueprints/BP_InputReciever.BP_InputReciever_C" (Transformation|GetActorTransform (Utilities|Array|Get(acopy) (Variables|Player|GetPlayerStarts) (LocalVariables|GetIndex))) "Undefined" "MultiplyWithRoot" 0 (LocalVariables|GetIndex) 0))
          ;[0 0 0 0.5] Possess Pawn
          (Utilities|Array|AddUnique (Variables|Player|GetPlayerInputRecievers) _returnvalue_5)
          (Pawn|Possess (Class|GameplayStatics|GetPlayerControllerfromID (LocalVariables|GetIndex)) _returnvalue_5)
          (Utilities|Array|AddUnique (Variables|Player|GetPlayerControllers) (Class|GameplayStatics|GetPlayerControllerfromID (LocalVariables|GetIndex)))
          (Game|Player|SetViewTargetwithBlend (Game|GetPlayerController (LocalVariables|GetIndex)) (Variables|Camera|GetCameraRef) 0.0 "VTBlend_Linear" 0.0 false)))
      (else
        (Utilities|IsValid _returnvalue_3
          (:Is%20Valid
            (Input|AddMappingContext _returnvalue_3 "/Game/GameMode1/Programming/Player/Input/IMC_GM1.IMC_GM1" 0 "(bIgnoreAllPressedKeysUntilRelease=True,bForceImmediately=False)")
            (bind _returnvalue_6 (Game|SpawnActorfromClass "/Game/GameMode1/Programming/Player/Blueprints/BP_InputReciever.BP_InputReciever_C" (Transformation|GetActorTransform (Utilities|Array|Get(acopy) (Variables|Player|GetPlayerStarts) (LocalVariables|GetIndex))) "Undefined" "MultiplyWithRoot" 0 (LocalVariables|GetIndex) 0))
            (Utilities|Array|AddUnique (Variables|Player|GetPlayerInputRecievers) _returnvalue_6)
            (Pawn|Possess _returnvalue _returnvalue_6)
            (Utilities|Array|AddUnique (Variables|Player|GetPlayerControllers) _returnvalue)
            (Game|Player|SetViewTargetwithBlend (Game|GetPlayerController 0) (Variables|Camera|GetCameraRef) 0.0 "VTBlend_Linear" 0.0 false))))))
  (CallFunction|RemoveUnusedCameras))

(fn GameStarted
  (Variables|Player|SetisInGame true)
  (Default|GameStarted (Variables|Camera|GetCameraRef) (Variables|Player|GetPlayers))
  (Development|PrintString "GameStarted"))

(fn RemoveUnusedCameras
  (bind _outactors (Actor|GetAllActorsOfClass "/Script/Engine.CameraActor"))
  (for _array_element _outactors
    (Actor|DestroyActor _array_element)))

(fn GetIsinGame
  (return (Variables|Player|GetisInGame)))

(fn ResetGame
  (for _array_element (Variables|Player|GetPlayerControllers)
    (Development|ExecuteConsoleCommand "RestartLevel" _array_element))
  (return true))

(fn SpawnPlayer
  (params (CurrentPlayerIndex :type Integer) (InputReciever :type BP%20Input%20Reciever%20Object%20Reference))
  ;[0 0 0 0.5] Spawn Player Pawn and Possess
  (bind _returnvalue (Game|SpawnActorfromClass "/Game/GameMode1/Programming/Player/Blueprints/BP_Player_GM1.BP_Player_GM1_C" (Transformation|GetActorTransform InputReciever) "Undefined" "MultiplyWithRoot" 0 CurrentPlayerIndex 0))
  (Utilities|Array|Add (Variables|Player|GetPlayers) _returnvalue)
  (Pawn|Possess (Game|GetPlayerController CurrentPlayerIndex) _returnvalue)
  (Game|Player|SetViewTargetwithBlend (Game|GetPlayerController CurrentPlayerIndex) (Variables|Camera|GetCameraRef) 0.0 "VTBlend_Linear" 0.0 false)
  (return false))

(fn StartGame
  (if (>= (Utilities|Array|Length (Variables|Player|GetPlayers)) (Variables|Player|GetMinPlayers))
    (CallFunction|GameStarted)
    (Default|CallOnStartGame)
    (return false)))