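; Game mode for GM1 that sets up local multiplayer on a shared camera and gates the match start.
; BeginPlay creates a local player per player start, adds the input mapping, possesses a spawned input receiver and destroys CameraActors.
; SpawnPlayer spawns a player pawn at a given receiver, possesses it and records it.
; StartGame requires a minimum player count, then GameStarted flags in-game and passes the players to the camera manager.
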(event EventBeginPlay
  (bind _outactors (Actor|GetAllActorsOfClass "/Game/GameMode1/Programming/Player/Blueprints/BP_CameraManager_GM1.BP_CameraManager_GM1_C"))
  (Variables|Default|SetCameraRef (Utilities|Array|Get(acopy) _outactors))
  ;[0 0 0 0.5] Basic Start
  (CallFunction|GetPlayerStartPoints)
  (CallFunction|SpawnInputRecievers)
  (Development|PrintString (Utilities|String|ToString(Integer) (Utilities|Array|Length (Variables|Default|GetPlayers)))))

(fn ConstructionScript)

(fn GetPlayerStartPoints
  (bind _outactors (Actor|GetAllActorsOfClass "/Game/GameMode1/Programming/Player/Blueprints/BP_PlayerStart_GM1.BP_PlayerStart_GM1_C"))
  (Variables|Default|SetPlayerStarts _outactors))

(fn SpawnInputRecievers
  (bind _returnvalue (Class|GameplayStatics|GetPlayerControllerfromID))
  (for (_ _array_index) (Variables|Default|GetPlayerStarts)
    (LocalVariables|SetIndex _array_index)
    ;[0 0 0 0.5] Setup Local Players and Assign IMCs
    (bind _returnvalue_2 (Class|GameplayStatics|CreatePlayer (LocalVariables|GetIndex))) ; -1 Auto Increment doesn't work in UE5 :D
    (if (> (LocalVariables|GetIndex) 0)
      ;[0 0 0 0.5] Spawn Input Recievers
      (Input|AddMappingContext (PlayerController|LocalPlayerSubsystems|GetEnhancedInputLocalPlayerSubsystem _returnvalue_2) "/Game/GameMode1/Programming/Player/Input/IMC_GM1.IMC_GM1" 0 "(bIgnoreAllPressedKeysUntilRelease=True,bForceImmediately=False)")
      (bind _returnvalue_3 (Game|SpawnActorfromClass "/Game/GameMode1/Programming/Player/Blueprints/BP_InputReciever.BP_InputReciever_C" (Transformation|GetActorTransform (Utilities|Array|Get(acopy) (Variables|Default|GetPlayerStarts) (LocalVariables|GetIndex))) "Undefined" "MultiplyWithRoot" 0 (LocalVariables|GetIndex) 0))
      ;[0 0 0 0.5] Possess Pawn
      (Utilities|Array|AddUnique (Variables|Default|GetPlayerInputRecievers) _returnvalue_3)
      (Pawn|Possess (Class|GameplayStatics|GetPlayerControllerfromID (LocalVariables|GetIndex)) _returnvalue_3)
      (Utilities|Array|AddUnique (Variables|Default|GetPlayerControllers) (Class|GameplayStatics|GetPlayerControllerfromID (LocalVariables|GetIndex)))
      (Game|Player|SetViewTargetwithBlend (Game|GetPlayerController (LocalVariables|GetIndex)) (Variables|Default|GetCameraRef) 0.0 "VTBlend_Linear" 0.0 false)
      (else
        (Input|AddMappingContext (PlayerController|LocalPlayerSubsystems|GetEnhancedInputLocalPlayerSubsystem (Game|GetPlayerController 0)) "/Game/GameMode1/Programming/Player/Input/IMC_GM1.IMC_GM1" 0 "(bIgnoreAllPressedKeysUntilRelease=True,bForceImmediately=False)")
        (bind _returnvalue_4 (Game|SpawnActorfromClass "/Game/GameMode1/Programming/Player/Blueprints/BP_InputReciever.BP_InputReciever_C" (Transformation|GetActorTransform (Utilities|Array|Get(acopy) (Variables|Default|GetPlayerStarts) (LocalVariables|GetIndex))) "Undefined" "MultiplyWithRoot" 0 (LocalVariables|GetIndex) 0))
        (Utilities|Array|AddUnique (Variables|Default|GetPlayerInputRecievers) _returnvalue_4)
        (Pawn|Possess _returnvalue _returnvalue_4)
        (Utilities|Array|AddUnique (Variables|Default|GetPlayerControllers) _returnvalue)
        (Game|Player|SetViewTargetwithBlend (Game|GetPlayerController 0) (Variables|Default|GetCameraRef) 0.0 "VTBlend_Linear" 0.0 false))))
  (CallFunction|RemoveUnusedCameras))

(fn GameStarted
  (Variables|Default|SetisInGame true)
  (Default|GameStarted (Variables|Default|GetCameraRef) (Variables|Default|GetPlayers))
  (Development|PrintString "GameStarted"))

(fn RemoveUnusedCameras
  (bind _outactors (Actor|GetAllActorsOfClass "/Script/Engine.CameraActor"))
  (for _array_element _outactors
    (Actor|DestroyActor _array_element)))

(fn GetIsinGame
  (return (Variables|Default|GetisInGame)))

(fn SpawnPlayer
  (params (CurrentPlayerIndex :type Integer) (InputReciever :type BP%20Input%20Reciever%20Object%20Reference))
  ;[0 0 0 0.5] Spawn Player Pawn and Possess
  (bind _returnvalue (Game|SpawnActorfromClass "/Game/GameMode1/Programming/Player/Blueprints/BP_Player_GM1.BP_Player_GM1_C" (Transformation|GetActorTransform InputReciever) "Undefined" "MultiplyWithRoot" 0 CurrentPlayerIndex 0))
  (Utilities|Array|Add (Variables|Default|GetPlayers) _returnvalue)
  (Pawn|Possess (Game|GetPlayerController CurrentPlayerIndex) _returnvalue)
  (Game|Player|SetViewTargetwithBlend (Game|GetPlayerController CurrentPlayerIndex) (Variables|Default|GetCameraRef) 0.0 "VTBlend_Linear" 0.0 false)
  (return false))

(fn StartGame
  (if (>= (Utilities|Array|Length (Variables|Default|GetPlayers)) (Variables|Default|GetMinPlayers))
    (CallFunction|GameStarted)
    (return false)))