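; PC_GM1 is the GameMode1 player controller, handling Enhanced Input movement for the player's pawn.
; IA_Move feeds its X and Y axes into AddMovementInput on player pawn 0, along right and forward vectors from control rotation with pitch zeroed.
; Nodes for adding the IMC_GM1 mapping context, jumping and stopping a jump are disconnected and never run, and BeginPlay is empty.
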(event Input|EnhancedActionEvents|EnhancedInputActionIA_Move
  (params (ActionValue :type Vector%202D%20Structure) (ElapsedSeconds :type Float%20%28double-precision%29) (TriggeredSeconds :type Float%20%28double-precision%29) (InputAction :type Input%20Action%20Object%20Reference :default "/Game/GameMode1/Programming/Player/Input/Actions/IA_Move.IA_Move"))
  (bind _returnvalue (Pawn|GetControlRotation :!class /Script/Engine.Controller))
  (:Triggered
    (Pawn|Input|AddMovementInput (Game|Player|GetPlayerPawn 0) (Math|Vector|GetRightVector (Math|Rotator|MakeRotator (.roll _returnvalue) 0.0 (.yaw _returnvalue))) (.x ActionValue) false)
    (Pawn|Input|AddMovementInput (Game|Player|GetPlayerPawn 0) (Math|Vector|GetForwardVector (Math|Rotator|MakeRotator 0.0 0.0 (.yaw (Pawn|GetControlRotation :!class /Script/Engine.Controller)))) (.y ActionValue) false)))

(event Input|EnhancedActionEvents|EnhancedInputActionIA_Jump
  (params (ActionValue :type Boolean) (ElapsedSeconds :type Float%20%28double-precision%29) (TriggeredSeconds :type Float%20%28double-precision%29) (InputAction :type Input%20Action%20Object%20Reference :default "/Game/GameMode1/Programming/Player/Input/Actions/IA_Jump.IA_Jump")))

(event EventBeginPlay)

(fn ConstructionScript)