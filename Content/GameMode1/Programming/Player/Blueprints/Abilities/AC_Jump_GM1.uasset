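; AC_Jump_GM1 is the jump ability for the GameMode1 player.
; TryToJump starts a jump only when CheckCanJump finds the player neither dashing nor crouched.
; StartJump and EndJump call the player's Jump and StopJumping and set its IsJumping flag to match.
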(fn TrytoJump
  (bind _canjump (CallFunction|CheckCanJump))
  (if _canjump
    (CallFunction|StartJump)))

(fn CheckCanJump
  (bind _as_bp_player_gm1 (Variables|Default|GetAs%20BP%20Player%20GM1))
  (return (and (not (Variables|/Game/GameMode1/Programming/Player/Blueprints/BP_Player_GM1.BP_Player_GM1_C|GetisDashing _as_bp_player_gm1)) (not (Variables|/Script/Engine.Character|GetbIsCrouched _as_bp_player_gm1)))))

(fn StartJump
  (bind _as_bp_player_gm1 (Variables|Default|GetAs%20BP%20Player%20GM1))
  (Character|Jump _as_bp_player_gm1)
  (Variables|/Game/GameMode1/Programming/Player/Blueprints/BP_Player_GM1.BP_Player_GM1_C|SetisJumping _as_bp_player_gm1 true))

(fn EndJump
  (bind _as_bp_player_gm1 (Variables|Default|GetAs%20BP%20Player%20GM1))
  (Character|StopJumping _as_bp_player_gm1)
  (Variables|/Game/GameMode1/Programming/Player/Blueprints/BP_Player_GM1.BP_Player_GM1_C|SetisJumping _as_bp_player_gm1 false))