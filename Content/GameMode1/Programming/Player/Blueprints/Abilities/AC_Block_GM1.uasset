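; Block ability component for the GameMode1 player, which sets the player's IsBlocking flag and plays a sound.
; TryAbilityBlock gates blocking behind a cooldown timer, printing a debug message while it runs, and passes the timer handle to a cooldown delegate.
; TryToBlock starts a block without checking the cooldown.
; EndBlock clears the flag but is not called here, as timer expiry only invalidates the handle.
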(event Custom|TryAbilityBlock
  (if (Class|KismetSystemLibrary|TimerExistsHandle (Variables|Default|GetCooldownTimerHandle))
    (Development|PrintString "cant block")
    (else
      (CallFunction|StartBlock)
      (bind _returnvalue (Utilities|Time|SetTimerbyEvent (delegate Custom|CooldownTimerExpired) (Variables|Default|GetCooldown)))
      (bind _output_get (Variables|Default|SetCooldownTimerHandle _returnvalue))
      (Default|CallCooldownDelegate _output_get))))

(event Custom|CooldownTimerExpired
  (Utilities|Time|ClearandInvalidateTimerbyHandle (Variables|Default|GetCooldownTimerHandle)))

(fn TrytoBlock
  (if true
    (CallFunction|StartBlock)))

(fn StartBlock
  (Variables|/Game/GameMode1/Programming/Player/Blueprints/BP_Player_GM1.BP_Player_GM1_C|SetbIsBlocking (Variables|Default|GetAs%20BP%20Player%20GM1) true)
  (Audio|PlaySound2D "/Game/GameMode1/Audio/Placeholder/Q_Block.Q_Block" 1.0 1.0 0.0 0 0))

(fn EndBlock
  (Variables|/Game/GameMode1/Programming/Player/Blueprints/BP_Player_GM1.BP_Player_GM1_C|SetbIsBlocking (Variables|Default|GetAs%20BP%20Player%20GM1) false))