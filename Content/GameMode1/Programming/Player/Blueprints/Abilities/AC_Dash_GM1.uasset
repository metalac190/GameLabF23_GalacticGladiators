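; Dash ability component for the GameMode1 player that launches the owner forward and knocks away players or crates it hits.
; TryAbilityDash binds capsule overlap, starts the dash and a cooldown timer, and passes the timer handle to a delegate.
; Hits launch non-blocking players or impulse crates, then end the dash.
; Cooldown expiry applies the miss cooldown, flashes the player and ends the dash; several helpers are stubs or unused.
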(event Custom|TryAbilityDash
  (if (Class|KismetSystemLibrary|TimerExistsHandle (Variables|Default|GetCooldownTimerHandle))
    (Development|PrintString "Dash on Cooldown")
    (else
      (Collision|BindEventtoOnComponentBeginOverlap (Variables|/Game/GameMode1/Programming/Player/Blueprints/BP_Player_GM1.BP_Player_GM1_C|GetCapsule (Variables|Default|GetAs%20BP%20Player%20GM1)) (delegate Custom|LaunchEnemy))
      (CallFunction|StartDash)
      (bind _returnvalue (Utilities|Time|SetTimerbyEvent (delegate Custom|CooldownTimeExpired) (Variables|Default|GetCooldown)))
      (bind _output_get (Variables|Default|SetCooldownTimerHandle _returnvalue))
      (Default|CallDelegateCooldown _output_get))))

(event Custom|CooldownTimeExpired
  (Utilities|Time|ClearandInvalidateTimerbyHandle (Variables|Default|GetCooldownTimerHandle))
  (CallFunction|ResetDashCooldown false)
  (CallFunction|ToggleFlash (Variables|Default|GetAs%20BP%20Player%20GM1) true)
  (Utilities|FlowControl|Delay 0.2)
  (CallFunction|ToggleFlash (Variables|Default|GetAs%20BP%20Player%20GM1) false)
  (CallFunction|EndDash))

(event Custom|LaunchEnemy
  (params (OverlappedComponent :type Primitive%20Component%20Object%20Reference) (OtherActor :type Actor%20Object%20Reference) (OtherComp :type Primitive%20Component%20Object%20Reference) (OtherBodyIndex :type Integer) (bFromSweep :type Boolean) (SweepResult :type Hit%20Result%20Structure%20%28by%20ref%29))
  (if (Variables|/Game/GameMode1/Programming/Player/Blueprints/BP_Player_GM1.BP_Player_GM1_C|GetbIsDashing (Variables|Default|GetAs%20BP%20Player%20GM1))
    (if (== (Utilities|GetClass OtherActor) "/Game/GameMode1/Programming/Player/Blueprints/BP_Player_GM1.BP_Player_GM1_C")
      (CallFunction|LaunchHitPlayer OtherActor)
      (else
        (CallFunction|LaunchHitObject OtherActor)))
    (CallFunction|EndDash)))

(fn TrytoDash
  ;[0 0 0 0.5] You Better Not Fuck This Up (it doesnt actually do anything lol)
)

(fn CheckCanDash
  (bind _output_get (Variables|/Game/GameMode1/Programming/Player/Blueprints/BP_Player_GM1.BP_Player_GM1_C|SetbCanDash (Variables|Default|GetAs%20BP%20Player%20GM1) (not (Class|KismetSystemLibrary|TimerExistsHandle (Variables|Default|GetCooldownTimerHandle)))))
  (return _output_get))

(fn StartDash
  (bind _as_bp_player_gm1 (Variables|Default|GetAs%20BP%20Player%20GM1))
  (bind _as_bp_player_gm1_2 (Variables|Default|GetAs%20BP%20Player%20GM1))
  (Variables|/Game/GameMode1/Programming/Player/Blueprints/BP_Player_GM1.BP_Player_GM1_C|SetbIsDashing _as_bp_player_gm1 true)
  (Character|LaunchCharacter _as_bp_player_gm1 (CallFunction|GetForwardLaunchVelocity _as_bp_player_gm1_2 (Variables|/Game/GameMode1/Programming/Player/Systems/Data/PDA_Player_GM1.PDA_Player_GM1_C|GetDashLaunchVelocity (Variables|/Game/GameMode1/Programming/Player/Blueprints/BP_Player_GM1.BP_Player_GM1_C|GetPlayerData _as_bp_player_gm1_2))) true false))

(fn CheckHitActor
  (return false))

(fn EndDash
  (Variables|/Game/GameMode1/Programming/Player/Blueprints/BP_Player_GM1.BP_Player_GM1_C|SetbIsDashing (Variables|Default|GetAs%20BP%20Player%20GM1) false)
  (EventDispatchers|UnbindallEventsfromOnComponentBeginOverlap (Variables|/Game/GameMode1/Programming/Player/Blueprints/BP_Player_GM1.BP_Player_GM1_C|GetCapsule (Variables|Default|GetAs%20BP%20Player%20GM1)))
  (Development|PrintString "dash ended"))

(fn CheckifEndDash
  (if (<= (Math|Vector|VectorLength (Transformation|GetVelocity (Variables|Default|GetAs%20BP%20Player%20GM1))) (Variables|/Script/Engine.CharacterMovementComponent|GetMaxWalkSpeed (Variables|/Script/Engine.Character|GetCharacterMovement (Variables|Default|GetAs%20BP%20Player%20GM1))))
    (CallFunction|EndDash)))

(fn StartDashCooldown)

(fn ResetDashCooldown
  (params (Hit :type Boolean))
  (bind _as_bp_player_gm1 (Variables|Default|GetAs%20BP%20Player%20GM1))
  (bind _playerdata (Variables|/Game/GameMode1/Programming/Player/Blueprints/BP_Player_GM1.BP_Player_GM1_C|GetPlayerData _as_bp_player_gm1))
  (Variables|Default|SetCooldown (Math|Float|SelectFloat (Variables|/Game/GameMode1/Programming/Player/Systems/Data/PDA_Player_GM1.PDA_Player_GM1_C|GetDashHitCooldown _playerdata) (Variables|/Game/GameMode1/Programming/Player/Systems/Data/PDA_Player_GM1.PDA_Player_GM1_C|GetDashMissCooldown _playerdata) Hit))
  (Development|PrintString (select Hit "DashHitCooldown" "DashMissCooldown")))

(fn LaunchHitPlayer
  (params (Player :type Actor%20Object%20Reference))
  (bind _asbp_player_gm1 (Utilities|Casting|CastToBP_Player_GM1 Player))
  (bind _as_bp_player_gm1 (Variables|Default|GetAs%20BP%20Player%20GM1))
  (if (not (Variables|/Game/GameMode1/Programming/Player/Blueprints/BP_Player_GM1.BP_Player_GM1_C|GetbIsBlocking _asbp_player_gm1))
    (Character|LaunchCharacter _asbp_player_gm1 (CallFunction|GetForwardLaunchVelocity _as_bp_player_gm1 (Variables|/Game/GameMode1/Programming/Player/Systems/Data/PDA_Player_GM1.PDA_Player_GM1_C|GetDashHitLaunchVelocity (Variables|/Game/GameMode1/Programming/Player/Blueprints/BP_Player_GM1.BP_Player_GM1_C|GetPlayerData _as_bp_player_gm1))) true false)))

(fn LaunchHitObject
  (params (Actor :type Actor%20Object%20Reference))
  (bind _as_bp_player_gm1 (Variables|Default|GetAs%20BP%20Player%20GM1))
  (bind _asbp_collideable_crate (Utilities|Casting|CastToBP_CollideableCrate Actor))
  (Physics|AddImpulse (Variables|/Game/GameMode1/Programming/Gameplay/BP_CollideableCrate.BP_CollideableCrate_C|GetStaticMesh _asbp_collideable_crate) (CallFunction|GetForwardLaunchVelocity _as_bp_player_gm1 (Variables|/Game/GameMode1/Programming/Player/Systems/Data/PDA_Player_GM1.PDA_Player_GM1_C|GetDashHitLaunchVelocity (Variables|/Game/GameMode1/Programming/Player/Blueprints/BP_Player_GM1.BP_Player_GM1_C|GetPlayerData _as_bp_player_gm1))) "None" true))

(fn ACDashGM1AutoGenFunc
  (params (OverlappedComponent :type Primitive%20Component%20Object%20Reference) (OtherActor :type Actor%20Object%20Reference) (OtherComp :type Primitive%20Component%20Object%20Reference) (OtherBodyIndex :type Integer) (bFromSweep :type Boolean) (SweepResult :type Hit%20Result%20Structure%20%28by%20ref%29))
  (if (== (Utilities|GetClass OtherActor) "/Game/GameMode1/Programming/Player/Blueprints/BP_Player_GM1.BP_Player_GM1_C")
    (CallFunction|LaunchHitPlayer OtherActor)
    (else
      (CallFunction|LaunchHitObject OtherActor)))
  (CallFunction|EndDash)
  (return))

(fn ToggleFlash
  (params (Player :type BP%20Player%20GM1%20Object%20Reference) (FlashOn :type Boolean))
  (Rendering|Material|SetVectorParameterValueonMaterials (Variables|/Game/GameMode1/Programming/Player/Blueprints/BP_Player_GM1.BP_Player_GM1_C|GetCylinder Player) "Emissive" (Math|Vector|SelectVector "1.000000,1.000000,1.000000" "0, 0, 0" FlashOn)))