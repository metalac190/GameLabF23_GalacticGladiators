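; Player crouch ability component for GameMode1, which makes the GM1 player character crouch and stand back up.
; TryToCrouch starts a crouch only when CheckCanCrouch finds the player neither jumping nor dashing.
; StartCrouch and EndCrouch wrap the character's Crouch and UnCrouch calls, with no condition on ending the crouch.
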(fn TrytoCrouch
  (bind _cancrouch (CallFunction|CheckCanCrouch))
  (if _cancrouch
    (CallFunction|StartCrouch)))

(fn CheckCanCrouch
  (bind _as_bp_player_gm1 (Variables|Default|GetAs%20BP%20Player%20GM1))
  (return (and (not (Variables|/Game/GameMode1/Programming/Player/Blueprints/BP_Player_GM1.BP_Player_GM1_C|GetisJumping _as_bp_player_gm1)) (not (Variables|/Game/GameMode1/Programming/Player/Blueprints/BP_Player_GM1.BP_Player_GM1_C|GetisDashing _as_bp_player_gm1)))))

(fn StartCrouch
  (Character|Crouch (Variables|Default|GetAs%20BP%20Player%20GM1)))

(fn EndCrouch
  (Character|UnCrouch (Variables|Default|GetAs%20BP%20Player%20GM1)))