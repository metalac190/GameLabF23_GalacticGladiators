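; Player Blueprint for GameMode1 that handles per-player color and Enhanced Input actions.
; On BeginPlay, Index selects a blue, green, red or yellow material for the Cylinder.
; Move input drives the pawn at that player Index through two direction helpers, whose control-rotation vector nodes are left unused.
; Jump, crouch and dash are placeholders that only print the action with the player's name.
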(event Input|EnhancedActionEvents|EnhancedInputActionIA_Jump_GM1
  (params (ActionValue :type Boolean) (ElapsedSeconds :type Float%20%28double-precision%29) (TriggeredSeconds :type Float%20%28double-precision%29) (InputAction :type Input%20Action%20Object%20Reference :default "/Game/GameMode1/Programming/Player/Input/Actions/IA_Jump_GM1.IA_Jump_GM1"))
  (:Triggered
    (Development|PrintText (Utilities|Text|FormatText "{p} jump" (Utilities|GetDisplayName self)))))

(event Input|EnhancedActionEvents|EnhancedInputActionIA_Crouch_GM1
  (params (ActionValue :type Boolean) (ElapsedSeconds :type Float%20%28double-precision%29) (TriggeredSeconds :type Float%20%28double-precision%29) (InputAction :type Input%20Action%20Object%20Reference :default "/Game/GameMode1/Programming/Player/Input/Actions/IA_Crouch_GM1.IA_Crouch_GM1"))
  (:Triggered
    (Development|PrintText (Utilities|Text|FormatText "{p} crouch" (Utilities|GetDisplayName self)))))

(event Input|EnhancedActionEvents|EnhancedInputActionIA_Dash_GM1
  (params (ActionValue :type Boolean) (ElapsedSeconds :type Float%20%28double-precision%29) (TriggeredSeconds :type Float%20%28double-precision%29) (InputAction :type Input%20Action%20Object%20Reference :default "/Game/GameMode1/Programming/Player/Input/Actions/IA_Dash_GM1.IA_Dash_GM1"))
  (:Triggered
    (Development|PrintText (Utilities|Text|FormatText "{p} dash" (Utilities|GetDisplayName self)))))

(event Input|EnhancedActionEvents|EnhancedInputActionIA_Move_GM1
  (params (ActionValue :type Vector%202D%20Structure) (ElapsedSeconds :type Float%20%28double-precision%29) (TriggeredSeconds :type Float%20%28double-precision%29) (InputAction :type Input%20Action%20Object%20Reference :default "/Game/GameMode1/Programming/Player/Input/Actions/IA_Move_GM1.IA_Move_GM1"))
  (bind (_x _y) (Math|Vector2D|BreakVector2D ActionValue))
  ;[0 0 0 0.5] Move
  (:Triggered
    (Pawn|Input|AddMovementInput (Game|Player|GetPlayerPawn (Variables|Default|GetIndex)) (Utilities|GetHorizontalWorldDirection) _x false)
    (Pawn|Input|AddMovementInput (Game|Player|GetPlayerPawn (Variables|Default|GetIndex)) (Utilities|GetVerticalWorldDirection) _y false)))

(event EventBeginPlay
  ;[0 0 0 0.5] Color
  (Rendering|Material|SetMaterial (Variables|Default|GetCylinder) 0 (Utilities|Select :Index (Variables|Default|GetIndex) :Option%200 "/Game/GameMode1/Art/PlayerMaterials/MI_PlayerMat_Blue.MI_PlayerMat_Blue" :Option%201 "/Game/GameMode1/Art/PlayerMaterials/MI_PlayerMat_Green.MI_PlayerMat_Green" :Option%202 "/Game/GameMode1/Art/PlayerMaterials/MI_PlayerMat_Red.MI_PlayerMat_Red" :Option%203 "/Game/GameMode1/Art/PlayerMaterials/MI_PlayerMat_Yellow.MI_PlayerMat_Yellow")))

(fn ConstructionScript)