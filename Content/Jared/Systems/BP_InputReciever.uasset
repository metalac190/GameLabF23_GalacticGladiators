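; BP_InputReciever is a controlled actor that listens for the join input, apparently for a lobby.
; On BeginPlay it stores its player controller and, when its Index is 0, injects IA_Join through the Enhanced Input subsystem, simulating a join press for that player.
; The IA_Join handler only casts the game mode to GM_Lobby, with no further logic after the cast.
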(event Input|EnhancedActionEvents|EnhancedInputActionIA_Join
  (params (ActionValue :type Boolean) (ElapsedSeconds :type Float%20%28double-precision%29) (TriggeredSeconds :type Float%20%28double-precision%29) (InputAction :type Input%20Action%20Object%20Reference :default "/Game/Jared/Systems/Input/Actions/Lobby/IA_Join.IA_Join"))
  (:Triggered
    (Utilities|Casting|CastToGM_Lobby (Game|GetGameMode))))

(event EventBeginPlay
  (bind _asplayer_controller (Utilities|Casting|CastToPlayerController (Pawn|GetController)))
  (Variables|Default|SetPC _asplayer_controller)
  (if (== (Variables|Default|GetIndex) 0)
    (Class|EnhancedInputSubsystemInterface|InjectInputforAction (PlayerController|LocalPlayerSubsystems|GetEnhancedInputLocalPlayerSubsystem (Variables|Default|GetPC)) "/Game/Jared/Systems/Input/Actions/Lobby/IA_Join.IA_Join" (Class|EnhancedInputLibrary|MakeInputActionValueOfType 1.0 1.0 1.0 "Boolean"))))

(fn ConstructionScript)