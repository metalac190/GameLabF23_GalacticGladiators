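; Lobby game mode that prepares the local multiplayer lobby screen.
; On begin play it shows the first player's mouse cursor and disables splitscreen.
; AddLocalPlayer records each player controller and has the player start at the given index spawn a BP_LobbyPlayer pawn for it.
; SetupInputRecievers is an empty stub.
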(event EventBeginPlay
  (Variables|/Script/Engine.PlayerController|SetbShowMouseCursor (Game|GetPlayerController 0) true)
  (Class|GameplayStatics|SetForceDisableSplitscreen true))

(fn ConstructionScript
  (|CallParentFunction))

(fn SetupInputRecievers)

(fn AddLocalPlayer
  (params (PC :type Player%20Controller%20Object%20Reference) (Index :type Integer) (FirstPlayer :type Player%20State%20Object%20Reference))
  (Utilities|Array|Add (Variables|Default|GetPlayerControllers) PC)
  (Default|SpawnPawnHere (Utilities|Array|Get(acopy) (Variables|Default|GetPlayerStarts) Index) "/Game/Jared/Lobby/BP_LobbyPlayer.BP_LobbyPlayer_C" PC))