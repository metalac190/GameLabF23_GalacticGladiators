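; Player start point that spawns a pawn at its own transform and has a given controller possess it.
; SpawnPlayerHere spawns BP_PlayerBase owned by the controller and passes in PlayerData, leaving its Player input unused.
; SpawnPawnHere spawns any supplied pawn class, adjusting for collisions but always spawning.
; Both functions align control rotation to the start's rotation and return the new pawn.
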(fn ConstructionScript)

(fn SpawnPlayerHere
  (params (PC :type Player%20Controller%20Object%20Reference) (Player :type Actor%20Object%20Reference) (PlayerData :type F%20Player%20Character%20Data%20Structure))
  (Pawn|SetControlRotation PC (Transformation|GetActorRotation))
  (bind _returnvalue (Game|SpawnActorfromClass "/Game/Programming/ReferenceFolder/Systems/BP_PlayerBase.BP_PlayerBase_C" (Transformation|GetActorTransform) "Undefined" "MultiplyWithRoot" PC PlayerData 0))
  (Pawn|Possess PC _returnvalue)
  (return _returnvalue))

(fn SpawnPawnHere
  (params (Pawn :type Pawn%20Class%20Reference) (PC :type Player%20Controller%20Object%20Reference))
  (Pawn|SetControlRotation PC (Transformation|GetActorRotation))
  (bind _returnvalue (Game|SpawnActorfromClass Pawn (Transformation|GetActorTransform) "AdjustIfPossibleButAlwaysSpawn" "MultiplyWithRoot" 0 0))
  (Pawn|Possess PC _returnvalue)
  (return _returnvalue))