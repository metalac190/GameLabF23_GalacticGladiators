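; GM_Lobby is the lobby game mode, handling both local and remote players.
; On BeginPlay it disables splitscreen, creates local players for the placed BP_InputReciever actors and has controllers possess them with the lobby input mapping.
; AddLocalPlayer and HandleStartingNewPlayer (for non-local controllers) spawn BP_LobbyPlayer pawns at indexed PlayerStarts.
; Joins, logouts and controller swaps trigger player-list updates, while local additions also record index and first player in PS_Base.
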(event EventHandleStartingNewPlayer
  (params (NewPlayer :type Player%20Controller%20Object%20Reference))
  ;[0 0 0 0.5] Check for New Player
  (|CallParentFunction NewPlayer)
  (if (Pawn|IsLocalController NewPlayer)
    _
    (else
      (Utilities|Array|Add (Variables|Default|GetPlayerControllers) 0)
      (Default|SpawnPawnHere (Utilities|Array|Get(acopy) (Variables|Default|GetPlayerStarts) (Utilities|Array|FindItem (Variables|/Script/Engine.GameStateBase|GetPlayerArray (Game|GetGameState)) (Variables|/Script/Engine.Controller|GetPlayerState NewPlayer))) "/Game/Programming/ReferenceFolder/Lobby/BP_LobbyPlayer.BP_LobbyPlayer_C" NewPlayer)))
  (Class|BPIGameState|UpdatePlayerList(Message) (Game|GetGameMode)))

(event EventPostLogin
  (params (NewPlayer :type Player%20Controller%20Object%20Reference))
  ;[0 0 0 0.5] Check for New Player
  (|CallParentFunction NewPlayer)
  (Class|BPIGameState|UpdatePlayerList(Message) (Game|GetGameMode)))

(event EventBeginPlay
  (Variables|/Script/Engine.PlayerController|SetbShowMouseCursor (Game|GetPlayerController 0) true)
  (Class|GameplayStatics|SetForceDisableSplitscreen true)
  (CallFunction|SetupInputRecievers)
  (Utilities|FlowControl|Delay 0.5))

(event EventOnLogout
  (params (ExitingController :type Controller%20Object%20Reference))
  ;[0 0 0 0.5] Check for New Player
  (|CallParentFunction ExitingController)
  (Class|BPIGameState|UpdatePlayerList(Message) (Game|GetGameMode)))

(event EventOnSwapPlayerControllers
  (params (OldPC :type Player%20Controller%20Object%20Reference) (NewPC :type Player%20Controller%20Object%20Reference))
  ;[0 0 0 0.5] Check for New Player
  (|CallParentFunction OldPC NewPC)
  (Class|BPIGameState|UpdatePlayerList(Message) (Game|GetGameMode)))

(fn ConstructionScript
  (|CallParentFunction))

(fn SetupInputRecievers
  (bind _outactors (Actor|GetAllActorsOfClass "/Game/Programming/ReferenceFolder/Systems/BP_InputReciever.BP_InputReciever_C"))
  (for _array_element _outactors
    (bind _returnvalue (Class|GameplayStatics|CreatePlayer (Variables|/Game/Programming/ReferenceFolder/Systems/BP_InputReciever.BP_InputReciever_C|GetIndex _array_element)))
    (Utilities|IsValid _returnvalue
      (:Is%20Valid
        (bind _asps_base (Utilities|Casting|CastToPS_Base (Variables|/Script/Engine.Controller|GetPlayerState _returnvalue)))
        (Variables|/Game/Programming/ReferenceFolder/Systems/PS_Base.PS_Base_C|SetLocalIndex _asps_base -1)
        (Input|AddMappingContext (PlayerController|LocalPlayerSubsystems|GetEnhancedInputLocalPlayerSubsystem (select (> (Variables|/Game/Programming/ReferenceFolder/Systems/BP_InputReciever.BP_InputReciever_C|GetIndex _array_element) 0) _returnvalue (Game|GetPlayerController 0))) "/Game/Programming/ReferenceFolder/Systems/Input/IMC_Lobby.IMC_Lobby" 0 "(bIgnoreAllPressedKeysUntilRelease=True,bForceImmediately=False)")
        (Pawn|Possess (select (> (Variables|/Game/Programming/ReferenceFolder/Systems/BP_InputReciever.BP_InputReciever_C|GetIndex _array_element) 0) _returnvalue (Game|GetPlayerController 0)) _array_element)))))

(fn AddLocalPlayer
  (params (PC :type Player%20Controller%20Object%20Reference) (Index :type Integer) (FirstPlayer :type Player%20State%20Object%20Reference))
  (Utilities|Array|Add (Variables|Default|GetPlayerControllers) PC)
  (Default|SpawnPawnHere (Utilities|Array|Get(acopy) (Variables|Default|GetPlayerStarts) Index) "/Game/Programming/ReferenceFolder/Lobby/BP_LobbyPlayer.BP_LobbyPlayer_C" PC)
  (bind _asps_base (Utilities|Casting|CastToPS_Base (Variables|/Script/Engine.Controller|GetPlayerState PC))
    (:then
      (Variables|/Game/Programming/ReferenceFolder/Systems/PS_Base.PS_Base_C|SetLocalIndex _asps_base Index)
      (bind _asps_base_2 (Utilities|Casting|CastToPS_Base FirstPlayer))
      (Variables|/Game/Programming/ReferenceFolder/Systems/PS_Base.PS_Base_C|SetFirstPlayer _asps_base _asps_base_2)
      (Class|BPIGameState|UpdatePlayerList(Message) (Game|GetGameState)))
    (:CastFailed
      (Development|PrintString "Wrong Player State"))))