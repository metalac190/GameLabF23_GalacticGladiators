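; Player dash ability component that shoves rival players and crates, gated by a cooldown and blocking.
; Looping timers add curve-scaled forward velocity up to a max speed, then wait for slowdown before clearing the dashing state.
; A repeating forward sphere trace selects hit or miss cooldown, launches non-blocking players, making them drop the crown, and impulses crates.
; Cooldown expiry flashes the player's emissive material.
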(event Custom|TryAbilityDash
  (if (CallFunction|CheckCanDash)
    (CallFunction|StartDash)
    (bind _returnvalue (Utilities|Time|SetTimerbyEvent (delegate Custom|CooldownTimeExpired) (Variables|Default|GetCooldown)))
    (bind _output_get (Variables|Default|SetCooldownTimerHandle _returnvalue))
    (Default|CallDelegateCooldown _output_get)))

(event Custom|CooldownTimeExpired
  (Utilities|Time|ClearandInvalidateTimerbyHandle (Variables|Default|GetCooldownTimerHandle))
  (CallFunction|ToggleFlash (Variables|Default|GetPlayer) true)
  (Utilities|FlowControl|Delay 0.2)
  (CallFunction|ToggleFlash (Variables|Default|GetPlayer) false)
  (CallFunction|EndDash))

(event EventTick
  (params (DeltaSeconds :type Float%20%28single-precision%29)))

(fn CheckCanDash
  (bind _player (Variables|Default|GetPlayer))
  (bind _output_get (Variables|/Game/Programming/GM1/Blueprints/Player/Blueprints/BP_Player_GM1.BP_Player_GM1_C|SetbCanDash _player (and (not (Class|KismetSystemLibrary|TimerExistsHandle (Variables|Default|GetCooldownTimerHandle))) (not (Variables|/Game/Programming/GM1/Blueprints/Player/Blueprints/BP_Player_GM1.BP_Player_GM1_C|GetbIsBlocking _player)))))
  (return _output_get))

(fn StartDash
  (bind _dashdata (Variables|Default|GetDashData))
  (CallFunction|PlayAbilityEffects (Variables|/Game/Programming/GM1/Blueprints/Player/Systems/Data/PDA_Dash.PDA_Dash_C|GetDashSFX _dashdata) (Variables|/Game/Programming/GM1/Blueprints/Player/Systems/Data/PDA_Dash.PDA_Dash_C|GetDashVFX _dashdata))
  (Default|CallOnDash)
  (Variables|/Game/Programming/GM1/Blueprints/Player/Blueprints/BP_Player_GM1.BP_Player_GM1_C|SetbIsDashing (Variables|Default|GetPlayer) true)
  (Variables|Default|SetTimePassed 0.0)
  (bind _returnvalue (Utilities|Time|SetTimerbyFunctionName 0 "DashUpdate" (Variables|Default|GetDelta) true))
  (Variables|Default|SetDashTimer _returnvalue)
  (bind _returnvalue_2 (Utilities|Time|SetTimerbyFunctionName 0 "CheckHitActor" (Variables|Default|GetDelta) true))
  (Variables|Default|SetHitActorHandle _returnvalue_2))

(fn CheckHitActor
  (bind _player (Variables|Default|GetPlayer))
  (bind _returnvalue (Transformation|GetActorLocation _player))
  (bind _outhit (Collision|SphereTraceByChannel _returnvalue (+ _returnvalue (* (Transformation|GetActorForwardVector _player) (Variables|/Game/Programming/GM1/Blueprints/Player/Systems/Data/PDA_Dash.PDA_Dash_C|GetRange (Variables|Default|GetDashData)))) (Variables|/Game/Programming/GM1/Blueprints/Player/Systems/Data/PDA_Dash.PDA_Dash_C|GetRadius (Variables|Default|GetDashData)) "TraceTypeQuery2" false 0 "ForDuration"))
  (Utilities|IsActorPlayer (.HitActor (Collision|BreakHitResult _outhit))
    (:IsPlayer
      (Variables|Default|SetCooldown (Variables|/Game/Programming/GM1/Blueprints/Player/Systems/Data/PDA_Dash.PDA_Dash_C|GetHitCooldown (Variables|Default|GetDashData)))
      (CallFunction|LaunchHitPlayer (.HitActor (Collision|BreakHitResult _outhit)))
      (return))
    (:IsNotPlayer
      (Variables|Default|SetCooldown (Variables|/Game/Programming/GM1/Blueprints/Player/Systems/Data/PDA_Dash.PDA_Dash_C|GetMissCooldown (Variables|Default|GetDashData)))
      (CallFunction|LaunchHitObject (.HitActor (Collision|BreakHitResult _outhit)))
      (return))))

(fn EndDash
  (CallFunction|CancelDash))

(fn CheckifEndDash
  (if (<= (Math|Vector|VectorLength (Transformation|GetVelocity (Variables|Default|GetPlayer))) (Variables|/Script/Engine.CharacterMovementComponent|GetMaxWalkSpeed (Variables|/Script/Engine.Character|GetCharacterMovement (Variables|Default|GetPlayer))))
    (CallFunction|EndDash)))

(fn StartDashCooldown)

(fn ResetDashCooldown
  (params (Hit :type Boolean)))

(fn LaunchHitPlayer
  (params (Player :type Actor%20Object%20Reference))
  (bind _asbp_player_gm1 (Utilities|Casting|CastToBP_Player_GM1 Player))
  (if (not (Variables|/Game/Programming/GM1/Blueprints/Player/Blueprints/BP_Player_GM1.BP_Player_GM1_C|GetbIsBlocking _asbp_player_gm1))
    (Character|LaunchCharacter _asbp_player_gm1 (CallFunction|GetForwardLaunchVelocity (Variables|Default|GetPlayer) (Variables|/Game/Programming/GM1/Blueprints/Player/Systems/Data/PDA_Player_GM1.PDA_Player_GM1_C|GetDashHitLaunchVelocity (Variables|/Game/Programming/GM1/Blueprints/Player/Blueprints/BP_Player_GM1.BP_Player_GM1_C|GetPlayerData (Variables|Default|GetPlayer)))) true false)
    (Default|DropCrown _asbp_player_gm1 (Variables|Default|GetPlayer))
    (bind _asgi_core_game_instance (Utilities|Casting|CastToGI_CORE_GameInstance (Game|GetGameInstance)))
    (CallFunction|PlayAbilityEffects (Variables|/Game/Programming/Core/Blueprints/GameInstance/PDA_GameInstanceSettings.PDA_GameInstanceSettings_C|GetGenericImpactSFX (Variables|/Game/Programming/Core/Blueprints/GameInstance/GI_CORE_GameInstance.GI_CORE_GameInstance_C|GetGameInstanceVariables _asgi_core_game_instance)) (Variables|/Game/Programming/Core/Blueprints/GameInstance/PDA_GameInstanceSettings.PDA_GameInstanceSettings_C|GetGenericImpactVFX (Variables|/Game/Programming/Core/Blueprints/GameInstance/GI_CORE_GameInstance.GI_CORE_GameInstance_C|GetGameInstanceVariables _asgi_core_game_instance)))
    (CallFunction|Play3DSFX "NewEnumerator9" (Transformation|GetActorLocation (Components|GetOwner)) "0, 0, 0")))

(fn LaunchHitObject
  (params (Actor :type Actor%20Object%20Reference))
  (bind _player (Variables|Default|GetPlayer))
  (bind _asbp_collideable_crate (Utilities|Casting|CastToBP_CollideableCrate Actor))
  (Physics|AddImpulse (Variables|/Game/Programming/GM1/Blueprints/Gameplay/BP_CollideableCrate.BP_CollideableCrate_C|GetStaticMesh _asbp_collideable_crate) (CallFunction|GetForwardLaunchVelocity _player (Variables|/Game/Programming/GM1/Blueprints/Player/Systems/Data/PDA_Player_GM1.PDA_Player_GM1_C|GetDashHitLaunchVelocity (Variables|/Game/Programming/GM1/Blueprints/Player/Blueprints/BP_Player_GM1.BP_Player_GM1_C|GetPlayerData _player))) "None" true)
  (Development|PrintString "Hello"))

(fn ACDashGM1AutoGenFunc
  (params (OverlappedComponent :type Primitive%20Component%20Object%20Reference) (OtherActor :type Actor%20Object%20Reference) (OtherComp :type Primitive%20Component%20Object%20Reference) (OtherBodyIndex :type Integer) (bFromSweep :type Boolean) (SweepResult :type Hit%20Result%20Structure%20%28by%20ref%29))
  (if (== (Utilities|GetClass OtherActor) "/Game/Programming/GM1/Blueprints/Player/Blueprints/BP_Player_GM1.BP_Player_GM1_C")
    (CallFunction|LaunchHitPlayer OtherActor)
    (else
      (CallFunction|LaunchHitObject OtherActor)))
  (CallFunction|EndDash)
  (return))

(fn ToggleFlash
  (params (Player :type BP%20Player%20GM1%20Object%20Reference) (FlashOn :type Boolean))
  (Rendering|Material|SetVectorParameterValueonMaterials (Variables|/Game/Programming/GM1/Blueprints/Player/Blueprints/BP_Player_GM1.BP_Player_GM1_C|GetCylinder Player) "Emissive" (Math|Vector|SelectVector "1.000000,1.000000,1.000000" "0, 0, 0" FlashOn)))

(fn DashUpdate
  (bind _max_dash_speed (Variables|Default|Getmax%20dash%20speed))
  (bind _character_movement (Variables|Default|GetCharacter%20Movement))
  (bind _velocity (Variables|/Script/Engine.MovementComponent|GetVelocity _character_movement))
  (Utilities|CalculateNewVelocity)
  (Utilities|PlusEqualsFloat (Variables|Default|GetTimePassed) (Variables|Default|GetDelta)
    (:%20%20
      (if (or (> (Math|Float|Absolute(Float) (.x _velocity)) _max_dash_speed) (> (Math|Float|Absolute(Float) (.y _velocity)) _max_dash_speed))
        (CallFunction|EndDash)
        (bind _returnvalue (Utilities|Time|SetTimerbyFunctionName 0 "DashCancelUpdate" (Variables|Default|GetDelta) true))
        (Variables|Default|Setfuck _returnvalue)))))

(fn CancelDash
  (Utilities|Time|ClearandInvalidateTimerbyHandle (Variables|Default|GetDashTimer)))

(fn DashCancelUpdate
  (bind _character_movement (Variables|Default|GetCharacter%20Movement))
  (bind _velocity (Variables|/Script/Engine.MovementComponent|GetVelocity _character_movement))
  (if (and (<= (Math|Float|Absolute(Float) (.x _velocity)) 6e+02) (<= (Math|Float|Absolute(Float) (.y _velocity)) 6e+02))
    (Variables|/Game/Programming/GM1/Blueprints/Player/Blueprints/BP_Player_GM1.BP_Player_GM1_C|SetbIsDashing (Variables|Default|GetPlayer) false)
    (Utilities|Time|ClearandInvalidateTimerbyHandle (Variables|Default|Getfuck))
    (Utilities|Time|ClearandInvalidateTimerbyHandle (Variables|Default|GetHitActorHandle))
    (else
      (Variables|/Game/Programming/GM1/Blueprints/Player/Blueprints/BP_Player_GM1.BP_Player_GM1_C|SetbIsDashing (Variables|Default|GetPlayer) true))))