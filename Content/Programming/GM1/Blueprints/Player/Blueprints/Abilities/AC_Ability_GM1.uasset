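; AC_Ability_GM1 is an ability component for the GM1 player, apparently a base for specific abilities.
; On BeginPlay it casts its owner to BP_Player_GM1 and caches the player and its CharacterMovement.
; PlayAbilityEffects plays a supplied sound and spawns a supplied visual effect system at the player's location.
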(event Custom|PlayAbilityEffects
  (params (Audio :type Sound%20Base%20Object%20Reference) (Visual :type Niagara%20System%20Object%20Reference))
  (bind _player (Variables|Default|GetPlayer))
  (bind _returnvalue (Transformation|GetActorLocation _player))
  (Audio|PlaySoundatLocation Audio _returnvalue "0, 0, 0" 1.0 1.0 0.0 0 0 0 0)
  (Niagara|SpawnSystematLocation Visual _returnvalue))

(event EventBeginPlay
  (|CallParentFunction)
  (bind _asbp_player_gm1 (Utilities|Casting|CastToBP_Player_GM1 (Components|GetOwner)))
  (bind _output_get (Variables|Default|SetPlayer _asbp_player_gm1))
  (Variables|Default|SetCharacter%20Movement (Variables|/Script/Engine.Character|GetCharacterMovement _output_get)))