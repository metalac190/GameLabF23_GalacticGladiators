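; BP_IceMeteor is an ice variant of a meteor hazard that leaves an ice patch where it lands.
; It overrides Impact, runs the parent logic, then spawns BP_IcePatch at the meteor's location with a random yaw and a scale derived from its Radius.
; All other behavior comes from the parent class, as its own event graph and construction script add nothing.
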(event EventBeginPlay
  (|CallParentFunction) ; This node is disabled and will not be called.\nDrag off pins to build functionality.
)

(event Collision|EventActorBeginOverlap
  (params (OtherActor :type Actor%20Object%20Reference))
  (|CallParentFunction OtherActor) ; This node is disabled and will not be called.\nDrag off pins to build functionality.
)

(event EventTick
  (params (DeltaSeconds :type Float%20%28single-precision%29))
  (|CallParentFunction DeltaSeconds) ; This node is disabled and will not be called.\nDrag off pins to build functionality.
)

(fn ConstructionScript
  (|CallParentFunction))

(fn Impact
  (|CallParentFunction)
  ;[0 0 0] Spawn an ice patch at the meteor's transform
  (Game|SpawnActorfromClass "/Game/Programming/GM1/Blueprints/Hazards/BP_IcePatch.BP_IcePatch_C" (Math|Transform|MakeTransform (Transformation|GetActorLocation) (Math|Rotator|MakeRotator 0.0 0.0 (Math|Random|RandomFloatinRange 0.0 3.6e+02)) (Math|Conversions|ToVector(Float) (/ (Variables|Default|GetRadius) 5e+01))) "Undefined" "MultiplyWithRoot" 0 0))