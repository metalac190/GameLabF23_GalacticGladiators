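; BP_GM1_Meteor is a meteor hazard for GM1 that knocks back nearby players and static mesh actors on impact.
; DelayImpact waits a predicted fall time, teleports the meteor to the given hit location and calls Impact, rather than detecting collision.
; Impact uses a sphere overlap to apply radial, optionally horizontal-only impulses, and makes hit players drop their crown.
; The meteor then hides and destroys itself after its impact audio finishes.
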(event Custom|DelayImpact
  (params (HitLocation :type Vector) (TimeTillHit :type Float%20%28double-precision%29) (Impact%20SW :type Sound%20Wave%20Object%20Reference))
  (bind _hazard_impact_audio (Variables|Default|GetHazard%20Impact%20Audio))
  ;[0 0 0 0.25] Should be deprecated in favor of using a built in collision event at some point. Requiring the system to know when and where an impact will occur prior to spawning a meteor makes it difficult to use meteors when arena parts can move.
  (Utilities|FlowControl|Delay TimeTillHit) ; Wait till predicted impact time
  (Transformation|SetActorLocation HitLocation false true) ; Teleport to Impact Location
  (Physics|SetPhysicsLinearVelocity (Variables|Default|GetSphereCol) "0, 0, 0" false "None")
  (CallFunction|Impact)
  ;;[0 0 0] Hide the meteor, then destroy it once the impact SFX have stopped playing
  (Audio|Components|Audio|Stop (Variables|Default|GetHazard%20Fall%20Audio))
  (Audio|Components|Audio|Play _hazard_impact_audio 0.0)
  (Rendering|SetActorHiddenInGame true)
  (Utilities|FlowControl|Delay 0.5 :!label _label)
  (if (Audio|Components|Audio|IsPlaying _hazard_impact_audio)
    (goto _label)
    (else
      (Actor|DestroyActor))))

(fn ConstructionScript)

(fn Impact
  (bind _returnvalue (Transformation|GetActorLocation))
  ;[0 0 0] Knock back each actor in the radius of effect. Effectively apes a RadialForceComponent except that we can fix the impulse to the horizontal.
  (bind _outactors (Collision|SphereOverlapActors _returnvalue (Variables|Default|GetRadius) (Variables|Default|GetAffect%20Channels) 0))
  (for _array_element _outactors
    (bind _asbp_player_gm1 (Utilities|Casting|CastToBP_Player_GM1 _array_element)
      (:then
        (Physics|AddImpulse (Variables|/Script/Engine.Character|GetCharacterMovement _asbp_player_gm1) (* (Math|Vector|SelectVector (Class|KismetMathLibrary|VectorNormal2D (- (Transformation|GetActorLocation _array_element) _returnvalue) 0.0001) (Math|Vector|Normalize (- (Transformation|GetActorLocation _array_element) _returnvalue)) (Variables|Default|GetHorizontalImpulseOnly)) (Variables|Default|GetForce)) false)
        (Default|DropCrown _asbp_player_gm1))
      (:CastFailed
        (bind _asstatic_mesh_actor (Utilities|Casting|CastToStaticMeshActor _array_element))
        (Physics|AddImpulse (Variables|/Script/Engine.StaticMeshActor|GetStaticMeshComponent _asstatic_mesh_actor) (* (Math|Vector|SelectVector (Class|KismetMathLibrary|VectorNormal2D (- (Transformation|GetActorLocation _array_element) _returnvalue) 0.0001) (Math|Vector|Normalize (- (Transformation|GetActorLocation _array_element) _returnvalue)) (Variables|Default|GetHorizontalImpulseOnly)) (Variables|Default|GetForce)) "None" false)))))

(fn SetMeteorSettings
  (params (speed :type Float%20%28double-precision%29) (size :type Float%20%28double-precision%29) (force :type Float%20%28double-precision%29) (horizontalOnly :type Boolean))
  (Variables|Default|SetRadius (* size 5e+01))
  (Variables|Default|SetForce force)
  (Variables|Default|SetHorizontalImpulseOnly horizontalOnly))