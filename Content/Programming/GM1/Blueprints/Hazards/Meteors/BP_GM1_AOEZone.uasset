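; BP_GM1_AOEZone is an area-of-effect warning decal for meteor hazards.
; On spawn, a timeline scales it up to its placed X scale, applied uniformly.
; Tick waits for a valid WatchingHazard, then activates warning audio and starts a timeline pulsing the decal toward white.
; When that hazard becomes hidden, treated as destroyed, the decal fades out and destroys the actor.
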(event EventBeginPlay
  ;[0 0 0] Animate Scale Intro
  (Variables|Default|SettargetSize (.X (Math|Vector|BreakVector (Transformation|GetActorScale3D))))
  (bind _scale (Timeline|SizeAnim PlayFromStart)
    (:Update
      (Transformation|SetActorScale3D (Math|Conversions|ToVector(Float) (* _scale (Variables|Default|GettargetSize)))))))

(event EventTick
  (params (DeltaSeconds :type Float%20%28single-precision%29))
  ;[0 0 0] Currently looking for Hazard?
  (if (Variables|Default|GetcheckingForHazard)
    (if (Variables|/Script/Engine.Actor|GetbHidden (Variables|Default|GetwatchingHazard))
      ;[0 0 0] Hazard was destroyed, setup Fade Out auto destroy
      (Variables|Default|SetcheckingForHazard false)
      (Rendering|Components|Decal|SetFadeOut (Variables|Default|GetAOE%20Zone%20Decal) 0.01 0.25 true)
      (Variables|Default|SetwatchingHazard 0)
      (elif (not (Variables|Default|GetisFlashing))
        ;[0 0 0] Set Original Color
        (Variables|Default|SetorigColor (Variables|/Script/Engine.DecalComponent|GetDecalColor (Variables|Default|GetAOE%20Zone%20Decal)))
        (Variables|Default|SetisFlashing true)
        (Components|Activation|Activate (Variables|Default|GetAOE%20Warning%20Audio) false)
        ;[0 0 0] Pulse/Flash Animation
        (bind _pulseflash (Timeline|FlashAnim PlayFromStart)
          (:Update
            (Rendering|Components|Decal|SetDecalColor (Variables|Default|GetAOE%20Zone%20Decal) (Math|Color|Lerp(LinearColor) (Variables|Default|GetorigColor) "(R=1.000000,G=1.000000,B=1.000000,A=1.000000)" _pulseflash))))))
    (else
      ;[0 0 0] Flag that primes if this AOE Zone is ready to destroy itself with Hazard
      (Utilities|IsValid (Variables|Default|GetwatchingHazard)
        (:Is%20Valid
          (Variables|Default|SetcheckingForHazard true))))))

(fn ConstructionScript)