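; BP_Bumper1 is a stage-hazard bumper that launches players along their reflected velocity on hit, drops their crown and plays a bump animation and sound.
; Once registered with GM_GM1, it responds to the hazard-start event by briefly showing a warning decal, then raising its mesh with a timeline.
; Editor-only functions save or append placed bumper locations to a hazard data asset, destroying those bumpers.
; Another function respawns bumpers from that data.
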(event Custom|Register%20As%20Stage%20Hazard
  (EventDispatchers|BindEventtoOnStageHazardStart (.AsGM%20GM1 (Utilities|Casting|CastToGM_GM1 (Game|GetGameMode))) (delegate Custom|RaiseBumper)))

(event Custom|RaiseBumper
  (bind _staticmeshcomponent (Variables|Debug|GetStaticMeshComponent))
  (bind _returnvalue (Transformation|GetWorldLocation _staticmeshcomponent))
  ;[0 0 0] Briefly display warning
  (Development|SetHiddeninGame (Variables|Default|GetDecalWarning) false false)
  (Utilities|FlowControl|Delay 3.0)
  (Development|SetHiddeninGame (Variables|Default|GetDecalWarning) true false)
  ;[0 0 0] Animate bumper upward
  (bind _alpha (Timeline|Rise PlayFromStart)
    (:Update
      (Transformation|SetWorldLocation (Variables|Debug|GetStaticMeshComponent) (Math|Vector|MakeVector (.x _returnvalue) (.y _returnvalue) (Math|Float|Lerp (.Z (Math|Vector|BreakVector (Transformation|GetActorLocation))) 16.0 _alpha)) false false))))

(event Collision|EventHit
  (params (MyComp :type Primitive%20Component%20Object%20Reference) (Other :type Actor%20Object%20Reference) (OtherComp :type Primitive%20Component%20Object%20Reference) (bSelfMoved :type Boolean) (HitLocation :type Vector :default "0, 0, 0") (HitNormal :type Vector :default "0, 0, 0") (NormalImpulse :type Vector :default "0, 0, 0") (Hit :type Hit%20Result%20Structure%20%28by%20ref%29))
  ;[0 0 0] If we hit a player, bounce that player and play animation
  (bind _asbp_player_gm1 (Utilities|Casting|CastToBP_Player_GM1 Other))
  (CallFunction|Bump _asbp_player_gm1 (Math|Vector|GetReflectionVector (Transformation|GetVelocity Other) (* HitNormal -1.0))) ; Bump seems to trigger twice on every hit, but it doesn't seem to cause any issues yet. This is less expensive, so it's better for now
  (Components|Animation|PlayAnimation (Variables|Default|GetBumper) "/Game/GameMode1/Art/EnviormentAssets/Bumper/BumperAnim_Bump.BumperAnim_Bump" false))

(fn ConstructionScript)

(fn Bump
  (params (player :type BP%20Player%20GM1%20Object%20Reference) (direction :type Vector))
  (bind _returnvalue (Math|Vector|Normalize direction))
  (bind _bouncevelocity (Variables|Default|GetbounceVelocity))
  (bind _returnvalue_2 (* _returnvalue _bouncevelocity))
  (bind (_x _y) (Math|Vector|BreakVector _returnvalue_2))
  ;[0 0 0] Boink the player
  (Character|LaunchCharacter player (Math|Vector|MakeVector _x _y 0.0) true false)
  (Default|DropCrown player)
  (Audio|PlaySound2D "/Game/Audio/Placeholder/Q_Bumper.Q_Bumper" 1.0 1.0 0.0 0 0))

(fn SaveBumperLocations
  ;[0 0 0] EDITOR ONLY: Save the location of all bumpers in current level to the bumper hazard data asset, overwriting any previously saved data, then destroy those bumpers
  (bind _outactors (Actor|GetAllActorsOfClass "BP_Bumper1_C"))
  (if (!= (Utilities|Array|Length _outactors) 0)
    (Default|CopyLocationsOfBumpers (Variables|Default|GetStageHazardData) _outactors)
    (for _array_element _outactors
      (Actor|DestroyActor _array_element))))

(fn AddBumperLocations
  ;[0 0 0] EDITOR ONLY: Save the location of all bumpers in current level to the bumper hazard data asset, appending to any previously saved data, then destroy those bumpers
  (bind _outactors (Actor|GetAllActorsOfClass "BP_Bumper1_C"))
  (if (!= (Utilities|Array|Length _outactors) 0)
    (Default|AddLocationsOfBumpers (Variables|Default|GetStageHazardData) _outactors)
    (for _array_element _outactors
      (Actor|DestroyActor _array_element))))

(fn SpawnSavedBumpers
  ;[0 0 0] Destroy any bumpers in the level
  (bind _outactors (Actor|GetAllActorsOfClass "BP_Bumper1_C"))
  (for _array_element _outactors
    (Actor|DestroyActor _array_element))
  ;[0 0 0] Spawn a bumper at each location saved to the bumper hazard data asset
  (for _array_element_2 (Variables|/Game/Programming/GM1/Blueprints/Hazards/Data/PDA_BumperHazard.PDA_BumperHazard_C|GetBumperLocations (Variables|Default|GetStageHazardData))
    (Game|SpawnActorfromClass "BP_Bumper1_C" (Math|Conversions|ToTransform(Vector) _array_element_2) "AlwaysSpawn" "MultiplyWithRoot" 0 0 0)))