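; GM1 is a Blueprint function library of small shared helpers for gameplay code.
; It computes trace-style start and end points from an actor's location, forward vector and a given distance.
; It also returns the DA_Gameplay asset as a central access point and derives a forward launch velocity from a target's rotation and a launch speed.
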(fn GetStartEndLocationbyDistance
  (params (Actor :type Actor%20Object%20Reference) (Distance :type Float%20%28double-precision%29))
  (bind _returnvalue (Transformation|GetActorLocation Actor))
  (return _returnvalue (+ _returnvalue (* (Transformation|GetActorForwardVector Actor) Distance))))

(fn GetGameplayData
  (return "/Game/Design/Data/GM1/DA_Gameplay.DA_Gameplay"))

(fn GetForwardLaunchVelocity
  (params (Target :type Actor%20Object%20Reference) (LaunchVelocity :type Float%20%28single-precision%29))
  (return (* (Math|Vector|GetForwardVector (Transformation|GetActorRotation Target)) LaunchVelocity)))