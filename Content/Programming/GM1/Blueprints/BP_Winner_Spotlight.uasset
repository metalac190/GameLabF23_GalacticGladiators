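; BP_Winner_Spotlight is a spotlight actor that hovers above the player with the highest score in the GM1 game mode.
; It stays hidden until the first score change, binding to the game mode's start event and then the HUD widget's score change event.
; Each score change rescans the HUD's score array to retarget the leader's pawn, which Tick follows from a fixed height.
; The construction script applies configurable intensity, color and cone angle.
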(event Custom|ScoreChange
  (params (PlayerIndex :type Integer) (Amount :type Integer))
  (bind _spotlight (Variables|Default|GetSpotLight))
  ;[0 0 0] Sets Tracked Actor When New Player Has Highest Score
  (for (_array_element _array_index) (Variables|/Game/Programming/GM1/Widgets/WBP_GM1_CrownMode.WBP_GM1_CrownMode_C|GetScoreArray (Variables|/Game/Programming/GM1/Blueprints/Systems/GM_GM1.GM_GM1_C|GetHUDWidget (.AsGM%20GM1 (Utilities|Casting|CastToGM_GM1 (Game|GetGameMode)))))
    (if (> (Variables|/Game/Programming/GM1/Widgets/WBP_GM1_PlayerScore.WBP_GM1_PlayerScore_C|GetTotal%20Score _array_element) (Variables|Default|GetHighestScore))
      (Variables|Default|SetHighestScore (Variables|/Game/Programming/GM1/Widgets/WBP_GM1_PlayerScore.WBP_GM1_PlayerScore_C|GetTotal%20Score _array_element))
      (Variables|Default|SetIndexOfHighestScore _array_index)))
  (Variables|Default|SetHighestScore 0)
  (bind _asbp_player_gm1 (Utilities|Casting|CastToBP_Player_GM1 (Pawn|GetControlledPawn (Class|GameplayStatics|GetPlayerControllerfromID (Variables|Default|GetIndexOfHighestScore)))))
  (bind _output_get (Variables|Default|SetTrackedActor _asbp_player_gm1))
  ;[0 0 0] Initial Setup
  (Utilities|FlowControl|DoOnce false
    (:Completed
      (Transformation|SetWorldLocation _spotlight (Math|Vector|MakeVector (.x (Transformation|GetActorLocation _output_get)) (.y (Transformation|GetActorLocation _output_get)) (+ (.z (Transformation|GetActorLocation _output_get)) 1.25e+03)) false false)
      (Rendering|SetVisibility _spotlight true false))))

(event Custom|Start%20Game
  ;[0 0 0] Event Bindings
  (EventDispatchers|BindEventtoOnScoreChange (Variables|/Game/Programming/GM1/Blueprints/Systems/GM_GM1.GM_GM1_C|GetHUDWidget (.AsGM%20GM1 (Utilities|Casting|CastToGM_GM1 (Game|GetGameMode)))) (delegate Custom|ScoreChange)))

(event EventBeginPlay
  ;[0 0 0] Event Bindings
  (EventDispatchers|BindEventtoOnStartGame (.AsGM%20GM1 (Utilities|Casting|CastToGM_GM1 (Game|GetGameMode))) (delegate Custom|Start%20Game))
  (Rendering|SetVisibility (Variables|Default|GetSpotLight) false false))

(event Collision|EventActorBeginOverlap
  (params (OtherActor :type Actor%20Object%20Reference)))

(event EventTick
  (params (DeltaSeconds :type Float%20%28single-precision%29))
  (bind _trackedactor (Variables|Default|GetTrackedActor))
  (bind _returnvalue (Transformation|GetActorLocation _trackedactor))
  ;[0 0 0] Set Position
  (Utilities|IsValid _trackedactor
    (:Is%20Valid
      (Transformation|SetWorldLocation (Variables|Default|GetSpotLight) (Math|Vector|MakeVector (.x _returnvalue) (.y _returnvalue) (+ (.z _returnvalue) 1.25e+03)) false false))))

(fn ConstructionScript
  (bind _spotlight (Variables|Default|GetSpotLight))
  (Rendering|Components|Light|SetIntensity _spotlight (Variables|Default|GetSpotlightIntensity))
  (Rendering|Components|Light|SetLightColor _spotlight (Variables|Default|GetSpotlightColor) true)
  (Rendering|Lighting|SetOuterConeAngle _spotlight (Variables|Default|GetSpotlightOuterConeAngle)))