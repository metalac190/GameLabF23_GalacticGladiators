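; BP_TargetedCamera is a camera actor that follows a group of target actors and zooms to keep them in view.
; Each tick it eases toward the targets' average location, then AutoZoom tests their angles from the camera's forward vector against TrackedFOV and steps a clamped, interpolated boom distance in or out.
; Functions add or remove targets, yaw the camera, or, as a temporary hack, gather all BP_Player_GM1 actors as targets.
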(event EventBeginPlay)

(event Collision|EventActorBeginOverlap
  (params (OtherActor :type Actor%20Object%20Reference)))

(event EventTick
  (params (DeltaSeconds :type Float%20%28single-precision%29))
  (bind _returnvalue (Class|GameplayStatics|GetActorArrayAverageLocation (Variables|Default|GettargetActors)))
  (Transformation|SetActorLocation (Math|Interpolation|VInterpTo (Transformation|GetActorLocation) _returnvalue DeltaSeconds (Variables|Default|GetinterpolationSpeed)) false false)
  (CallFunction|AutoZoom DeltaSeconds))

(fn ConstructionScript)

(fn AddTargetActor
  (params (newTarget :type Actor%20Object%20Reference))
  (bind _returnvalue (Utilities|Array|AddUnique (Variables|Default|GettargetActors) newTarget)))

(fn RemoveTargetActor
  (params (removeTarget :type Actor%20Object%20Reference))
  (Utilities|Array|RemoveItem (Variables|Default|GettargetActors) removeTarget))

(fn RotateThisFrame
  (params (input :type Float%20%28double-precision%29))
  (Class|Actor|AddActorWorldRotation (Math|Rotator|MakeRotator 0.0 0.0 (* (Variables|Default|GetrotationalSpeed) (Utilities|Time|GetWorldDeltaSeconds) input))))

(fn IsinFOV
  (params (actorToCheck :type Actor%20Object%20Reference))
  (bind _returnvalue (Transformation|GetActorLocation actorToCheck))
  (bind _maincamera (Variables|Default|GetMainCamera))
  (bind _returnvalue_2 (Math|Vector|GetForwardVector _maincamera))
  (bind _returnvalue_3 (Transformation|GetWorldLocation _maincamera))
  (bind (_x _y) (Math|Vector|BreakVector _returnvalue_3))
  (bind _returnvalue_4 (Math|Vector|Normalize _returnvalue_2))
  (bind _returnvalue_5 (Math|Vector|MakeVector _x _y 0.0))
  (bind _returnvalue_6 (- _returnvalue _returnvalue_5))
  (bind _returnvalue_7 (Math|Vector|Normalize _returnvalue_6))
  (bind _returnvalue_8 (Math|Vector|DotProduct _returnvalue_4 _returnvalue_7))
  (bind _returnvalue_9 (Class|KismetMathLibrary|DegAcos _returnvalue_8))
  (return (>= (Variables|Default|GettrackedFOV) _returnvalue_9) _returnvalue_9))

(fn AutoZoom
  (params (deltaSeconds :type Float%20%28double-precision%29))
  (bind _maincamera (Variables|Default|GetMainCamera))
  (bind _relativelocation (Variables|/Script/Engine.SceneComponent|GetRelativeLocation _maincamera))
  (for _array_element (Variables|Default|GettargetActors)
    (bind (_isinfov _angle) (CallFunction|IsinFOV _array_element))
    (Variables|Default|SetFOVCheck (and (Variables|Default|GetFOVCheck) _isinfov))
    (Variables|Default|SetgreatestAngleThisFrame (Math|Float|Max(Float) (Variables|Default|GetgreatestAngleThisFrame) _angle)))
  (if (Utilities|NearTargetFOV)
    _
    (elif (Variables|Default|GetFOVCheck)
      (Variables|Default|SettargetDistance (Math|Float|Clamp(Float) (- (Variables|Default|GettargetDistance) 1e+01) 6.4e+02 5e+03))
      (else
        (Variables|Default|SettargetDistance (Math|Float|Clamp(Float) (+ (Variables|Default|GettargetDistance) 1e+01) 6.4e+02 5e+03))
        (Variables|Default|SetFOVCheck true))))
  (Transformation|SetRelativeLocation _maincamera (Math|Interpolation|VInterpTo _relativelocation (* (Math|Vector|Normalize _relativelocation) (Variables|Default|GettargetDistance)) deltaSeconds (Variables|Default|GetzoomSpeed)) false false)
  (Variables|Default|SetgreatestAngleThisFrame -1.0))

(fn UpdateTargetActors
  (bind _outactors (Actor|GetAllActorsOfClass "/Game/Programming/GM1/Blueprints/GM1/Player/Blueprints/BP_Player_GM1.BP_Player_GM1_C"))
  (bind _output_get (Variables|Default|SettargetActors _outactors))
  (for _array_element _output_get
    (Development|PrintString (Utilities|GetDisplayName _array_element) true true "(R=0.000000,G=0.660000,B=1.000000,A=1.000000)" 1e+01)))