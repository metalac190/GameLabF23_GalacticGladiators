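; Shared GM1 camera that frames all active players once GameStarted registers them as tracked targets and binds to their OnDie events.
; Each tick it lerps its Sphere toward the targets' average location plus padding.
; The largest pairwise target distance drives a clamped, lerped spring arm length for zoom.
; CameraData supplies tuning and starting FOV, arm length and transform; the old singleton camera manager is unused.
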(event EventBeginPlay
  (CallFunction|ApplyStartingValues))

(event EventTick
  (params (DeltaSeconds :type Float%20%28single-precision%29))
  (if (Variables|Default|GetbGameStarted)
    (CallFunction|CalculateCameraMovement false)
    (for (_array_element _array_index) (Variables|Targets|GetActive%20Targets)
      (Variables|Targets|SetTarget _array_element)
      (for _index (range (+ _array_index 1) (- (Utilities|Array|Length (Variables|Targets|GetActive%20Targets)) 1))
        (Utilities|Array|Add (Variables|Default|GetDistance) (Transformation|GetDistanceTo (Variables|Targets|GetTarget) (Utilities|Array|Get(acopy) (Variables|Targets|GetActive%20Targets) _index)))))
    (Utilities|SetLargestTargetArmLength)))

(fn ConstructionScript
  (CallFunction|ApplyStartingValues))

(fn GameStarted
  (params (ActivePlayers :type Array%20of%20BP%20Player%20GM1%20Object%20References))
  (for _array_element ActivePlayers
    (CallFunction|AddTrackedTarget _array_element)
    (Development|PrintString (Utilities|GetDisplayName _array_element)))
  (Variables|Default|SetbGameStarted true))

(fn CalculateCameraMovement
  (params (DrawDebug :type Boolean))
  (bind _returnvalue (Class|GameplayStatics|GetActorArrayAverageLocation (Variables|Targets|GetActive%20Targets)))
  (Transformation|SetWorldLocation (Variables|Default|GetSphere) (Math|Vector|Lerp(Vector) (Transformation|GetWorldLocation (Variables|Default|GetSphere)) (+ _returnvalue (Variables|/Game/Programming/GM1/Blueprints/Camera/Data/PDA_Camera_GM1.PDA_Camera_GM1_C|GetcameraPadding (Variables|Data|GetCameraData))) (Variables|/Game/Programming/GM1/Blueprints/Camera/Data/PDA_Camera_GM1.PDA_Camera_GM1_C|GetcameraLerpAlpha (Variables|Data|GetCameraData))) false false)
  (if DrawDebug
    (Rendering|Debug|DrawDebugSphere (Math|Vector|Lerp(Vector) (Transformation|GetWorldLocation (Variables|Default|GetSphere)) (+ _returnvalue (Variables|/Game/Programming/GM1/Blueprints/Camera/Data/PDA_Camera_GM1.PDA_Camera_GM1_C|GetcameraPadding (Variables|Data|GetCameraData))) (Variables|/Game/Programming/GM1/Blueprints/Camera/Data/PDA_Camera_GM1.PDA_Camera_GM1_C|GetcameraLerpAlpha (Variables|Data|GetCameraData))) 1e+01 12 "(R=1.000000,G=1.000000,B=1.000000,A=1.000000)" 0.0 5.0)))

(fn AddTrackedTarget
  (params (AddTarget :type Actor%20Object%20Reference))
  (Utilities|Array|AddUnique (Variables|Targets|GetActive%20Targets) AddTarget)
  (bind _asbp_player_gm1 (Utilities|Casting|CastToBP_Player_GM1 AddTarget))
  (EventDispatchers|BindEventtoOnDie _asbp_player_gm1 (EventDispatchers|CreateEvent :!event RemoveTrackedTarget)))

(fn RemoveTrackedTarget
  (params (RemoveTarget :type Actor%20Object%20Reference))
  (Utilities|Array|RemoveItem (Variables|Targets|GetActive%20Targets) RemoveTarget)
  (bind _asbp_player_gm1 (Utilities|Casting|CastToBP_Player_GM1 RemoveTarget))
  (EventDispatchers|UnbindEventfromOnDie _asbp_player_gm1 (EventDispatchers|CreateEvent :!event RemoveTrackedTarget)))

(fn ApplyStartingValues
  (bind _cameradata (Variables|Data|GetCameraData))
  (Camera|SetFieldOfView (Variables|Default|GetCamera) (Variables|/Game/Programming/GM1/Blueprints/Camera/Data/PDA_Camera_GM1.PDA_Camera_GM1_C|GetcameraFOV (Variables|Data|GetCameraData)))
  (Variables|/Script/Engine.SpringArmComponent|SetTargetArmLength (Variables|Default|GetSpringArm) (Variables|/Game/Programming/GM1/Blueprints/Camera/Data/PDA_Camera_GM1.PDA_Camera_GM1_C|GetstartArmLength _cameradata))
  (Transformation|SetActorTransform (Variables|/Game/Programming/GM1/Blueprints/Camera/Data/PDA_Camera_GM1.PDA_Camera_GM1_C|GetstartTransform _cameradata)))

(fn CopyStartingValues
  (bind _cameradata (Variables|Data|GetCameraData))
  (Variables|/Game/Programming/GM1/Blueprints/Camera/Data/PDA_Camera_GM1.PDA_Camera_GM1_C|SetcameraFOV (Variables|Data|GetCameraData) (Variables|/Script/Engine.CameraComponent|GetFieldOfView (Variables|Default|GetCamera)))
  (Variables|/Game/Programming/GM1/Blueprints/Camera/Data/PDA_Camera_GM1.PDA_Camera_GM1_C|SetstartArmLength _cameradata (Variables|/Script/Engine.SpringArmComponent|GetTargetArmLength (Variables|Default|GetSpringArm)))
  (Variables|/Game/Programming/GM1/Blueprints/Camera/Data/PDA_Camera_GM1.PDA_Camera_GM1_C|SetstartTransform _cameradata (Transformation|GetActorTransform)))