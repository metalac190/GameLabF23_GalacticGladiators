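; BP_GM1_AudioDataTracker tracks per-clip cooldowns for audio, gating how often a named clip may trigger.
; A Clips map keys each clip name to a cooldown and last timestamp.
; Update returns true and stores the passed-in time once the cooldown has elapsed, and returns false for early or unknown clips.
; Reset rewrites every timestamp with a value derived from that clip's cooldown.
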(fn Update
  (params (Clip%20Name :type E_GM1_AudioClips%20Enum :default "NewEnumerator0") (Time :type Float%20%28double-precision%29))
  (bind _clips (Variables|Default|GetClips))
  (bind (_value _returnvalue) (Utilities|Map|Find _clips Clip%20Name))
  (bind (_cooldown _timestamp) (Utilities|Struct|BreakBS_GM1_AudioData _value))
  (if _returnvalue
    (if (>= (- Time _timestamp) _cooldown)
      (Utilities|Map|Add (Variables|Default|GetClips) Clip%20Name (Utilities|Struct|MakeBS_GM1_AudioData _cooldown Time))
      (return true)
      (else
        (return false)))
    (else
      (return false))))

(fn Reset
  (bind _keys (Utilities|Map|Keys (Variables|Default|GetClips)))
  (for _array_element _keys
    (bind _result (Math|Float|NegateFloat (.Cooldown (Utilities|Struct|BreakBS_GM1_AudioData (.Value (Utilities|Map|Find (Variables|Default|GetClips) _array_element)))))
      (:%20%20
        (Utilities|Map|Add (Variables|Default|GetClips) _array_element (Utilities|Struct|MakeBS_GM1_AudioData (.Cooldown (Utilities|Struct|BreakBS_GM1_AudioData (.Value (Utilities|Map|Find (Variables|Default|GetClips) _array_element)))) _result))))))