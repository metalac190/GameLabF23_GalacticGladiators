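; Hardpoint zone for GM1 that repeatedly appears at an area-uniform random point inside the arena once the game starts.
; Three chained timelines scale it through spawn, countdown and end phases, while the main camera tracks it from countdown onward.
; Overlapping players tint their dynamic material parameter until the countdown finishes and locks occupancy.
; At round end it broadcasts MaxScore split among occupants, hides, then restarts after a delay.
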(event OnComponentBeginOverlap(Cylinder)
  (params (OverlappedComponent :type Primitive%20Component%20Object%20Reference) (OtherActor :type Actor%20Object%20Reference) (OtherComp :type Primitive%20Component%20Object%20Reference) (OtherBodyIndex :type Integer) (bFromSweep :type Boolean) (SweepResult :type Hit%20Result%20Structure%20%28by%20ref%29))
  ;[0 0 0] Player Overlap
  (if (Utilities|Enum|Equal(Enum) (Variables|Default|GetState) "NewEnumerator0")
    (bind _asbp_player_gm1 (Utilities|Casting|CastToBP_Player_GM1 OtherActor))
    (Utilities|Array|AddUnique (Variables|Default|GetPlayersInZone) _asbp_player_gm1)
    (Rendering|Material|SetVectorParameterValue (Variables|Default|GetMaterial) (Utilities|Array|Get(acopy) (Variables|Default|GetParamNameArray) (Variables|/Game/Programming/GM1/Blueprints/Player/Blueprints/BP_Player_GM1.BP_Player_GM1_C|GetIndex _asbp_player_gm1)) (Utilities|Array|Get(acopy) (Variables|Default|GetCharacterColors) (Variables|/Game/Programming/GM1/Blueprints/Player/Blueprints/BP_Player_GM1.BP_Player_GM1_C|GetIndex _asbp_player_gm1)) :!class /Script/Engine.MaterialInstanceDynamic)))

(event OnComponentEndOverlap(Cylinder)
  (params (OverlappedComponent :type Primitive%20Component%20Object%20Reference) (OtherActor :type Actor%20Object%20Reference) (OtherComp :type Primitive%20Component%20Object%20Reference) (OtherBodyIndex :type Integer))
  ;[0 0 0] Player Overlap
  (if (Utilities|Enum|Equal(Enum) (Variables|Default|GetState) "NewEnumerator0")
    (bind _asbp_player_gm1 (Utilities|Casting|CastToBP_Player_GM1 OtherActor))
    (Utilities|Array|RemoveItem (Variables|Default|GetPlayersInZone) _asbp_player_gm1)
    (Rendering|Material|SetVectorParameterValue (Variables|Default|GetMaterial) (Utilities|Array|Get(acopy) (Variables|Default|GetParamNameArray) (Variables|/Game/Programming/GM1/Blueprints/Player/Blueprints/BP_Player_GM1.BP_Player_GM1_C|GetIndex _asbp_player_gm1)) "(R=1.000000,G=1.000000,B=1.000000,A=1.000000)" :!class /Script/Engine.MaterialInstanceDynamic)))

(event Custom|Start%20Zone%20Timer
  (bind _arena (Variables|Default|GetArena))
  (bind _defaultsceneroot (Variables|Default|GetDefaultSceneRoot))
  (bind _staticmeshcomponent (Variables|/Script/Engine.StaticMeshActor|GetStaticMeshComponent _arena))
  (bind (_origin _boxextent) (Collision|GetComponentBounds _staticmeshcomponent))
  ;[0 0 0] Start of Zone Timer
  (bind _asgm_gm1 (Utilities|Casting|CastToGM_GM1 (Game|GetGameMode)))
  (if (Variables|/Game/Programming/GM1/Blueprints/Systems/GM_GM1.GM_GM1_C|GetisInGame _asgm_gm1)
    (if (Variables|Default|GetisDebug)
      (CallFunction|DebugDraws))
    (Default|CallEDStartZone (Variables|Default|GetMaxTime))
    (bind (_x _y) (CallFunction|RandomPointinCircle (- (.x _boxextent) (Variables|Default|GetZoneExtent)) (.x _origin) (.y _origin)))
    (Transformation|SetWorldLocation _defaultsceneroot (Math|Vector|MakeVector _x _y (.z (Transformation|GetWorldLocation (Variables|Default|GetCylinder)))) false false)
    (Variables|Default|SetState "NewEnumerator0")
    (CallFunction|ResetColors)
    (Rendering|SetVisibility _defaultsceneroot true true)
    (bind _alpha (Timeline|Spawn%20Hardpoint PlayFromStart)
      (:Update
        (Transformation|SetWorldScale3D (Variables|Default|GetDefaultSceneRoot) (Math|Vector|MakeVector (Math|Float|Lerp 0.0 1.0 _alpha) (Math|Float|Lerp 0.0 1.0 _alpha) 0.0)))
      (:Finished
        (Audio|PlaySound2D "/Game/Audio/Placeholder/countdown_timer_10_to_0.countdown_timer_10_to_0" 0.5 1.0 0.0 0 0)
        (for _array_element (Variables|Default|GetPlayersInZone)
          (Rendering|Material|SetVectorParameterValue (Variables|Default|GetMaterial) (Utilities|Array|Get(acopy) (Variables|Default|GetParamNameArray) (Variables|/Game/Programming/GM1/Blueprints/Player/Blueprints/BP_Player_GM1.BP_Player_GM1_C|GetIndex _array_element)) (Utilities|Array|Get(acopy) (Variables|Default|GetCharacterColors) (Variables|/Game/Programming/GM1/Blueprints/Player/Blueprints/BP_Player_GM1.BP_Player_GM1_C|GetIndex _array_element)) :!class /Script/Engine.MaterialInstanceDynamic))
        (Default|AddTrackedTarget (Variables|Default|GetMainCamera) self)
        (bind _alpha_2 (Timeline|Timer PlayFromStart)
          (:Update
            (Transformation|SetWorldScale3D (Variables|Default|GetDefaultSceneRoot) (Math|Vector|MakeVector (Math|Float|Lerp 0.0 1.0 _alpha_2) (Math|Float|Lerp 0.0 1.0 _alpha_2) 0.0)))
          (:Finished
            (Variables|Default|SetState "NewEnumerator1")
            (bind _alpha_3 (Timeline|End%20Timer PlayFromStart)
              (:Update
                (Transformation|SetWorldScale3D (Variables|Default|GetDefaultSceneRoot) (Math|Vector|MakeVector (Math|Float|Lerp 0.0 1.0 _alpha_3) (Math|Float|Lerp 0.0 1.0 _alpha_3) 0.0)))
              (:Finished
                (CallFunction|EndZoneTimer)))))))))

(event Custom|End%20Zone%20Timer
  (bind _indexofplayers (Variables|Default|GetIndexOfPlayers))
  (bind _playersinzone (Variables|Default|GetPlayersInZone))
  (bind _maxscore (Variables|Default|GetMaxScore))
  (bind _returnvalue (Utilities|Array|Length _playersinzone))
  (bind _returnvalue_2 (/ _maxscore _returnvalue))
  ;[0 0 0] End of Zone Timer
  (if (Variables|Default|GetisDebug)
    (CallFunction|DebugDraws))
  (Rendering|SetVisibility (Variables|Default|GetDefaultSceneRoot) false true)
  (for _array_element _playersinzone
    (Development|PrintString (Utilities|String|Append "Player " (Utilities|String|ToString(Integer) (+ (Variables|/Game/Programming/GM1/Blueprints/Player/Blueprints/BP_Player_GM1.BP_Player_GM1_C|GetIndex _array_element) 1)) " Gained " (Utilities|String|ToString(Integer) _returnvalue_2) " Score!"))
    (Utilities|Array|Add (Variables|Default|GetIndexOfPlayers) (Variables|/Game/Programming/GM1/Blueprints/Player/Blueprints/BP_Player_GM1.BP_Player_GM1_C|GetIndex _array_element)))
  (Default|CallEDEndZone _returnvalue_2 _indexofplayers)
  (Utilities|Array|Clear _indexofplayers)
  (for _array_element_2 (Variables|Default|GetParamNameArray)
    (Rendering|Material|SetVectorParameterValue (Variables|Default|GetMaterial) _array_element_2 "(R=1.000000,G=1.000000,B=1.000000,A=1.000000)" :!class /Script/Engine.MaterialInstanceDynamic))
  (Default|RemoveTrackedTarget (Variables|Default|GetMainCamera) self)
  (Utilities|FlowControl|Delay (Variables|Default|GetDelayBetweenRounds))
  (CallFunction|StartZoneTimer))

(event Custom|Start%20Game
  ;[0 0 0] Begin Play and Bind Event
  (Utilities|FlowControl|Delay (Variables|Default|GetInitialDelay))
  (CallFunction|StartZoneTimer)
  (bind _foundwidgets (Widget|GetAllWidgetsOfClass "/Game/Programming/GM1/Blueprints/WBP_GM1_Hardpoint.WBP_GM1_Hardpoint_C" true))
  (Variables|Default|SetHardpointWidget (Utilities|Array|Get(acopy) _foundwidgets)))

(event Custom|Reset%20Colors
  ;[1 1 1] Reset Colors
  (Utilities|Array|Clear (Variables|Default|GetPlayersInZone))
  (Rendering|Material|SetVectorParameterValue (Variables|Default|GetMaterial) "None" "(R=1.000000,G=1.000000,B=1.000000,A=1.000000)" :!class /Script/Engine.MaterialInstanceDynamic))

(event EventBeginPlay
  ;[0 0 0] Begin Play and Bind Event
  (EventDispatchers|BindEventtoOnStartGame (.AsGM%20GM1 (Utilities|Casting|CastToGM_GM1 (Game|GetGameMode))) (delegate Custom|Start%20Game))
  (Rendering|SetVisibility (Variables|Default|GetDefaultSceneRoot) false true)
  (bind _returnvalue (Actor|GetActorOfClass "/Game/Programming/GM1/Blueprints/Camera/CM_GM1.CM_GM1_C"))
  (Variables|Default|SetMainCamera _returnvalue)
  ;[1 1 1] blegh
  (Variables|Default|SetZoneExtent (* (.x (.boxextent (StaticMesh|GetBounds (Variables|/Script/Engine.StaticMeshComponent|GetStaticMesh (Variables|Default|GetCylinder))))) (.x (Transformation|GetWorldScale (Variables|Default|GetCylinder))) (.x (Transformation|GetWorldScale (Variables|Default|GetDefaultSceneRoot))))))

(fn ConstructionScript
  (bind _charactercolors (Variables|Default|GetCharacterColors))
  (bind _cylinder (Variables|Default|GetCylinder))
  ;[0 0 0] Allows Change in Material
  (bind _returnvalue (Rendering|Material|CreateDynamicMaterialInstance _cylinder 0 (Rendering|Material|GetMaterial _cylinder 0) "None" :!class /Script/Engine.PrimitiveComponent))
  (bind _output_get (Variables|Default|SetMaterial _returnvalue))
  (Rendering|Material|SetMaterial _cylinder 0 _output_get)
  (Utilities|FlowControl|Sequence
    (:then_0
      (bind _returnvalue_2 (Rendering|Material|GetVectorParameterValue _returnvalue "Player1_Color" :!class /Script/Engine.MaterialInstanceDynamic))
      (Utilities|Array|Add _charactercolors _returnvalue_2)
      (bind _returnvalue_3 (Rendering|Material|GetVectorParameterValue _returnvalue "Player2_Color" :!class /Script/Engine.MaterialInstanceDynamic))
      (Utilities|Array|Add _charactercolors _returnvalue_3)
      (bind _returnvalue_4 (Rendering|Material|GetVectorParameterValue _returnvalue "Player3_Color" :!class /Script/Engine.MaterialInstanceDynamic))
      (Utilities|Array|Add _charactercolors _returnvalue_4)
      (bind _returnvalue_5 (Rendering|Material|GetVectorParameterValue _returnvalue "Player4_Color" :!class /Script/Engine.MaterialInstanceDynamic))
      (Utilities|Array|Add _charactercolors _returnvalue_5))
    (:then_1
      (Rendering|Material|SetVectorParameterValue _returnvalue "Player1_Color" "(R=1.000000,G=1.000000,B=1.000000,A=1.000000)" :!class /Script/Engine.MaterialInstanceDynamic)
      (Rendering|Material|SetVectorParameterValue _returnvalue "Player2_Color" "(R=1.000000,G=1.000000,B=1.000000,A=1.000000)" :!class /Script/Engine.MaterialInstanceDynamic)
      (Rendering|Material|SetVectorParameterValue _returnvalue "Player3_Color" "(R=1.000000,G=1.000000,B=1.000000,A=1.000000)" :!class /Script/Engine.MaterialInstanceDynamic)
      (Rendering|Material|SetVectorParameterValue _returnvalue "Player4_Color" "(R=1.000000,G=1.000000,B=1.000000,A=1.000000)" :!class /Script/Engine.MaterialInstanceDynamic))))

(fn DebugDraws
  (bind _arena (Variables|Default|GetArena))
  (bind _cylinder (Variables|Default|GetCylinder))
  (bind _origin (Collision|GetComponentBounds _cylinder))
  (bind _staticmeshcomponent (Variables|/Script/Engine.StaticMeshActor|GetStaticMeshComponent _arena))
  (bind _boxextent (Collision|GetComponentBounds _staticmeshcomponent))
  (bind _origin_2 (Collision|GetComponentBounds _staticmeshcomponent))
  ;[0 0 0] Zone Rings
  (Rendering|Debug|DrawDebugCircle (Math|Vector|MakeVector (.x _origin) (.y _origin) 24.0) (/ (Variables|Default|GetZoneExtent) 5.0) 72 "(R=1.000000,G=1.000000,B=1.000000,A=1.000000)" 15.0 2.0 "0.000000,1.000000,0.000000" "1.000000,0.000000,0.000000")
  ;[0 0 0] Outer and Inner Ring
  (Utilities|FlowControl|DoOnce false
    (:Completed
      (Rendering|Debug|DrawDebugCircle (Math|Vector|MakeVector (.x _origin_2) (.y _origin_2) 24.0) (.x _boxextent) 108 "(R=1.000000,G=0.000000,B=0.217428,A=1.000000)" 1.2e+02 5.0 "0.000000,1.000000,0.000000" "1.000000,0.000000,0.000000")
      (Rendering|Debug|DrawDebugCircle (Math|Vector|MakeVector (.x _origin_2) (.y _origin_2) 24.0) (- (.x _boxextent) (Variables|Default|GetZoneExtent)) 108 "(R=0.000000,G=0.001776,B=1.000000,A=1.000000)" 1.2e+02 5.0 "0.000000,1.000000,0.000000" "1.000000,0.000000,0.000000"))))

(fn RandomPointinCircle
  (params (Radius :type Float%20%28double-precision%29) (OriginX :type Float%20%28double-precision%29) (OriginY :type Float%20%28double-precision%29))
  ;[0 0 0] Distance from Origin
  (LocalVariables|Setr (* Radius (Math|Float|Sqrt (Math|Random|RandomFloat))))
  ;[0 0 0] Angle
  (LocalVariables|Settheta (* (Math|Random|RandomFloat) 2.0 (Math|Trig|GetPI)))
  (return (+ OriginX (* (LocalVariables|Getr) (Math|Trig|Cos(Radians) (LocalVariables|Gettheta)))) (+ OriginY (* (LocalVariables|Getr) (Math|Trig|Sin(Radians) (LocalVariables|Gettheta))))))