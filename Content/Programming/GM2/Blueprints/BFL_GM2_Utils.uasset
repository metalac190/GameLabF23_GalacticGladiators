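; BFL_GM2_Utils is a library of small gameplay helper functions for GM2.
; SetActive toggles an actor's collision and visibility together, without touching its tick.
; The velocity helpers scale a collider's linear or angular physics velocity, either replacing or adding to the current value.
; The SFX helpers look up a cue in SoundAtlas and, if valid, play it in 2D or at a location.
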(fn SetActive
  (params (target :type Actor%20Object%20Reference) (active :type Boolean))
  (Collision|SetActorEnableCollision target active)
  (Rendering|SetActorHiddenInGame target (not active)))

(fn MultiplyLinearVelocity
  (params (Collider :type Capsule%20Component%20Object%20Reference) (Multiplier :type Float%20%28double-precision%29) (Add%20to%20Current :type Boolean))
  (bind _returnvalue (Physics|GetPhysicsLinearVelocity Collider "None"))
  (Physics|SetPhysicsLinearVelocity Collider (* _returnvalue Multiplier) Add%20to%20Current "None"))

(fn MultiplyAngularVelocity
  (params (Collider :type Capsule%20Component%20Object%20Reference) (Multiplier :type Float%20%28double-precision%29) (Add%20to%20Current :type Boolean))
  (Class|PrimitiveComponent|SetAllPhysicsAngularVelocityinDegrees Collider (* (Physics|GetPhysicsAngularVelocityinDegrees Collider "None") Multiplier) Add%20to%20Current))

(fn Play2DSFX
  (params (Sound%20Cue%20Name :type E_GM2_AudioClips%20Enum :default "NewEnumerator0"))
  (bind _sound_cue (Default|GetSoundCue (LocalVariables|GetSound%20Atlas) Sound%20Cue%20Name))
  (Utilities|IsValid _sound_cue
    (:Is%20Valid
      (Audio|PlaySound2D 0 _sound_cue 1.0 1.0 0.0 0 0))))

(fn Play3DSFX
  (params (Sound%20Cue :type E_GM2_AudioClips%20Enum :default "NewEnumerator0") (Location :type Vector) (Rotation :type Rotator))
  (bind _sound_cue (Default|GetSoundCue (LocalVariables|GetSound%20Atlas) Sound%20Cue))
  (Utilities|IsValid _sound_cue
    (:Is%20Valid
      (Audio|PlaySoundatLocation 0 _sound_cue Location Rotation 1.0 1.0 0.0 0 0 0 0))))