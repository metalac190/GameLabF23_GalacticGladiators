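; HUD_GM2 is the GM2 game mode HUD that spawns global and player UI widgets and connects players to them.
; Initialize creates and shows one widget per configured class, sending InitializeMessage to each and an argument-less AddPlayerMessage to global ones.
; Only player widgets are stored in UIInstances.
; AddPlayer forwards the given player to those stored widgets, so they are shared instances rather than created per player.
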(event Custom|Add%20Player
  (params (Player :type PC%20GM2%20Player%20Object%20Reference))
  ;[1 1 1] Connect Player to HUD
  (for _array_element (Variables|Default|Get_UI_Instances)
    (Class|BIGM2PlayerUI|AddPlayer(Message) _array_element Player)))

(event Custom|Initialize
  ;[1 1 1] Initialize and Show Global HUD
  (for _array_element (Variables|Default|GetGlobal%20UI%20Types)
    (bind _returnvalue (UserInterface|CreateWidget _array_element))
    (UserInterface|Viewport|AddtoViewport _returnvalue 0)
    (Class|BIGM2PlayerUI|Initialize(Message) _returnvalue)
    (Class|BIGM2PlayerUI|AddPlayer(Message) _returnvalue))
  ;[1 1 1] Initialize and Player HUD
  (for _array_element_2 (Variables|Default|GetPlayer%20UI%20Types)
    (bind _returnvalue_2 (UserInterface|CreateWidget _array_element_2))
    (UserInterface|Viewport|AddtoViewport _returnvalue_2 0)
    (Utilities|Array|Add (Variables|Default|Get_UI_Instances) _returnvalue_2)
    (Class|BIGM2PlayerUI|Initialize(Message) _returnvalue_2)))

(fn ConstructionScript)