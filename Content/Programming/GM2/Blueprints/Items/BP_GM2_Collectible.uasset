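; BP_GM2_Collectible is a pickup actor that reacts when a PC_GM2_Player overlaps its trigger.
; Collected receives the player but only plays the collect sound and optional Niagara effect at the actor's transform.
; Depending on DestroyOnPickup, the actor then either destroys itself and its idle VFX, or disables itself via SetActive and reactivates after a delay with a respawn sound.
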(event OnComponentBeginOverlap(Trigger)
  (params (OverlappedComponent :type Primitive%20Component%20Object%20Reference) (OtherActor :type Actor%20Object%20Reference) (OtherComp :type Primitive%20Component%20Object%20Reference) (OtherBodyIndex :type Integer) (bFromSweep :type Boolean) (SweepResult :type Hit%20Result%20Structure%20%28by%20ref%29))
  (bind _aspc_gm2_player (Utilities|Casting|CastToPC_GM2_Player OtherActor))
  (Development|PrintString "Collected item")
  (CallFunction|Collected _aspc_gm2_player)
  (if (Variables|Default|GetDestroyOnPickup)
    ;[1 1 1] Destroy Collectible
    (Actor|DestroyActor)
    (bind _idle_vfx (Variables|Default|GetIdle%20VFX)
      (:then
        (Components|DestroyComponent _idle_vfx))
      (:else))
    (else
      ;[1 1 1] Temporarily Disable Collectible
      (CallFunction|SetActive self false)
      (Utilities|FlowControl|Delay (Variables|Default|GetTemporaryDisableOnPickup))
      (CallFunction|SetActive self true)
      (Audio|PlaySoundatLocation (Variables|Default|GetSFX_Respawn) (Transformation|GetActorLocation) "0, 0, 0" 1.0 1.0 0.0 0 0 0 0))))

(fn ConstructionScript)

(fn Collected
  (params (Player :type PC%20GM2%20Player%20Object%20Reference))
  (bind _returnvalue (Transformation|GetActorTransform))
  (bind (_location _rotation _scale) (Math|Transform|BreakTransform _returnvalue))
  (Audio|PlaySoundatLocation (Variables|Default|GetSFX_Collect) _location "0, 0, 0" 1.2 1.0 0.0 0 0 0 0)
  (bind _vfx_collect (Variables|Default|GetVFX_Collect)
    (:then
      (Niagara|SpawnSystematLocation _vfx_collect _location _rotation _scale))
    (:else)))