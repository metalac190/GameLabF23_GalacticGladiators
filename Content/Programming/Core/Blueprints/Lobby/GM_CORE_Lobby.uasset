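; Lobby game mode that spawns input pawns on BeginPlay and validates joined players before starting the game.
; TryGameStart counts connected players in the game instance (currently passing with just one) and rejects duplicate player models by comparing enum values as integers.
; OpenNextLevel then loads a random one of two game-mode pre-game screens in Tournament Mode, or LevelSelect otherwise.
; Several disconnected earlier attempts at these checks remain in the event graph.
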(event Custom|Try%20Game%20Start
  (bind _currentgameinstance (Variables|Default|GetCurrentGameInstance))
  (bind _currentgameinstance_2 (Variables|Default|GetCurrentGameInstance))
  (bind _playerdata (Variables|/Game/Programming/Core/Blueprints/GameInstance/GI_CORE_GameInstance.GI_CORE_GameInstance_C|GetPlayerData _currentgameinstance))
  (Development|PrintString "GM: Try Game Start")
  ;[0 0 0] Check if more than one player has joined
  (Variables|Local|SetPlayerCount 0)
  (for _array_element (Variables|/Game/Programming/Core/Blueprints/GameInstance/GI_CORE_GameInstance.GI_CORE_GameInstance_C|GetPlayerData (Variables|Default|GetCurrentGameInstance))
    (if (.PlayerConnected (Utilities|Struct|BreakBP_PlayerData _array_element))
      (Math|Integer|IncrementInt (Variables|Local|GetPlayerCount))))
  (if (> (Variables|Local|GetPlayerCount) 0)
    ;[0 0 0] Check players dont have the same models
    (Variables|Local|SetSameModel false)
    (for (_array_element_2 _array_index) _playerdata
      (for (_array_element_3 _array_index_2) _playerdata
        (bind _int (Default|GetIntfromEnum _currentgameinstance_2 (.PlayerModel (Utilities|Struct|BreakBP_PlayerData _array_element_2))))
        (bind _int_2 (Default|GetIntfromEnum _currentgameinstance_2 (.PlayerModel (Utilities|Struct|BreakBP_PlayerData _array_element_3))))
        (if (Math|Boolean|ANDBoolean (and (.PlayerConnected (Utilities|Struct|BreakBP_PlayerData _array_element_2)) (.PlayerConnected (Utilities|Struct|BreakBP_PlayerData _array_element_3))) (== _int _int_2) (!= _array_index _array_index_2)) ; If any have same model set to true
          (Variables|Local|SetSameModel true))))
    (if (Variables|Local|GetSameModel) ; After loop check if any were same
      (Development|PrintString "players cannot have the same model")
      (else
        (Development|PrintString "CheckSuccessful")
        (CallFunction|OpenNextLevel)))
    (else
      (Development|PrintText "Requires more than one player to start"))))

(event EventBeginPlay
  (CallFunction|SpawnInputPawns))

(fn ConstructionScript)

(fn OpenNextLevel
  (if (Variables|/Game/Programming/Core/Blueprints/GameInstance/PDA_GameInstanceSettings.PDA_GameInstanceSettings_C|GetTournamentMode (Variables|/Game/Programming/Core/Blueprints/GameInstance/GI_CORE_GameInstance.GI_CORE_GameInstance_C|GetGameInstanceVariables (Variables|Default|GetCurrentGameInstance)))
    (Development|PrintText (Utilities|Text|FormatText "The Game is in Tournament Mode: {TournamentMode}" 0) true true "(R=1.000000,G=0.202734,B=0.586872,A=1.000000)")
    ;[1 1 1] Tournament
    (if (Math|Random|RandomBool)
      ;;[1 1 1] Starts With GameMode 1
      (Development|PrintString "Starting with GameMode 1")
      (Game|OpenLevel(byObjectReference) "/Game/Programming/Core/Levels/GM1_PreGameScreen.GM1_PreGameScreen")
      (else
        ;;[1 1 1] Starts with GameMode 2
        (Development|PrintString "Starting with GameMode 2")
        (Game|OpenLevel(byObjectReference) "/Game/Programming/Core/Levels/GM2_PreGameScreen.GM2_PreGameScreen")))
    (else
      (Game|OpenLevel(byObjectReference) "/Game/Programming/Core/Levels/LevelSelect.LevelSelect"))))