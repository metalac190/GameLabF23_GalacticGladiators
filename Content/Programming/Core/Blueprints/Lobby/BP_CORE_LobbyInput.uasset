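; BP_CORE_LobbyInput handles lobby input for the player identified by PlayerID.
; On BeginPlay it caches the lobby menu widget and the lobby GameMode.
; Join and leave actions check the GameInstance's connected state before updating it and notifying the widget.
; Next-select triggers a widget color change, start asks the GameMode to try starting the game, and back opens the main menu.
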(event Input|EnhancedActionEvents|EnhancedInputActionIA_CORE_Join
  (params (ActionValue :type Boolean) (ElapsedSeconds :type Float%20%28double-precision%29) (TriggeredSeconds :type Float%20%28double-precision%29) (InputAction :type Input%20Action%20Object%20Reference :default "/Game/Programming/Core/Input/LobbyInput/IA_CORE_Join.IA_CORE_Join"))
  (bind _playerid (Variables|Default|GetPlayerID))
  (:Started
    ;[0 0 0] Player Joining Lobby (if GI says not joined)
    (bind _connected (Default|GetPlayerConnected (Variables|/Game/Programming/Core/Blueprints/BaseClasses/GM_Core_NoPlayerControllerInput.GM_Core_NoPlayerControllerInput_C|GetCurrentGameInstance (Variables|Default|GetGM)) (Variables|Default|GetPlayerID)))
    (if (not _connected)
      (Default|PlayerJoinedEvent (Variables|Default|GetLobbyWidget) (Variables|Default|GetPlayerID))
      (Default|SetPlayerConnected (Variables|/Game/Programming/Core/Blueprints/BaseClasses/GM_Core_NoPlayerControllerInput.GM_Core_NoPlayerControllerInput_C|GetCurrentGameInstance (Variables|Default|GetGM)) _playerid true)
      ;[1 1 1] Debug
      (Development|PrintText (Utilities|Text|FormatText "BP: Player Joined {0}" _playerid)))))

(event Input|EnhancedActionEvents|EnhancedInputActionIA_CORE_Start
  (params (ActionValue :type Boolean) (ElapsedSeconds :type Float%20%28double-precision%29) (TriggeredSeconds :type Float%20%28double-precision%29) (InputAction :type Input%20Action%20Object%20Reference :default "/Game/Programming/Core/Input/LobbyInput/IA_CORE_Start.IA_CORE_Start"))
  (:Started
    ;[0 0 0] Players Press Enter to Continue Game
    (Default|TryGameStart (Variables|Default|GetGM))))

(event Input|EnhancedActionEvents|EnhancedInputActionIA_CORE_NextSelect
  (params (ActionValue :type Boolean) (ElapsedSeconds :type Float%20%28double-precision%29) (TriggeredSeconds :type Float%20%28double-precision%29) (InputAction :type Input%20Action%20Object%20Reference :default "/Game/Programming/Core/Input/LobbyInput/IA_CORE_NextSelect.IA_CORE_NextSelect"))
  (:Started
    ;[0 0 0] Trigger Color Change
    (Default|SelectNextEvent (Variables|Default|GetLobbyWidget) (Variables|Default|GetPlayerID))))

(event Input|EnhancedActionEvents|EnhancedInputActionIA_CORE_Leave
  (params (ActionValue :type Boolean) (ElapsedSeconds :type Float%20%28double-precision%29) (TriggeredSeconds :type Float%20%28double-precision%29) (InputAction :type Input%20Action%20Object%20Reference :default "/Game/Programming/Core/Input/LobbyInput/IA_CORE_Leave.IA_CORE_Leave"))
  (bind _playerid (Variables|Default|GetPlayerID))
  (:Started
    ;[0 0 0] Player Leaving Lobby
    (bind _connected (Default|GetPlayerConnected (Variables|/Game/Programming/Core/Blueprints/BaseClasses/GM_Core_NoPlayerControllerInput.GM_Core_NoPlayerControllerInput_C|GetCurrentGameInstance (Variables|Default|GetGM)) (Variables|Default|GetPlayerID)))
    (if _connected
      (Default|PlayerLeftEvent (Variables|Default|GetLobbyWidget) (Variables|Default|GetPlayerID))
      (Default|SetPlayerConnected (Variables|/Game/Programming/Core/Blueprints/BaseClasses/GM_Core_NoPlayerControllerInput.GM_Core_NoPlayerControllerInput_C|GetCurrentGameInstance (Variables|Default|GetGM)) _playerid false)
      ;[1 1 1] Debug
      (Development|PrintText (Utilities|Text|FormatText "BP: Player Left {0}" _playerid)))))

(event Input|EnhancedActionEvents|EnhancedInputActionIA_Core_Back
  (params (ActionValue :type Boolean) (ElapsedSeconds :type Float%20%28double-precision%29) (TriggeredSeconds :type Float%20%28double-precision%29) (InputAction :type Input%20Action%20Object%20Reference :default "/Game/Programming/Core/Input/LobbyInput/IA_Core_Back.IA_Core_Back"))
  (:Started
    (Game|OpenLevel(byObjectReference) "/Game/Programming/Core/Levels/MainMenu.MainMenu")))

(event EventBeginPlay
  ;[0 0 0] Get Lobby Widget
  (bind _foundwidgets (Widget|GetAllWidgetsOfClass "/Game/Programming/Core/Widgets/Lobby/WBP_CORE_LobbyMenu.WBP_CORE_LobbyMenu_C" true))
  (Variables|Default|SetLobbyWidget (Utilities|Array|Get(acopy) _foundwidgets))
  ;[0 0 0] Set GameMode Variable
  (bind _asgm_core_lobby (Utilities|Casting|CastToGM_CORE_Lobby (Game|GetGameMode)))
  (Variables|Default|SetGM _asgm_core_lobby))

(fn ConstructionScript)