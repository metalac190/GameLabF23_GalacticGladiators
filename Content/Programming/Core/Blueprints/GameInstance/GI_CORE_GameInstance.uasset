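; Game Instance that holds per-player data and tournament state for a multiplayer game.
; An indexed PlayerData struct array stores each player's connection, name, model and score, exposed through getter and setter functions, with enum-to-index conversion for models.
; A GameInstanceVariables struct tracks games played against an adjustable, minimum-clamped limit to decide whether a tournament continues.
; Returning to the main menu disconnects players and resets tournament progress, leaving scores untouched.
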(event EventInit)

(fn GetPlayerModel
  (params (InputInt :type Integer))
  (return (.playermodel (Utilities|Array|Get(acopy) (Variables|Main|GetPlayerData) InputInt))))

(fn GetPlayerConnected
  (params (PlayerID :type Integer))
  (return (.playerconnected (Utilities|Array|Get(acopy) (Variables|Main|GetPlayerData) PlayerID))))

(fn SetPlayerConnected
  (params (PlayerID :type Integer) (Connected :type Boolean))
  (|SetBy-RefVar (.playerconnected (Utilities|Array|Get(acopy) (Variables|Main|GetPlayerData) PlayerID)) Connected)
  (return))

(fn HasPlayers
  (bind _playerdata (Variables|Main|GetPlayerData))
  (if (!= (Utilities|Array|Length _playerdata) 0)
    (for _array_element _playerdata
      (if (.PlayerConnected (Utilities|Struct|BreakBP_PlayerData _array_element))
        ;[1 1 1] A player is connected
        (return true)))
    ;[1 1 1] No player is connected
    (return false)
    (else
      ;[1 1 1] No players collected
      (return false))))

(fn GetPlayerData
  (params (ID :type Integer))
  (bind _playerdata (Variables|Main|GetPlayerData))
  (if (< ID (Utilities|Array|Length _playerdata))
    (return (Utilities|Array|Get(acopy) _playerdata ID))))

(fn GetPlayerScore
  (params (ID :type Integer))
  (bind _playerdata (Variables|Main|GetPlayerData))
  (bind _output (Utilities|Array|Get(acopy) _playerdata ID))
  (Development|PrintString (.playername _output))
  (return (.playerscore _output)))

(fn GetEnumfromInt
  (params (int :type Integer))
  (return (Utilities|Array|Get(acopy) (Variables|Private|GetPlayerEnums) int)))

(fn GetIntfromEnum
  (params (enum :type BP_PlayerModel%20Enum :default "NewEnumerator4"))
  (return (Utilities|Select :Index enum :NewEnumerator4 0 :NewEnumerator0 1 :NewEnumerator1 2 :NewEnumerator2 3)))

(fn SetPlayerModel
  (params (PlayerID :type Integer) (Enum :type BP_PlayerModel%20Enum :default "NewEnumerator4"))
  (|SetBy-RefVar (.playermodel (Utilities|Array|Get(acopy) (Variables|Main|GetPlayerData) PlayerID)) Enum))

(fn AddPlayerScore
  (params (Score :type Integer) (Index :type Integer))
  (bind _playerdata (Variables|Main|GetPlayerData))
  (bind _output (Utilities|Array|Get(acopy) _playerdata Index))
  (bind _structout (Utilities|Struct|SetmembersinBP_PlayerData _output (+ (.PlayerScore (Utilities|Struct|BreakBP_PlayerData _output)) Score)))
  (Development|PrintText (Utilities|Text|FormatText "GAME_INSTANCE: Added {score} to Player {Index}; Total Score is {totalScore}" Score Index (.playerscore _structout)) true true "(R=1.000000,G=0.673184,B=0.172875,A=1.000000)" 5.0)
  (return))

(fn SetPlayerName
  (params (Name :type String) (Id :type Integer))
  (Utilities|Struct|SetmembersinBP_PlayerData (Utilities|Array|Get(acopy) (Variables|Main|GetPlayerData) Id) Name)
  (return))

(fn GetPlayerName
  (params (ID :type Integer))
  (return (.playername (Utilities|Array|Get(acopy) (Variables|Main|GetPlayerData) ID))))

(fn ClearPlayerData
  (bind _gameinstancevariables (Variables|Default|GetGameInstanceVariables))
  (for (_ _array_index) (Variables|Main|GetPlayerData)
    (SetStructData|SetPlayerConnected _array_index false)
    (Variables|/Game/Programming/Core/Blueprints/GameInstance/PDA_GameInstanceSettings.PDA_GameInstanceSettings_C|SetNumGamesPlayed _gameinstancevariables 0)
    (Variables|/Game/Programming/Core/Blueprints/GameInstance/PDA_GameInstanceSettings.PDA_GameInstanceSettings_C|SetTournamentMode _gameinstancevariables false)))

(fn IncrementNumGamesPlayed
  (Math|Integer|IncrementInt (Variables|/Game/Programming/Core/Blueprints/GameInstance/PDA_GameInstanceSettings.PDA_GameInstanceSettings_C|GetNumGamesPlayed (Variables|Default|GetGameInstanceVariables))))

(fn CanGotoNextTournamentLevel
  (bind _gameinstancevariables (Variables|Default|GetGameInstanceVariables))
  (bind _numgamesplayed (Variables|/Game/Programming/Core/Blueprints/GameInstance/PDA_GameInstanceSettings.PDA_GameInstanceSettings_C|GetNumGamesPlayed _gameinstancevariables))
  ;[1 0.7255 0.2078] If TournamentMode is not enabled, go to Level Select
  (if (Variables|/Game/Programming/Core/Blueprints/GameInstance/PDA_GameInstanceSettings.PDA_GameInstanceSettings_C|GetTournamentMode (Variables|Default|GetGameInstanceVariables))
    ;[1 0.7255 0.2078] If NumOfGamesPlayed is less than MaxNumGames, then go to next Gamemode
    (Development|PrintText (Utilities|Text|FormatText "NumGamesPlayed: {NumGamesPlayed}" _numgamesplayed) true true "(R=1.000000,G=0.652687,B=0.176490,A=1.000000)")
    (if (< _numgamesplayed (Variables|/Game/Programming/Core/Blueprints/GameInstance/PDA_GameInstanceSettings.PDA_GameInstanceSettings_C|GetMaxNumTournamentGames _gameinstancevariables))
      (return true)
      (else
        _)))
  (return false))

(fn GetConnectedPlayerDataArray
  (bind _connectedplayerarray (LocalVariables|GetConnectedPlayerArray))
  (for (_array_element _array_index) (Variables|Main|GetPlayerData)
    (bind _connected (GetStructData|GetPlayerConnected _array_index))
    (if _connected
      (Utilities|Array|Add _connectedplayerarray _array_element)
      (return _connectedplayerarray))))

(fn BacktoMainMenu
  (SetStructData|ClearPlayerData)
  (Game|OpenLevel(byObjectReference) "/Game/Programming/Core/Levels/MainMenu.MainMenu"))

(fn ModifyMaxNumGames
  (params (Modifier%20Number :type Integer))
  (bind _gameinstancevariables (Variables|Default|GetGameInstanceVariables))
  (bind _minnum (LocalVariables|GetMinNum))
  (bind _output_get (Variables|/Game/Programming/Core/Blueprints/GameInstance/PDA_GameInstanceSettings.PDA_GameInstanceSettings_C|SetMaxNumTournamentGames _gameinstancevariables (+ Modifier%20Number (Variables|/Game/Programming/Core/Blueprints/GameInstance/PDA_GameInstanceSettings.PDA_GameInstanceSettings_C|GetMaxNumTournamentGames _gameinstancevariables))))
  (if (< _output_get _minnum)
    (Variables|/Game/Programming/Core/Blueprints/GameInstance/PDA_GameInstanceSettings.PDA_GameInstanceSettings_C|SetMaxNumTournamentGames _gameinstancevariables _minnum)))