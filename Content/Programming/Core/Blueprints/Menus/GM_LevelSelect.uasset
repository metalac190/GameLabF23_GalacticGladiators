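; Game mode for the level select menu, which sets up menu input and the on-screen widget.
; On BeginPlay it sets the default menu mapping context, spawns input pawns and creates the WBP_LevelSelect widget in the viewport.
; It then hands that widget reference to each local BP_MenuInputReciever.
; A call to clear the game instance's player data is present but disconnected.
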(event EventBeginPlay
  (bind _asgi_core_game_instance (Utilities|Casting|CastToGI_CORE_GameInstance (Game|GetGameInstance)))
  (Variables|Default|SetDefaultIMC "/Game/Programming/Core/Input/MenuInput/IMC_Core_MenuDefault.IMC_Core_MenuDefault")
  (CallFunction|SpawnInputPawns)
  (bind _returnvalue (UserInterface|CreateWidget "/Game/Programming/Core/Widgets/Menus/WBP_LevelSelect.WBP_LevelSelect_C"))
  (bind _output_get (Variables|Default|SetLevelSelect _returnvalue))
  (UserInterface|Viewport|AddtoViewport _output_get 0)
  ;[1 1 1] Gives Each Input Reciever a Refernce to Main Menu Widget
  (for _array_element (Variables|Default|GetLocalInputs)
    (bind _asbp_menu_input_reciever (Utilities|Casting|CastToBP_MenuInputReciever _array_element))
    (Default|SetWidgetReference _asbp_menu_input_reciever (Variables|Default|GetLevelSelect))))

(fn ConstructionScript)