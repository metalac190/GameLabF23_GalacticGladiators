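; GM_Menu is the menu game mode, which clears player data on the game instance and opens the main menu at BeginPlay.
; It sets the default menu input mapping context, spawns input pawns and adds WBP_MainMenu to the viewport.
; Each local BP_MenuInputReciever gets a reference to that widget.
; SetWidgetRef can repoint all receivers at any given widget.
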(event EventBeginPlay
  (bind _asgi_core_game_instance (Utilities|Casting|CastToGI_CORE_GameInstance (Game|GetGameInstance)))
  (Default|ClearPlayerData _asgi_core_game_instance)
  (Variables|Default|SetDefaultIMC "/Game/Programming/Core/Input/MenuInput/IMC_Core_MenuDefault.IMC_Core_MenuDefault")
  (CallFunction|SpawnInputPawns)
  (bind _returnvalue (UserInterface|CreateWidget "/Game/Programming/Core/Widgets/Menus/WBP_MainMenu.WBP_MainMenu_C"))
  (bind _output_get (Variables|Default|SetCurrentWidget _returnvalue))
  (UserInterface|Viewport|AddtoViewport _output_get 0)
  ;[1 1 1] Gives Each Input Reciever a Refernce to Main Menu Widget
  (for _array_element (Variables|Default|GetLocalInputs)
    (bind _asbp_menu_input_reciever (Utilities|Casting|CastToBP_MenuInputReciever _array_element))
    (Default|SetWidgetReference _asbp_menu_input_reciever (Variables|Default|GetCurrentWidget))))

(event EventTick
  (params (DeltaSeconds :type Float%20%28single-precision%29)))

(fn ConstructionScript)

(fn SetWidgetRef
  (params (Widget :type WBP%20GG%20Widge%20Base%20Object%20Reference))
  (for _array_element (Variables|Default|GetLocalInputs)
    (bind _asbp_menu_input_reciever (Utilities|Casting|CastToBP_MenuInputReciever _array_element))
    (Default|SetWidgetReference _asbp_menu_input_reciever Widget)))