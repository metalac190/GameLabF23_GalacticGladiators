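; Game mode for the GM2 pre-game menu screen, which it sets up on BeginPlay.
; It sets the default menu input mapping context and spawns input pawns, then creates the GM2 pre-game widget with the game instance's pre-game scene time as its time until returning to the main menu.
; Each local menu input receiver gets a reference to that widget.
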(event EventBeginPlay
  (Variables|Default|SetDefaultIMC "/Game/Programming/Core/Input/MenuInput/IMC_Core_MenuDefault.IMC_Core_MenuDefault")
  (CallFunction|SpawnInputPawns)
  (bind _asgi_core_game_instance (Utilities|Casting|CastToGI_CORE_GameInstance (Game|GetGameInstance)))
  (bind _returnvalue (UserInterface|CreateWidget "/Game/Programming/Core/Widgets/Menus/WBP_GM2_PreGameScreen.WBP_GM2_PreGameScreen_C" 0 (Variables|/Game/Programming/Core/Blueprints/GameInstance/PDA_GameInstanceSettings.PDA_GameInstanceSettings_C|GetPreGameSceneTime (Variables|/Game/Programming/Core/Blueprints/GameInstance/GI_CORE_GameInstance.GI_CORE_GameInstance_C|GetGameInstanceVariables _asgi_core_game_instance))))
  (bind _output_get (Variables|Default|SetWidget _returnvalue))
  (UserInterface|Viewport|AddtoViewport _output_get 0)
  (for _array_element (Variables|Default|GetLocalInputs)
    (bind _asbp_menu_input_reciever (Utilities|Casting|CastToBP_MenuInputReciever _array_element))
    (Default|SetWidgetReference _asbp_menu_input_reciever (Variables|Default|GetWidget))))

(event EventTick
  (params (DeltaSeconds :type Float%20%28single-precision%29)))

(fn ConstructionScript)