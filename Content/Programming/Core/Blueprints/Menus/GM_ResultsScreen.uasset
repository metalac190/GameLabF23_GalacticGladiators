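; Game mode for the results screen, which shows each player's score once a match ends.
; On BeginPlay it sets the default menu input context, spawns input pawns and creates the results widget.
; It hands that widget to each local menu input receiver for control.
; Scores from the game instance's player data are pushed into the widget, which then orders them once.
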(event EventBeginPlay
  (Variables|Default|SetDefaultIMC "/Game/Programming/Core/Input/MenuInput/IMC_Core_MenuDefault.IMC_Core_MenuDefault")
  (CallFunction|SpawnInputPawns)
  ;[1 1 1] Getting Game Instance Reference
  (bind _asgi_core_game_instance (Utilities|Casting|CastToGI_CORE_GameInstance (Game|GetGameInstance)))
  (Variables|Default|SetGameInstance _asgi_core_game_instance)
  ;[1 1 1] Add Results Screen to Viewport
  (bind _returnvalue (UserInterface|CreateWidget "/Game/Programming/Core/Widgets/Menus/WBP_ResultsScreen.WBP_ResultsScreen_C"))
  (bind _output_get (Variables|Default|SetResultsScreen _returnvalue))
  (UserInterface|Viewport|AddtoViewport _output_get 0)
  ;[1 1 1] Setting Widget Reference
  (for _array_element (Variables|Default|GetLocalInputs)
    (bind _asbp_menu_input_reciever (Utilities|Casting|CastToBP_MenuInputReciever _array_element))
    (Default|SetWidgetReference _asbp_menu_input_reciever (Variables|Default|GetResultsScreen)))
  ;[1 1 1] Set Player Score for each Player
  (for (_ _array_index) (Variables|/Game/Programming/Core/Blueprints/GameInstance/GI_CORE_GameInstance.GI_CORE_GameInstance_C|GetPlayerData (Variables|Default|GetGameInstance))
    (bind _score (Default|GetPlayerScore (Variables|Default|GetGameInstance) _array_index))
    (Default|SetPlayerScore (Variables|Default|GetResultsScreen) _array_index _score))
  ;[0.7344 1 0.4688] Only calls it once
  (Default|OrderPlayerScores (Variables|Default|GetResultsScreen)))

(event EventTick
  (params (DeltaSeconds :type Float%20%28single-precision%29)))

(fn ConstructionScript)