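; Game mode base that gives each BP_Core_NoPlayerControllerPawn in the level its own local player for input, apparently for menus.
; SpawnInputPawns caches the core game instance, gathers those pawns and, per index, reuses or creates the matching local player.
; Each player receives the default Enhanced Input mapping context, possesses its pawn and joins the controller list, while the pawn's PlayerID is set to that index.
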(event Custom|SpawnInputPawns
  (bind _defaultimc (Variables|Default|GetDefaultIMC))
  ;[0 0 0] Get game mode and existing menu inputs
  (bind _asgi_core_game_instance (Utilities|Casting|CastToGI_CORE_GameInstance (Game|GetGameInstance)))
  (Variables|Default|SetCurrentGameInstance _asgi_core_game_instance)
  (bind _outactors (Actor|GetAllActorsOfClass "/Game/Programming/Core/Blueprints/BaseClasses/BP_Core_NoPlayerControllerPawn.BP_Core_NoPlayerControllerPawn_C"))
  (bind _output_get (Variables|Default|SetLocalInputs _outactors))
  (for (_ _array_index) _output_get
    ;[0 0 0] If a local player exists, use it. Else, create new one and use that
    (bind _output_get_2 (Variables|Default|SetArrayIndex _array_index))
    (Utilities|IsValid (Class|GameplayStatics|GetPlayerControllerfromID _output_get_2)
      (:Is%20Valid
        ;[0 0 0] Set the current LPCs input mapping context
        (Input|AddMappingContext (PlayerController|LocalPlayerSubsystems|GetEnhancedInputLocalPlayerSubsystem (Class|GameplayStatics|GetPlayerControllerfromID _output_get_2)) _defaultimc 0 "(bIgnoreAllPressedKeysUntilRelease=True,bForceImmediately=False)"))
      (:Is%20Not%20Valid
        (bind _returnvalue (Class|GameplayStatics|CreatePlayer _output_get_2))
        (Input|AddMappingContext (PlayerController|LocalPlayerSubsystems|GetEnhancedInputLocalPlayerSubsystem _returnvalue) _defaultimc 0 "(bIgnoreAllPressedKeysUntilRelease=True,bForceImmediately=False)")))
    ;[0 0 0] Force the current LPC to possess the menu input at the current index. Then, add the current LPC to the list of LPCs and set the menu input's PID
    (Pawn|Possess (Class|GameplayStatics|GetPlayerControllerfromID (Variables|Default|GetArrayIndex)) (Utilities|Array|Get(acopy) (Variables|Default|GetLocalInputs) (Variables|Default|GetArrayIndex)))
    (Utilities|Array|AddUnique (Variables|Default|GetPlayerControllers) (Class|GameplayStatics|GetPlayerControllerfromID (Variables|Default|GetArrayIndex)))
    (Variables|/Game/Programming/Core/Blueprints/BaseClasses/BP_Core_NoPlayerControllerPawn.BP_Core_NoPlayerControllerPawn_C|SetPlayerID (Utilities|Array|Get(acopy) (Variables|Default|GetLocalInputs) (Variables|Default|GetArrayIndex)) (Variables|Default|GetArrayIndex))))

(fn ConstructionScript)