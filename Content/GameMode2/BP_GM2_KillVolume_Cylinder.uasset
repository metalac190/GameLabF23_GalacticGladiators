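; Cylinder kill volume for GameMode2 that kills and respawns players who enter it.
; On player entry it calls the player's kill handler, forces a respawn and prints a debug message with the player number.
; The thunder-ball hit particle starts inactive and is activated when a player exits the volume, with no later deactivation.
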(event EventBeginPlay
  (Components|Activation|SetActive (Variables|Default|GetP_ky_ThunderBallHit) false false))

(fn ConstructionScript
  (|CallParentFunction))

(fn PlayerEntered
  (params (Player :type PC%20GM2%20Player%20Object%20Reference))
  (Default|CallOnPlayerKill Player)
  (Default|ForceRespawn Player false)
  (Development|PrintString (Utilities|String|Append "Player " (Utilities|String|ToString(Integer) (Variables|/Game/GameMode2/Programming/Movement/PC_GM2_Player.PC_GM2_Player_C|GetPlayer%20Number Player)) " is being respawned.")))

(fn PlayerExited
  (params (Player :type PC%20GM2%20Player%20Object%20Reference))
  (Components|Activation|SetActive (Variables|Default|GetP_ky_ThunderBallHit) true false))