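; BP_GM2_BigStar is a collectible big star pickup for GameMode2 that awards score points to the player who collects it.
; On spawn it plays sound and VFX, randomly varies its rotation speed, and applies color and scale from the DAPlayer data.
; Collection runs the parent's Collected logic, then adds the point value from the same DAPlayer data to that player's score.
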(event EventBeginPlay
  (bind _returnvalue (Transformation|GetActorLocation))
  (bind _rotatingmovement (Variables|Default|GetRotatingMovement))
  (bind _da_player (Variables|Default|GetDA_Player))
  (Audio|PlaySoundatLocation (Variables|Default|GetSFX_Spawned) _returnvalue "0, 0, 0" 1.0 1.0 0.0 0 0 0 0)
  (Niagara|SpawnSystematLocation (Variables|Default|GetVFX_Spawned) _returnvalue)
  (Variables|/Script/Engine.RotatingMovementComponent|SetRotationRate _rotatingmovement (Math|Rotator|CombineRotators (Variables|/Script/Engine.RotatingMovementComponent|GetRotationRate _rotatingmovement) (* (Variables|/Script/Engine.RotatingMovementComponent|GetRotationRate _rotatingmovement) (Math|Random|RandomFloatinRange -0.25 0.25))))
  (bind _returnvalue_2 (Rendering|Material|CreateDynamicMaterialInstance (Variables|Default|GetSM_Star) 0 "/Game/GameMode2/Art/Powerups/Star/Source/M_Star.M_Star" "None" :!class /Script/Engine.PrimitiveComponent))
  (Rendering|Material|SetVectorParameterValue _returnvalue_2 "Color" (Variables|/Game/GameMode2/Programming/PLAYERDATA/DA_Player.DA_Player_C|GetBigStarColor _da_player) :!class /Script/Engine.MaterialInstanceDynamic)
  (Transformation|SetRelativeScale3D (Variables|Default|GetDefaultSceneRoot) (Variables|/Game/GameMode2/Programming/PLAYERDATA/DA_Player.DA_Player_C|GetBigStarSize _da_player)))

(fn ConstructionScript
  (|CallParentFunction))

(fn Collected
  (params (Player :type PC%20GM2%20Player%20Object%20Reference))
  (|CallParentFunction Player)
  (Default|AddtoScore Player (Variables|/Game/GameMode2/Programming/PLAYERDATA/DA_Player.DA_Player_C|GetBigStarPoints (Variables|Default|GetDA_Player))))