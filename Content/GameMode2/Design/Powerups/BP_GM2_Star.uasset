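; BP_GM2_Star is a collectible star powerup for GameMode2 that awards points to the player who picks it up.
; On spawn it plays a sound and effect at its location and randomly varies its rotating movement rate by up to a quarter either way.
; Collection runs the parent powerup's logic, then adds its Points to the collecting player's score.
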(event EventBeginPlay
  (bind _returnvalue (Transformation|GetActorLocation))
  (bind _rotatingmovement (Variables|Default|GetRotatingMovement))
  (Audio|PlaySoundatLocation (Variables|Default|GetSFX_Spawned) _returnvalue "0, 0, 0" 1.0 1.0 0.0 0 0 0 0)
  (Niagara|SpawnSystematLocation (Variables|Default|GetVFX_Spawned) _returnvalue)
  (Variables|/Script/Engine.RotatingMovementComponent|SetRotationRate _rotatingmovement (Math|Rotator|CombineRotators (Variables|/Script/Engine.RotatingMovementComponent|GetRotationRate _rotatingmovement) (* (Variables|/Script/Engine.RotatingMovementComponent|GetRotationRate _rotatingmovement) (Math|Random|RandomFloatinRange -0.25 0.25)))))

(fn ConstructionScript
  (|CallParentFunction))

(fn Collected
  (params (Player :type PC%20GM2%20Player%20Object%20Reference))
  (|CallParentFunction Player)
  (Default|AddtoScore Player (Variables|Default|GetPoints)))