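; Bounce pad obstacle for GameMode2, named for use in Whitebox05 only, that launches an overlapping PC_GM2_Player upward.
; On overlap it zeroes the capsule's vertical physics velocity and scales the horizontal velocity by DirectionalMultiplier, so earlier fall or rise speed does not affect the bounce.
; It then applies a mass-dependent upward impulse of JumpForce to the capsule and plays a 2D sound effect.
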(event Collision|EventActorBeginOverlap
  (params (OtherActor :type Actor%20Object%20Reference))
  (bind _aspc_gm2_player (Utilities|Casting|CastToPC_GM2_Player OtherActor))
  (bind _returnvalue (Physics|GetPhysicsLinearVelocity (Variables|/Script/Engine.Character|GetCapsuleComponent _aspc_gm2_player) "None"))
  (Class|PrimitiveComponent|SetAllPhysicsLinearVelocity (Variables|/Script/Engine.Character|GetCapsuleComponent _aspc_gm2_player) (* (Math|Vector|MakeVector (.X (Math|Vector|BreakVector _returnvalue)) (.Y (Math|Vector|BreakVector _returnvalue)) 0.0) (Variables|Default|GetDirectionalMultiplier)) false)
  (Physics|AddImpulse (Variables|/Script/Engine.Character|GetCapsuleComponent _aspc_gm2_player) (Math|Vector|MakeVector 0.0 0.0 (Variables|Default|GetJump%20Force)) "None" false)
  (Audio|PlaySound2D (Variables|Default|GetSFX) 1.0 1.0 0.0 0 0))

(fn ConstructionScript)