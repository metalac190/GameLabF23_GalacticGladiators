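; BP_GM2_LaunchPad_2 is a launch pad obstacle that boosts the PC_GM2_Player when it overlaps the Box.
; It applies an impulse to the player's capsule along the vector from Pad to Sphere, so the Sphere's placement sets direction and, with BoostStrength, force.
; The impulse respects mass, and the launch sound plays at the world origin rather than at the pad.
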(event OnComponentBeginOverlap(Box)
  (params (OverlappedComponent :type Primitive%20Component%20Object%20Reference) (OtherActor :type Actor%20Object%20Reference) (OtherComp :type Primitive%20Component%20Object%20Reference) (OtherBodyIndex :type Integer) (bFromSweep :type Boolean) (SweepResult :type Hit%20Result%20Structure%20%28by%20ref%29))
  (bind _aspc_gm2_player (Utilities|Casting|CastToPC_GM2_Player OtherActor))
  (Physics|AddImpulse (Variables|/Script/Engine.Character|GetCapsuleComponent _aspc_gm2_player) (* (- (Transformation|GetWorldLocation (Variables|Default|GetPad)) (Transformation|GetWorldLocation (Variables|Default|GetSphere))) (* (Variables|Default|GetBoostStrength) -1.0)) "None" false)
  (Audio|PlaySoundatLocation (Variables|Default|GetSFX) "0, 0, 0" "0, 0, 0" 1.0 1.0 0.0 0 0 0 0))

(fn ConstructionScript)