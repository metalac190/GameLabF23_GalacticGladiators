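; BP_GM2_ShockBlock is an obstacle for GameMode2 that alternates between shocking and harmless states on a fixed timer.
; From BeginPlay, a self-repeating Shock event uses Delays to toggle ShockCollision's Pawn response between Overlap and Ignore, swapping the block's material between blue and glass to match.
; When the player pawn begins overlapping the actor, it casts to PC_GM2_Player and calls Shocked.
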(event Custom|Shock
  (bind _shockcollision (Variables|Default|GetShockCollision))
  (bind _shockblock (Variables|Default|GetShockBlock))
  ;[0.3438 0.3438 0.3438] Toggle Collision
  (Collision|SetCollisionResponsetoChannel _shockcollision "ECC_Pawn" "ECR_Overlap")
  (Rendering|Material|SetMaterial _shockblock 0 "/Game/GameMode1/Art/PlayerMaterials/MI_PlayerMat_Blue.MI_PlayerMat_Blue")
  (Utilities|FlowControl|Delay 3.0)
  (Rendering|Material|SetMaterial _shockblock 0 "/DatasmithContent/Materials/FBXImporter/VRED/Glass.Glass")
  (Collision|SetCollisionResponsetoChannel _shockcollision "ECC_Pawn" "ECR_Ignore")
  (Utilities|FlowControl|Delay 3.0)
  (CallFunction|Shock))

(event EventBeginPlay
  (CallFunction|Shock))

(event Collision|EventActorBeginOverlap
  (params (OtherActor :type Actor%20Object%20Reference))
  (bind _returnvalue (Game|Player|GetPlayerPawn 0))
  ;[0.375 0.375 0.375] Call Shocked event
  (if (== OtherActor _returnvalue)
    (bind _aspc_gm2_player (Utilities|Casting|CastToPC_GM2_Player _returnvalue)
      (:then
        (bind _output_get (Variables|Default|SetAs%20PC%20GM2%20Player _aspc_gm2_player))
        (Default|Shocked _output_get))
      (:CastFailed
        (Development|PrintString "cast to player failed")))))

(fn ConstructionScript)