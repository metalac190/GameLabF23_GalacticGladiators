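; BP_GM2_SlowVolume is a GameMode2 obstacle volume that slows players inside it.
; Entering adds an additive speed multiplier with zero duration, and exiting adds a value derived from the same multiplier, apparently its negation to undo it.
; Each tick it also calls SlowPlayerToFraction on every tracked player, using delta time and a velocity multiplier.
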(event EventTick
  (params (DeltaSeconds :type Float%20%28single-precision%29))
  (for _array_element (Variables|Default|GetPlayer)
    (Default|SlowPlayertoFraction _array_element DeltaSeconds (Variables|Default|GetPlayer%20Velocity%20Multiplier))))

(fn ConstructionScript
  (|CallParentFunction))

(fn PlayerEntered
  (params (Player :type PC%20GM2%20Player%20Object%20Reference))
  (Default|AddSpeedMultiplier Player (Utilities|Struct|MakeS_GM2_StatModifer (Variables|Default|GetAdditive%20Speed%20Multiplier) 0.0)))

(fn PlayerExited
  (params (Player :type PC%20GM2%20Player%20Object%20Reference))
  (bind _result (Math|Float|NegateFloat (Variables|Default|GetAdditive%20Speed%20Multiplier))
    (:%20%20
      (Default|AddSpeedMultiplier Player (Utilities|Struct|MakeS_GM2_StatModifer _result 0.0)))))