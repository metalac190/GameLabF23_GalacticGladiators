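; Placeholder actor that fakes a flashing light bar by blinking its own visibility in game.
; On BeginPlay it runs FakeFlashingLight, a hard-coded chain of SetActorHiddenInGame calls separated by short fixed delays rather than a loop.
; The sequence plays once and leaves the actor hidden, with no exposed duration, though a comment notes that a timed loop is wanted.
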(event Custom|Fake%20Flashing%20Light
  (Rendering|SetActorHiddenInGame true)
  (Utilities|FlowControl|Delay 0.2)
  (Rendering|SetActorHiddenInGame false)
  (Utilities|FlowControl|Delay 0.2)
  (Rendering|SetActorHiddenInGame true)
  (Utilities|FlowControl|Delay 0.2)
  (Rendering|SetActorHiddenInGame false)
  (Utilities|FlowControl|Delay 0.2)
  (Rendering|SetActorHiddenInGame true)
  (Utilities|FlowControl|Delay 0.2)
  (Rendering|SetActorHiddenInGame false)
  (Utilities|FlowControl|Delay 0.2)
  (Rendering|SetActorHiddenInGame true)
  (Utilities|FlowControl|Delay 0.2)
  (Rendering|SetActorHiddenInGame false)
  (Utilities|FlowControl|Delay 0.2)
  (Rendering|SetActorHiddenInGame true)
  (Utilities|FlowControl|Delay 0.2))

(event EventBeginPlay
  (CallFunction|FakeFlashingLight) ; Please make a loop for the fake light to flash for a certain amount of time (exposed), and IGNORE my stupidity
)

(event Collision|EventActorBeginOverlap
  (params (OtherActor :type Actor%20Object%20Reference)))

(event EventTick
  (params (DeltaSeconds :type Float%20%28single-precision%29)))

(fn ConstructionScript)