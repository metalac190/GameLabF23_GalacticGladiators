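; Placeholder GameMode2 actor that spawns a configurable actor class, by its name stars, at a set of spawn points.
; SpawnStars validates the class and point list, then plays a pre-spawn Niagara effect at each point.
; A Delay inside that loop ignores re-triggers while pending, so one shared SpawnDelay precedes a nested loop spawning the actor at every point's transform.
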(event Custom|SpawnStars
  (bind _starspawningpoints (Variables|Default|GetStarSpawningPoints))
  (if (and (Utilities|IsValidClass (Variables|Default|GetActorToBeSpawn)) (Utilities|Array|IsNotEmpty _starspawningpoints))
    (for _array_element _starspawningpoints
      (Niagara|SpawnSystematLocation (Variables|Default|GetPreSpawnVFX) (Transformation|GetActorLocation _array_element))
      (Utilities|FlowControl|Delay (Variables|Default|GetSpawnDelay))
      (for _array_element_2 (Variables|Default|GetStarSpawningPoints)
        (Game|SpawnActorfromClass (Variables|Default|GetActorToBeSpawn) (Transformation|GetActorTransform _array_element_2) "Undefined" "MultiplyWithRoot" 0 0)))))

(event EventBeginPlay)

(fn ConstructionScript)