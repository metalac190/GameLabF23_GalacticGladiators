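; BP_GM2_Volume is a GameMode2 volume actor that tracks which PC_GM2_Player actors are inside it.
; Overlap events add and remove players from the Player collection, acting only when membership changes.
; Each change calls PlayerEntered or PlayerExited, which only print the player number, then plays a sound at the volume's location: SFXPlayerDead on entry, SFXLightning on exit.
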(event Collision|EventActorBeginOverlap
  (params (OtherActor :type Actor%20Object%20Reference))
  (bind _player (Variables|Default|GetPlayer))
  (bind _aspc_gm2_player (Utilities|Casting|CastToPC_GM2_Player OtherActor))
  (if (not (Utilities|Array|ContainsItem _player _aspc_gm2_player))
    (Utilities|Array|Add _player _aspc_gm2_player)
    (CallFunction|PlayerEntered _aspc_gm2_player)
    (bind _returnvalue (Audio|SpawnSoundatLocation (Variables|Default|GetSFX_PlayerDead) (Transformation|GetActorLocation) "0, 0, 0" 1.0 1.0 0.0 0 0))
    (Audio|Components|Audio|Play _returnvalue 0.0)))

(event Collision|EventActorEndOverlap
  (params (OtherActor :type Actor%20Object%20Reference))
  (bind _aspc_gm2_player (Utilities|Casting|CastToPC_GM2_Player OtherActor))
  (bind _returnvalue (Utilities|Array|RemoveItem (Variables|Default|GetPlayer) _aspc_gm2_player))
  (if _returnvalue
    (CallFunction|PlayerExited _aspc_gm2_player)
    (bind _returnvalue_2 (Audio|SpawnSoundatLocation (Variables|Default|GetSFX_Lightning) (Transformation|GetActorLocation) "0, 0, 0" 1.0 1.0 0.0 0 0))
    (Audio|Components|Audio|Play _returnvalue_2 0.0)))

(fn ConstructionScript)

(fn PlayerEntered
  (params (Player :type PC%20GM2%20Player%20Object%20Reference))
  (Development|PrintString (Utilities|String|Append "Player " (Utilities|String|ToString(Integer) (Variables|/Game/GameMode2/Programming/Movement/PC_GM2_Player.PC_GM2_Player_C|GetPlayer%20Number Player)) " entered volume")))

(fn PlayerExited
  (params (Player :type PC%20GM2%20Player%20Object%20Reference))
  (Development|PrintString (Utilities|String|Append "Player " (Utilities|String|ToString(Integer) (Variables|/Game/GameMode2/Programming/Movement/PC_GM2_Player.PC_GM2_Player_C|GetPlayer%20Number Player)) " exited volume")))