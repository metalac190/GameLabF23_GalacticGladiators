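; Score tracker for GameMode2, meant to find the highest- and lowest-scoring players and announce leader changes.
; BeginPlay seeds the previous and new high/low player references with one found PC_GM2_Player.
; ScoreLogic's entry is unwired, so its loop over player scores and its CallNewHighScore/CallNewLowScore calls never run.
; That dead loop also assigns high and low players on every iteration, regardless of score comparison.
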(event EventBeginPlay
  (bind _returnvalue (Actor|GetActorOfClass "/Game/GameMode2/Programming/Movement/PC_GM2_Player.PC_GM2_Player_C"))
  (Variables|Default|SetPreviousHighestScorePlayer _returnvalue)
  (Variables|Default|SetPreviousLowestScorePlayer _returnvalue)
  (bind _output_get (Variables|Default|SetNewHighScorePlayer _returnvalue))
  (Variables|Default|SetNewLowScorePlayer _output_get))

(event Collision|EventActorBeginOverlap
  (params (OtherActor :type Actor%20Object%20Reference)))

(event EventTick
  (params (DeltaSeconds :type Float%20%28single-precision%29)))

(fn ConstructionScript)

(fn ScoreLogic
  (params (PreviousPlayerWithLowestScore :type PC%20GM2%20Player%20Object%20Reference) (PreviousPlayerWithHighestScore :type PC%20GM2%20Player%20Object%20Reference)))