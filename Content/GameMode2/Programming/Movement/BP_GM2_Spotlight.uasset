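; BP_GM2_Spotlight is a GameMode2 spotlight actor that hovers above the player with the highest score.
; StartGame shows the light and binds ScoreChange to player 0's score-change event.
; ScoreChange compares GM_GM2 scores by player index and tracks the leader's pawn, which Tick follows from a fixed height.
; The construction script applies configurable intensity, color and cone angle, and BeginPlay hides the light.
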(event Custom|ScoreChange
  (bind _spotlight (Variables|Default|GetSpotLight))
  ;[1 0 0] Point-based System. To use, hook the topmost bind event into OnBeginPlay
  (bind _outactors (Actor|GetAllActorsOfClass "/Game/GameMode2/Programming/Movement/PC_GM2_Player.PC_GM2_Player_C"))
  ;;[0 0 0] Sets Tracked Actor When New Player Has Highest Score
  (for (_ _array_index) _outactors
    (bind _score (Default|GetPlayerScore (.AsGM%20GM2 (Utilities|Casting|CastToGM_GM2 (Game|GetGameMode))) _array_index))
    (if (> _score (Variables|DEPRECATED|GetHighestScore))
      (Variables|DEPRECATED|SetHighestScore _score)
      (Variables|DEPRECATED|SetIndexOfHighestScore _array_index)))
  (Variables|DEPRECATED|SetHighestScore 0)
  (bind _aspc_gm2_player (Utilities|Casting|CastToPC_GM2_Player (Pawn|GetControlledPawn (Class|GameplayStatics|GetPlayerControllerfromID (Variables|DEPRECATED|GetIndexOfHighestScore)))))
  (bind _output_get (Variables|Default|SetTrackedActor _aspc_gm2_player))
  ;;[0 0 0] Initial Setup
  (Utilities|FlowControl|DoOnce false
    (:Completed
      (Transformation|SetWorldLocation _spotlight (Math|Vector|MakeVector (.x (Transformation|GetActorLocation _output_get)) (.y (Transformation|GetActorLocation _output_get)) (+ (.z (Transformation|GetActorLocation _output_get)) 1.25e+03)) false false)
      (Rendering|SetVisibility _spotlight true false))))

(event Custom|Start%20Game
  ;[1 0 0] Point-based System. To use, hook the topmost bind event into OnBeginPlay
  (EventDispatchers|BindEventtoScoreChanged (.AsPC%20GM2%20Player (Utilities|Casting|CastToPC_GM2_Player (Game|GetPlayerCharacter 0))) (delegate Custom|ScoreChange))
  (Rendering|SetVisibility (Variables|Default|GetSpotLight) true false))

(event EventBeginPlay
  ;[0 0 0] Event Bindings
  (Rendering|SetVisibility (Variables|Default|GetSpotLight) false false))

(event Collision|EventActorBeginOverlap
  (params (OtherActor :type Actor%20Object%20Reference)))

(event EventTick
  (params (DeltaSeconds :type Float%20%28single-precision%29))
  (bind _trackedactor (Variables|Default|GetTrackedActor))
  (bind _returnvalue (Transformation|GetActorLocation _trackedactor))
  ;[0 0 0] Set Position
  (Utilities|IsValid _trackedactor
    (:Is%20Valid
      (Transformation|SetWorldLocation (Variables|Default|GetSpotLight) (Math|Vector|MakeVector (.x _returnvalue) (.y _returnvalue) (+ (.z _returnvalue) 1.25e+03)) false false))))

(fn ConstructionScript
  (bind _spotlight (Variables|Default|GetSpotLight))
  (Rendering|Components|Light|SetIntensity _spotlight (Variables|Default|GetSpotlightIntensity))
  (Rendering|Components|Light|SetLightColor _spotlight (Variables|Default|GetSpotlightColor) true)
  (Rendering|Lighting|SetOuterConeAngle _spotlight (Variables|Default|GetSpotlightOuterConeAngle)))