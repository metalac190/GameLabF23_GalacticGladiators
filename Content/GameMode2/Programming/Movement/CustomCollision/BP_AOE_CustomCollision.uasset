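; BP_AOE_CustomCollision is an area-of-effect actor that fires a radial impulse as soon as it begins play.
; BeginPlay calls Trigger, then SpawnAOESphere, which configures the RadialForce component from its radius and force variables before firing the impulse.
; It draws a debug sphere and runs a Pawn sphere overlap, optionally ignoring the instigator.
; Overlapped actors only have their names printed, with no other effect applied.
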(event Custom|Trigger
  (CallFunction|SpawnAOESphere))

(event Custom|SpawnAOESphere
  (bind _radialforce (Variables|Default|GetRadialForce))
  (if true
    (bind _output_get (Variables|/Script/Engine.RadialForceComponent|SetRadius _radialforce (Variables|Default|GetRadius)))
    (bind _output_get_2 (Variables|/Script/Engine.RadialForceComponent|SetForceStrength _radialforce (Variables|Default|GetRadial%20Force)))
    (Variables|/Script/Engine.RadialForceComponent|SetImpulseStrength _radialforce _output_get_2)
    (Rendering|Debug|DrawDebugSphere (.location (Transformation|GetWorldTransform _radialforce)) _output_get 12 "(R=1.000000,G=1.000000,B=1.000000,A=1.000000)" 2.0 1.0)
    (Class|RadialForceComponent|FireImpulse _radialforce)
    (bind _outactors (Collision|SphereOverlapActors (Transformation|GetActorLocation) 0.0 (Utilities|Array|MakeArray "ObjectTypeQuery3") 0 (select (Variables|Default|GetIgnoreInstigator) (Utilities|Array|MakeArray (Game|GetInstigator)) 0)))
    (for _array_element _outactors
      (Development|PrintString (Utilities|GetDisplayName _array_element)))))

(event EventBeginPlay
  (CallFunction|Trigger))

(event Collision|EventActorBeginOverlap
  (params (OtherActor :type Actor%20Object%20Reference)))

(event EventTick
  (params (DeltaSeconds :type Float%20%28single-precision%29)))

(fn ConstructionScript)