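; Ability actor component for the GameMode2 player, providing the owner references and effect playback that an ability needs.
; On BeginPlay it casts its owner to PC_GM2_Player and caches the player and its CharacterMovement component.
; PlayAbilityEffects plays a given sound and spawns a given visual effect system at the player's location.
; It holds no ability logic of its own.
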(event Custom|PlayAbilityEffects
  (params (Audio :type Sound%20Base%20Object%20Reference) (Visual :type Niagara%20System%20Object%20Reference))
  (bind _player (Variables|Default|GetPlayer))
  (bind _returnvalue (Transformation|GetActorLocation _player))
  (Audio|PlaySoundatLocation Audio _returnvalue "0, 0, 0" 1.0 1.0 0.0 0 0 0 0)
  (Niagara|SpawnSystematLocation Visual _returnvalue))

(event EventBeginPlay
  (|CallParentFunction)
  (bind _aspc_gm2_player (Utilities|Casting|CastToPC_GM2_Player (Components|GetOwner)))
  (bind _output_get (Variables|Default|SetPlayer _aspc_gm2_player))
  (Variables|Default|SetCharacter%20Movement (Variables|/Script/Engine.Character|GetCharacterMovement _output_get)))