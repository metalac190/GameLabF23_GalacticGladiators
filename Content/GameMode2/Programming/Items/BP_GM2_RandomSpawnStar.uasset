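; Spawner actor for GameMode2 that keeps adding star items to the level, starting at BeginPlay and repeating every five seconds.
; Each pass shuffles all BP_GM2_StarSpawnPoint actors and spawns one BP_GM2_Star at the first point without a star at its exact location.
; SpawnStar re-calls itself after a delay and prints a debug message each pass, even when every point is occupied.
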(event Custom|SpawnStar
  (bind _outactors (Actor|GetAllActorsOfClass "/Game/GameMode2/Design/Powerups/BP_GM2_Star.BP_GM2_Star_C"))
  (bind _outactors_2 (Actor|GetAllActorsOfClass "/Game/GameMode2/Design/Powerups/BP_GM2_StarSpawnPoint.BP_GM2_StarSpawnPoint_C"))
  (Utilities|Array|Shuffle _outactors_2)
  (bind _array_element (Utilities|Array|ForEachLoopwithBreak _outactors_2 :!label _label)
    (:LoopBody
      (bind _array_element_2 (Utilities|Array|ForEachLoopwithBreak _outactors :!label _label_2)
        (:LoopBody
          (if (Utilities|Operators|EqualEqual (Transformation|GetActorLocation _array_element_2) (Transformation|GetActorLocation _array_element) 0.0)
            (Variables|Default|Set%20overlap true)
            (goto _label_2 Break)
            (else
              (Variables|Default|Set%20overlap false))))
        (:Completed
          (if (not (Variables|Default|Get%20overlap))
            (Game|SpawnActorfromClass "/Game/GameMode2/Design/Powerups/BP_GM2_Star.BP_GM2_Star_C" (Math|Transform|MakeTransform (Transformation|GetActorLocation _array_element) "0, 0, 0" "1.000000,1.000000,1.000000") "Undefined" "MultiplyWithRoot" 0 0)
            (goto _label Break)))))
    (:Completed
      (Development|PrintString "spawned star")
      (Utilities|FlowControl|Delay 5.0)
      (CallFunction|SpawnStar))))

(event EventBeginPlay
  (CallFunction|SpawnStar))

(fn ConstructionScript)