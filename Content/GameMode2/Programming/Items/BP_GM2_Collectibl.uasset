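; Base collectible item for GM2 that the player picks up by touching it.
; A Trigger overlap from a PC_GM2_Player calls Collected, a placeholder for child classes to override that only prints a not-implemented message.
; The item then either destroys itself or, when DestroyOnPickup is off, deactivates and reactivates after the TemporaryDisableOnPickup delay.
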(event OnComponentBeginOverlap(Trigger)
  (params (OverlappedComponent :type Primitive%20Component%20Object%20Reference) (OtherActor :type Actor%20Object%20Reference) (OtherComp :type Primitive%20Component%20Object%20Reference) (OtherBodyIndex :type Integer) (bFromSweep :type Boolean) (SweepResult :type Hit%20Result%20Structure%20%28by%20ref%29))
  (bind _aspc_gm2_player (Utilities|Casting|CastToPC_GM2_Player OtherActor))
  (Development|PrintString "Collected item")
  (CallFunction|Collected _aspc_gm2_player)
  (if (Variables|Default|GetDestroyOnPickup)
    ;[1 1 1] Destroy Collectible
    (Actor|DestroyActor)
    (else
      ;[1 1 1] Temporarily Disable Collectible
      (CallFunction|SetActive self false)
      (Utilities|FlowControl|Delay (Variables|Default|GetTemporaryDisableOnPickup))
      (CallFunction|SetActive self true))))

(fn ConstructionScript)

(fn Collected
  (params (Player :type PC%20GM2%20Player%20Object%20Reference))
  (Development|PrintString "BP_GM2_Collecteible.Collected() is not implemented."))