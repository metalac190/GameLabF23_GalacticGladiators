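; BP_GM2_CollectibleSpawner manages collectible spawning for game mode 2 across every BP_GM2_CollectibleSpawnPoint in the level.
; On BeginPlay it fills all points, waits an initial delay, then endlessly refills one random empty point at a time.
; A Delay-based loop polls while all points are full, then waits a random interval before the next spawn.
; GetRandomSpawner picks uniformly and still prints a TODO message.
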(event EventBeginPlay
  (bind _randomized_delay (Variables|Default|GetRandomized%20Delay))
  ;[1 1 1] Spawn Initial Stars
  (bind _outactors (Actor|GetAllActorsOfClass "/Game/GameMode2/Design/Powerups/BP_GM2_CollectibleSpawnPoint.BP_GM2_CollectibleSpawnPoint_C"))
  (bind _output_get (Variables|Default|SetSpawn%20Points _outactors))
  (for _array_element _output_get
    (Default|SpawnCollectible _array_element))
  (Utilities|FlowControl|Delay (Variables|Default|GetInitial%20Delay%20Till%20Random))
  ;[1 1 1] Randomly Refill Collectible Slots
  (bind _spawners (CallFunction|GetEmptySpawners :!label _label))
  (if (!= (Utilities|Array|Length _spawners) 0)
    (bind _spawner (CallFunction|GetRandomSpawner _spawners))
    (Default|SpawnCollectible _spawner)
    ;[1 1 1] Don't do random delay till a collector is empty
    (bind _is_full (CallFunction|AllSpawnersFull :!label _label_2))
    (if _is_full
      (Utilities|FlowControl|Delay 0.1)
      (goto _label_2)
      (else
        _)))
  ;[1 1 1] Randomly wait for next spawn
  (Utilities|FlowControl|Delay (Math|Random|RandomFloatinRange (.x _randomized_delay) (.y _randomized_delay)))
  (goto _label))

(fn ConstructionScript)

(fn GetEmptySpawners
  (LocalVariables|Setresult (Utilities|Array|MakeArray))
  (for _array_element (Variables|Default|GetSpawn%20Points)
    (bind _value (Default|HasCollectible _array_element))
    (if (not _value)
      (Utilities|Array|Add (LocalVariables|Getresult) _array_element)))
  (return (LocalVariables|Getresult)))

(fn GetRandomSpawner
  (params (Spawners :type Array%20of%20BP%20GM2%20Collectible%20Spawn%20Point%20Object%20References))
  (Development|PrintString "TODO: CollectibleSpawner.GetRandomSpawner()")
  (return (.OutItem (Utilities|Array|Random Spawners))))

(fn AllSpawnersFull
  (for _array_element (Variables|Default|GetSpawn%20Points)
    (bind _value (Default|HasCollectible _array_element))
    (if (not _value)
      (return false)))
  (return true))