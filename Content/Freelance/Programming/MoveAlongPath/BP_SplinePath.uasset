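; BP_SplinePath moves a target actor along its spline at a set speed.
; It starts at BeginPlay, after a delay, or through the TriggerMove interface event, depending on StartType.
; Each Tick advances the distance and applies the spline's local location as the actor's relative location, keeping rotation and scale.
; Loop closes the spline and resets distance at the end, with debug prints showing progress.
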(event EventTick
  (params (DeltaSeconds :type Float%20%28single-precision%29))
  (CallFunction|HandleMovement (Variables|Private|Get?%20CanMove)))

(event EventBeginPlay
  ;[1 1 1] Comment
  (Spline|SetClosedLoop (Variables|Default|GetSpline) (Variables|MovementSettings|Get?%20Loop) true)
  ;[1 1 1] Comment
  (switch Utilities|FlowControl|Switch|SwitchonEN_PathStartMode (Variables|MovementSettings|GetStartType)
    (:NewEnumerator0
      _)
    (:NewEnumerator1
      (Utilities|FlowControl|Delay (Variables|MovementSettings|GetMoveDelay))))
  (Variables|Private|Set?%20CanMove true))

(event EventTriggerMove
  ;[1 1 1] Interface Implementation
  (switch Utilities|FlowControl|Switch|SwitchonEN_PathStartMode (Variables|MovementSettings|GetStartType)
    (:NewEnumerator2
      (Variables|Private|Set?%20CanMove true))))

(fn ConstructionScript)

(fn HandleMovement
  (params (canMove :type Boolean))
  (bind _targetactor (Variables|PublicReference|GetTargetActor))
  (if canMove
    (Utilities|UpdateDistanceAlongSpline)
    (Transformation|SetActorRelativeTransform (Variables|PublicReference|GetTargetActor) (Math|Transform|MakeTransform (.location (Spline|GetTransformatDistanceAlongSpline (Variables|Default|GetSpline) (Variables|Private|GetDistanceAlongSpline) "Local" false)) (Transformation|GetActorRotation _targetactor) (Class|Actor|GetActorRelativeScale3D _targetactor)) false false)
    (Development|PrintText (Utilities|Text|FormatText "[{0}][{1}]" (Variables|Private|GetDistanceAlongSpline) (Spline|GetSplineLength (Variables|Default|GetSpline))))
    (if (and (Variables|MovementSettings|Get?%20Loop) (>= (Variables|Private|GetDistanceAlongSpline) (Spline|GetSplineLength (Variables|Default|GetSpline))))
      (Variables|Private|SetDistanceAlongSpline 0.0)
      (Development|PrintString "Repeat"))))