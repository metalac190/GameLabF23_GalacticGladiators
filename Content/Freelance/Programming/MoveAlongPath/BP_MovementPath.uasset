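; Spline path actor that positions a target actor at the path's start, with groundwork for moving it along the spline.
; BeginPlay applies the loop setting to the spline and snaps the target to distance zero, keeping its rotation and scale.
; TriggerMove sets CanMove in Move on Trigger mode, and a helper advances distance by speed and delta time.
; Tick only switches on StartMode, so no per-frame movement is wired up.
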(event EventBeginPlay
  ;[1 1 1] Set Loop
  (Spline|SetClosedLoop (Variables|Default|GetSpline) (Variables|MovementSettings|Get?%20Loop) true)
  ;[1 1 1] StartingPosition
  (Private|SetStartingPosition))

(event EventTick
  (params (DeltaSeconds :type Float%20%28single-precision%29))
  (switch Utilities|FlowControl|Switch|SwitchonEN_PathStartMode (Variables|MovementSettings|GetStartMode)))

(event EventTriggerMove
  (switch Utilities|FlowControl|Switch|SwitchonEN_PathStartMode (Variables|MovementSettings|GetStartMode)
    (:NewEnumerator2
      (Variables|Private|Set?%20CanMove true))))

(fn ConstructionScript)

(fn SetStartingPosition
  (bind _targetactor (Variables|Actor|GetTargetActor))
  (Transformation|SetActorRelativeTransform (Variables|Actor|GetTargetActor) (Math|Transform|MakeTransform (.location (Spline|GetTransformatDistanceAlongSpline (Variables|Default|GetSpline) 0.0 "World" false)) (Transformation|GetActorRotation _targetactor) (Class|Actor|GetActorRelativeScale3D _targetactor)) false false))