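; BP_CORE_LobbyInput handles Enhanced Input for players joining and starting from the lobby.
; The Join action finds the WBP_CORE_LobbyMenu widget, passes it this PlayerID through PlayerJoinedEvent and prints the join.
; The Start action only prints "Start Game" as a placeholder.
; Logic that flags the player as joined in GI_CORE_GameInstance is present but disconnected, so it never runs.
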(event Input|EnhancedActionEvents|EnhancedInputActionIA_CORE_Join
  (params (ActionValue :type Boolean) (ElapsedSeconds :type Float%20%28double-precision%29) (TriggeredSeconds :type Float%20%28double-precision%29) (InputAction :type Input%20Action%20Object%20Reference :default "/Game/Freelance/Programming/Input/IA_CORE_Join.IA_CORE_Join"))
  (bind _playerid (Variables|Default|GetPlayerID))
  (:Started
    ;[0 0 0] Player Joining Lobby
    (bind _foundwidgets (Widget|GetAllWidgetsOfClass "/Game/Core/Programming/Prototypes/WBP_CORE_LobbyMenu.WBP_CORE_LobbyMenu_C" true))
    (Default|PlayerJoinedEvent (Utilities|Array|Get(acopy) _foundwidgets) _playerid)
    (Development|PrintText (Utilities|Text|FormatText "Player Joined: {0}" _playerid))))

(event Input|EnhancedActionEvents|EnhancedInputActionIA_CORE_Start
  (params (ActionValue :type Boolean) (ElapsedSeconds :type Float%20%28double-precision%29) (TriggeredSeconds :type Float%20%28double-precision%29) (InputAction :type Input%20Action%20Object%20Reference :default "/Game/Freelance/Programming/Input/IA_CORE_Start.IA_CORE_Start"))
  (:Started
    ;[0 0 0] Players Press Enter to Continue Game
    (Development|PrintString "Start Game")))

(fn ConstructionScript)