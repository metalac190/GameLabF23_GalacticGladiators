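; Lobby game mode that sets up local multiplayer on BeginPlay, with one local player for each BP_CORE_LobbyStart actor in the level.
; For each start it creates a player by index, adds the IMC_LobbyInput mapping context, then spawns and possesses a BP_CORE_LobbyInput pawn tagged with that player ID.
; Index 0 takes a separate branch that maps input on the existing first controller.
; Spawned pawns and controllers are tracked in arrays.
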(event EventBeginPlay
  ;[0 0 0 0.5] Basic Start
  (Variables|Default|SetCurrentGameInstance (Game|GetGameInstance))
  (bind _outactors (Actor|GetAllActorsOfClass "/Game/Freelance/Programming/BP_CORE_LobbyStart.BP_CORE_LobbyStart_C"))
  (bind _output_get (Variables|Default|SetLobbyStarts _outactors))
  (for (_ _array_index) _output_get
    (bind _output_get_2 (Variables|Default|SetArray%20Index _array_index))
    (bind _returnvalue (Class|GameplayStatics|CreatePlayer _output_get_2))
    (if (> (Variables|Default|GetArray%20Index) 0)
      (Input|AddMappingContext (PlayerController|LocalPlayerSubsystems|GetEnhancedInputLocalPlayerSubsystem _returnvalue) "/Game/Freelance/Programming/Input/IMC_LobbyInput.IMC_LobbyInput" 0 "(bIgnoreAllPressedKeysUntilRelease=True,bForceImmediately=False)")
      (bind _returnvalue_2 (Game|SpawnActorfromClass "/Game/Freelance/Programming/BP_CORE_LobbyInput.BP_CORE_LobbyInput_C" (Transformation|GetActorTransform (Utilities|Array|Get(acopy) (Variables|Default|GetLobbyStarts) (Variables|Default|GetArray%20Index))) "Undefined" "MultiplyWithRoot" 0 0))
      (Utilities|Array|AddUnique (Variables|Default|GetLobbyInputs) _returnvalue_2)
      (Pawn|Possess (Class|GameplayStatics|GetPlayerControllerfromID (Variables|Default|GetArray%20Index)) _returnvalue_2)
      (Utilities|Array|AddUnique (Variables|Default|GetPlayerControllers) 0)
      (Variables|/Game/Freelance/Programming/BP_CORE_LobbyInput.BP_CORE_LobbyInput_C|SetPlayerID _returnvalue_2 (Variables|Default|GetArray%20Index))
      (else
        (Input|AddMappingContext (PlayerController|LocalPlayerSubsystems|GetEnhancedInputLocalPlayerSubsystem (Game|GetPlayerController 0)) "/Game/Freelance/Programming/Input/IMC_LobbyInput.IMC_LobbyInput" 0 "(bIgnoreAllPressedKeysUntilRelease=True,bForceImmediately=False)")
        (bind _returnvalue_3 (Game|SpawnActorfromClass "/Game/Freelance/Programming/BP_CORE_LobbyInput.BP_CORE_LobbyInput_C" (Transformation|GetActorTransform (Utilities|Array|Get(acopy) (Variables|Default|GetLobbyStarts) (Variables|Default|GetArray%20Index))) "Undefined" "MultiplyWithRoot" 0 0))
        (Utilities|Array|AddUnique (Variables|Default|GetLobbyInputs) _returnvalue_3)
        (Pawn|Possess (Class|GameplayStatics|GetPlayerControllerfromID (Variables|Default|GetArray%20Index)) _returnvalue_3)
        (Utilities|Array|AddUnique (Variables|Default|GetPlayerControllers) 0)
        (Variables|/Game/Freelance/Programming/BP_CORE_LobbyInput.BP_CORE_LobbyInput_C|SetPlayerID _returnvalue_3 (Variables|Default|GetArray%20Index))))))

(fn ConstructionScript)