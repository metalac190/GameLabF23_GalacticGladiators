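; Level hazard spawner that drops falling hazards at random points around itself, looping automatically with AutoSpawn or firing through SpawnAOEZoneAndHazard.
; SpawnAOEZone randomizes speed, size and force, temporarily teleports the actor within AOERange and spawns a warning zone.
; After a random delay, SpawnHazard launches a hazard from overhead with predicted impact time, links it to the zone and restores the transform.
; Construction script previews size, color and range.
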(event Custom|Spawn%20Hazard
  (bind _returnvalue (Transformation|GetActorLocation))
  (bind _temphazardsize (Variables|Default|GettempHazardSize))
  (bind _temphazardspeed (Variables|Default|GettempHazardSpeed))
  (bind _returnvalue_2 (+ _returnvalue "0.000000,0.000000,2000.000000" ""))
  (bind _returnvalue_3 (Math|Transform|MakeTransform _returnvalue_2))
  (bind _returnvalue_4 (Class|KismetAnimationLibrary|Lookat _returnvalue_3 _returnvalue "1.000000,0.000000,0.000000" false "0, 0, 0" 0.0))
  (bind _location (Math|Transform|BreakTransform _returnvalue_4))
  (bind _returnvalue_5 (Game|SpawnActorfromClass "/Game/Freelance/Programming/LevelHazards/BP_GM1_LvlHazardObj.BP_GM1_LvlHazardObj_C" _returnvalue_4 "AlwaysSpawn" "MultiplyWithRoot" 0 0))
  (Variables|/Game/Freelance/Programming/LevelHazards/BP_GM1_AOEZone.BP_GM1_AOEZone_C|SetwatchingHazard (stale Custom|Spawn%20AOE%20Zone _returnvalue_2) _returnvalue_5)
  ;[0 0 0] Scales Hazard
  (Transformation|SetActorScale3D _returnvalue_5 (* (Class|KismetMathLibrary|VectorOne) _temphazardsize))
  (Variables|/Script/Engine.RadialForceComponent|SetRadius (Variables|/Game/Freelance/Programming/LevelHazards/BP_GM1_LvlHazardObj.BP_GM1_LvlHazardObj_C|GetExplosion%20Force _returnvalue_5) (* _temphazardsize 5e+01))
  (Variables|/Script/Engine.RadialForceComponent|SetImpulseStrength (Variables|/Game/Freelance/Programming/LevelHazards/BP_GM1_LvlHazardObj.BP_GM1_LvlHazardObj_C|GetExplosion%20Force _returnvalue_5) (Variables|Default|GettempImpactForce))
  (Physics|AddImpulse (Variables|/Game/Freelance/Programming/LevelHazards/BP_GM1_LvlHazardObj.BP_GM1_LvlHazardObj_C|GetSphereCol _returnvalue_5) (* (Math|Vector|Normalize (- _returnvalue _location)) _temphazardspeed) "None" true)
  (Default|HazardLaunch _returnvalue_5 _returnvalue (/ (Math|Vector|Distance(Vector) _location _returnvalue) _temphazardspeed) "/Game/Freelance/Audio/LevelHazards/sfx_env_Hazard_Impact_2.sfx_env_Hazard_Impact_2")
  (Transformation|SetActorTransform (Variables|Default|GetoriginalTrasform) false true))

(event Custom|Spawn%20AOE%20Zone
  (bind _returnvalue (Math|Random|RandomFloatinRange 0.0 3.6e+02))
  (bind _hazard_speed (Variables|Default|GetHazard%20Speed))
  (bind _impact_force (Variables|Default|GetImpact%20Force))
  (bind _hazard_size (Variables|Default|GetHazard%20Size))
  (bind (_x _y) (Math|Vector2D|BreakVector2D _hazard_speed))
  (bind (_x_2 _y_2) (Math|Vector2D|BreakVector2D _impact_force))
  (bind (_x_3 _y_3) (Math|Vector2D|BreakVector2D _hazard_size))
  ;[0 0 0] Save old Transform and create new random offset transform
  ;[0 0 0] Random Point in XY Circle
  (bind _output_get (Variables|Default|SettempRandRange (Math|Random|RandomFloatinRange 0.0 (Variables|Default|GetAOE%20Range))))
  ;[0 0 0] Setup and Save Random Values
  (Variables|Default|SettempHazardSpeed (Math|Random|RandomFloatinRange _x _y))
  (Variables|Default|SettempHazardSize (Math|Random|RandomFloatinRange _x_3 _y_3))
  (Variables|Default|SettempImpactForce (Math|Random|RandomFloatinRange _x_2 _y_2))
  (Variables|Default|SetoriginalTrasform (Transformation|GetActorTransform))
  (Transformation|SetActorLocation (+ (Transformation|GetActorLocation) (* (Math|Vector|MakeVector (Math|Trig|Sin(Degrees) _returnvalue) (Math|Trig|Cos(Degrees) _returnvalue) 0.0) _output_get)) false true)
  (bind _returnvalue_2 (Game|SpawnActorfromClass "/Game/Freelance/Programming/LevelHazards/BP_GM1_AOEZone.BP_GM1_AOEZone_C" (Transformation|GetActorTransform) "AlwaysSpawn" "MultiplyWithRoot" 0 0))
  ;[0 0 0] Scales AOE Zone
  (Transformation|SetActorScale3D _returnvalue_2 (* (Class|KismetMathLibrary|VectorOne) (Variables|Default|GettempHazardSize)))
  (Variables|/Game/Freelance/Programming/LevelHazards/BP_GM1_AOEZone.BP_GM1_AOEZone_C|SetorigScale _returnvalue_2 (Variables|Default|GettempHazardSize))
  (Rendering|Components|Decal|SetDecalColor (Variables|/Game/Freelance/Programming/LevelHazards/BP_GM1_AOEZone.BP_GM1_AOEZone_C|GetAOE%20Zone%20Decal _returnvalue_2) (Variables|Default|GetAOE%20Color)))

(event Custom|Spawn%20AOE%20Zone%20And%20Hazard
  (bind _aoe_time (Variables|Default|GetAOE%20Time))
  (bind (_x _y) (Math|Vector2D|BreakVector2D _aoe_time))
  (CallFunction|SpawnAOEZone)
  (Utilities|FlowControl|Delay (Math|Random|RandomFloatinRange _x _y))
  (CallFunction|SpawnHazard))

(event EventBeginPlay
  (bind _launch_delay (Variables|Default|GetLaunch%20Delay))
  (bind _aoe_time (Variables|Default|GetAOE%20Time))
  (bind (_x _y) (Math|Vector2D|BreakVector2D _launch_delay))
  (bind (_x_2 _y_2) (Math|Vector2D|BreakVector2D _aoe_time))
  (bind _returnvalue (Math|Random|RandomFloatinRange _x _y))
  ;[0 0 0] Auto Spawn
  (if (Variables|Default|GetAuto%20Spawn) :!label _label
    (Utilities|FlowControl|Delay _returnvalue)
    (CallFunction|SpawnAOEZone)
    (Utilities|FlowControl|Delay (Math|Random|RandomFloatinRange _x_2 _y_2))
    (CallFunction|SpawnHazard)
    (if true
      (Utilities|FlowControl|Delay _returnvalue)
      (goto _label))))

(event Collision|EventActorBeginOverlap
  (params (OtherActor :type Actor%20Object%20Reference)))

(event EventTick
  (params (DeltaSeconds :type Float%20%28single-precision%29)))

(fn ConstructionScript
  (bind _visual__editor_only_ (Variables|Default|GetVisual%20%28EDITOR%20ONLY%29))
  (Transformation|SetWorldScale3D _visual__editor_only_ (Math|Conversions|ToVector(Float) (.X (Math|Vector2D|BreakVector2D (Variables|Default|GetHazard%20Size)))))
  (Rendering|Components|Decal|SetDecalColor _visual__editor_only_ (Variables|Default|GetAOE%20Color))
  (Rendering|Debug|DrawDebugCircle (Transformation|GetActorLocation) (Variables|Default|GetAOE%20Range) 32 "(R=0.000000,G=0.000000,B=1.000000,A=1.000000)" 1.0 5.0 "0.000000,1.000000,0.000000" "1.000000,0.000000,0.000000"))