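; BP_GM1_LvlHazardObj is a level hazard object that falls or flies to a predicted impact point and delivers an explosive impulse.
; HazardLaunch waits the supplied time until impact, then teleports the actor to the hit location and zeroes the sphere collision's velocity.
; It then fires the radial force, hides itself, swaps fall audio for impact audio and destroys itself after a short delay.
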(event Custom|HazardLaunch
  (params (HitLocation :type Vector) (TimeTillHit :type Float%20%28double-precision%29) (Impact%20SW :type Sound%20Wave%20Object%20Reference))
  (Utilities|FlowControl|Delay TimeTillHit) ; Wait till predicted impact time
  (Transformation|SetActorLocation HitLocation false true) ; Teleport to Impact Location
  (Physics|SetPhysicsLinearVelocity (Variables|Default|GetSphereCol) "0, 0, 0" false "None")
  (Class|RadialForceComponent|FireImpulse (Variables|Default|GetExplosion%20Force))
  (Rendering|SetActorHiddenInGame true)
  (Audio|Components|Audio|Stop (Variables|Default|GetHazard%20Fall%20Audio))
  (Audio|Components|Audio|Play (Variables|Default|GetHazard%20Impact%20Audio) 0.0)
  (Utilities|FlowControl|Delay 2.0)
  (Actor|DestroyActor))

(event EventBeginPlay)

(event Collision|EventActorBeginOverlap
  (params (OtherActor :type Actor%20Object%20Reference)))

(event EventTick
  (params (DeltaSeconds :type Float%20%28single-precision%29)))

(fn ConstructionScript)