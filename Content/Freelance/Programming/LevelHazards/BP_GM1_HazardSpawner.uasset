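; Level hazard spawner for GM_GM1 that drops data-configured hazards around itself, optionally auto-starting after game start and an initial delay.
; Each cycle places a colored AOE warning zone at a random spot within a range, waits a heads-up time, then launches a hazard downward from above.
; Size scales hazard force, distance over speed times the impact, and a randomized timer optionally repeats the cycle.
; The construction script previews size, color and range.
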(event Custom|Spawn%20AOE%20Zone%20And%20Hazard
  (bind (_zone _speed _size) (CallFunction|SpawnAOEZone))
  (Utilities|FlowControl|Delay (Variables|/Game/GameMode1/Programming/PDA_HazardSpawner.PDA_HazardSpawner_C|GetHeads-up%20Time (Variables|Default|GetData)))
  (CallFunction|SpawnHazard _zone _speed _size)
  (if (Variables|Default|GetbContinueSpawn)
    (Utilities|Time|SetTimerbyEvent (delegate Custom|Spawn%20AOE%20Zone%20And%20Hazard) (Utilities|RandomfromRange (Variables|/Game/GameMode1/Programming/PDA_HazardSpawner.PDA_HazardSpawner_C|GetTarget%20Timer (Variables|Default|GetData))))))

(event Custom|Start%20Game
  (Utilities|FlowControl|Delay (Variables|/Game/GameMode1/Programming/PDA_HazardSpawner.PDA_HazardSpawner_C|GetInitial%20Delay (Variables|Default|GetData)))
  (if (Variables|/Game/GameMode1/Programming/PDA_HazardSpawner.PDA_HazardSpawner_C|GetAuto%20Start (Variables|Default|GetData))
    (CallFunction|SpawnAOEZoneandHazard)))

(event EventBeginPlay
  (bind _asgm_gm1 (Utilities|Casting|CastToGM_GM1 (Game|GetGameMode)))
  (EventDispatchers|BindEventtoOnStartGame _asgm_gm1 (delegate Custom|Start%20Game)))

(event Collision|EventActorBeginOverlap
  (params (OtherActor :type Actor%20Object%20Reference)))

(event EventTick
  (params (DeltaSeconds :type Float%20%28single-precision%29)))

(fn ConstructionScript
  (bind _returnvalue (Transformation|GetActorLocation))
  (bind _visual__editor_only_ (Variables|Default|GetVisual%20%28EDITOR%20ONLY%29))
  (bind _data (Variables|Default|GetData))
  (bind _aoe_range (Variables|/Game/GameMode1/Programming/PDA_HazardSpawner.PDA_HazardSpawner_C|GetAOE%20Range _data))
  (bind (_lowerbound _upperbound) (Utilities|Struct|BreakFloatRange _aoe_range))
  (Transformation|SetWorldScale3D _visual__editor_only_ (Math|Conversions|ToVector(Float) (.Value (Utilities|Struct|BreakFloatRangeBound (.LowerBound (Utilities|Struct|BreakFloatRange (Variables|/Game/GameMode1/Programming/PDA_HazardSpawner.PDA_HazardSpawner_C|GetHazard%20Size (Variables|Default|GetData))))))))
  (Rendering|Components|Decal|SetDecalColor _visual__editor_only_ (Variables|/Game/GameMode1/Programming/PDA_HazardSpawner.PDA_HazardSpawner_C|GetAOE%20Color _data))
  (Rendering|Debug|DrawDebugCircle _returnvalue (.Value (Utilities|Struct|BreakFloatRangeBound _lowerbound)) 32 "(R=0.000000,G=0.500000,B=1.000000,A=1.000000)" 1.0 5.0 "0.000000,1.000000,0.000000" "1.000000,0.000000,0.000000")
  (Rendering|Debug|DrawDebugCircle _returnvalue (.Value (Utilities|Struct|BreakFloatRangeBound _upperbound)) 24 "(R=0.000000,G=0.500000,B=1.000000,A=1.000000)" 1.0 5.0 "0.000000,1.000000,0.000000" "1.000000,0.000000,0.000000"))

(fn SpawnAOEZone
  (bind _returnvalue (Game|SpawnActorfromClass "/Game/Freelance/Programming/LevelHazards/BP_GM1_AOEZone.BP_GM1_AOEZone_C" (Math|Transform|MakeTransform (+ (Transformation|GetActorLocation) (* (Utilities|RandomfromRange (Variables|/Game/GameMode1/Programming/PDA_HazardSpawner.PDA_HazardSpawner_C|GetAOE%20Range (Variables|Default|GetData))) (Math|Vector|Normalize (Math|Vector|MakeVector (Math|Random|RandomFloatinRange -1.0 1.0) (Math|Random|RandomFloatinRange -1.0 1.0) 0.0)))) "0, 0, 0" (Math|Conversions|ToVector(Float) (Utilities|RandomfromRange (Variables|/Game/GameMode1/Programming/PDA_HazardSpawner.PDA_HazardSpawner_C|GetHazard%20Size (Variables|Default|GetData))))) "AlwaysSpawn" "MultiplyWithRoot" 0 0))
  (Rendering|Components|Decal|SetDecalColor (Variables|/Game/Freelance/Programming/LevelHazards/BP_GM1_AOEZone.BP_GM1_AOEZone_C|GetAOE%20Zone%20Decal _returnvalue) (Variables|/Game/GameMode1/Programming/PDA_HazardSpawner.PDA_HazardSpawner_C|GetAOE%20Color (Variables|Default|GetData)))
  (return _returnvalue (Utilities|RandomfromRange (Variables|/Game/GameMode1/Programming/PDA_HazardSpawner.PDA_HazardSpawner_C|GetHazard%20Speed (Variables|Default|GetData))) (Variables|/Game/Freelance/Programming/LevelHazards/BP_GM1_AOEZone.BP_GM1_AOEZone_C|GettargetSize _returnvalue)))

(fn SpawnHazard
  (params (AOE%20Zone :type BP%20GM1%20AOE%20Zone%20Object%20Reference) (Speed :type Float%20%28double-precision%29) (Size :type Float%20%28double-precision%29))
  (bind _returnvalue (Math|Conversions|ToVector(Float) Size))
  (bind _returnvalue_2 (Transformation|GetActorLocation AOE%20Zone))
  (bind _returnvalue_3 (Transformation|GetActorLocation AOE%20Zone))
  (bind _returnvalue_4 (+ _returnvalue_2 "0.000000,0.000000,2000.000000"))
  (bind _returnvalue_5 (Math|Transform|MakeTransform _returnvalue_4 "0, 0, 0" _returnvalue))
  (bind _returnvalue_6 (Class|KismetAnimationLibrary|Lookat _returnvalue_5 _returnvalue_2 "1.000000,0.000000,0.000000" false "0, 0, 0" 0.0))
  (bind _returnvalue_7 (Game|SpawnActorfromClass (Variables|/Game/GameMode1/Programming/PDA_HazardSpawner.PDA_HazardSpawner_C|GetHazard%20Type (Variables|Default|GetData)) _returnvalue_6 "AlwaysSpawn" "MultiplyWithRoot" 0 0))
  (Variables|/Game/Freelance/Programming/LevelHazards/BP_GM1_AOEZone.BP_GM1_AOEZone_C|SetwatchingHazard AOE%20Zone _returnvalue_7)
  (Default|SetHazardSettings _returnvalue_7 Speed Size (Utilities|GetHazardForcefromSize Size))
  (Physics|AddImpulse (Variables|/Game/Freelance/Programming/LevelHazards/BP_GM1_Hazard.BP_GM1_Hazard_C|GetSphereCol _returnvalue_7) (* "0.000000,0.000000,-1.000000" Speed) "None" true)
  (Default|DelayImpact _returnvalue_7 _returnvalue_3 (/ (Math|Vector|Distance(Vector) (.Location (Math|Transform|BreakTransform _returnvalue_6)) _returnvalue_3) Speed) "/Game/Freelance/Audio/LevelHazards/sfx_env_Hazard_Impact_2.sfx_env_Hazard_Impact_2"))