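; BP_GM1_KnockbackHazard is a level hazard that knocks back its surroundings with a radial impulse.
; It overrides Impact to fire the ExplosionForce component's impulse.
; Its SetSpeedAndSize override passes zero speed to the parent, scales the blast radius with size, and randomizes impulse strength within the Force range.
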(event EventBeginPlay
  (|CallParentFunction) ; This node is disabled and will not be called.\nDrag off pins to build functionality.
)

(event Collision|EventActorBeginOverlap
  (params (OtherActor :type Actor%20Object%20Reference))
  (|CallParentFunction OtherActor) ; This node is disabled and will not be called.\nDrag off pins to build functionality.
)

(event EventTick
  (params (DeltaSeconds :type Float%20%28single-precision%29))
  (|CallParentFunction DeltaSeconds) ; This node is disabled and will not be called.\nDrag off pins to build functionality.
)

(fn ConstructionScript
  (|CallParentFunction))

(fn Impact
  (Class|RadialForceComponent|FireImpulse (Variables|Default|GetExplosionForce)))

(fn SetSpeedandSize
  (params (speed :type Float%20%28double-precision%29) (size :type Float%20%28double-precision%29))
  (bind _force (Variables|Default|GetForce))
  (bind _explosionforce (Variables|Default|GetExplosionForce))
  (bind (_lowerbound _upperbound) (Utilities|Struct|BreakFloatRange _force))
  (|CallParentFunction 0.0 size)
  (Variables|/Script/Engine.RadialForceComponent|SetRadius _explosionforce (* size 5e+01))
  (Variables|/Script/Engine.RadialForceComponent|SetImpulseStrength _explosionforce (Math|Random|RandomFloatinRange (.Value (Utilities|Struct|BreakFloatRangeBound _lowerbound)) (.Value (Utilities|Struct|BreakFloatRangeBound _upperbound)))))