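; BP_GM1_Hazard is a falling level hazard with an empty Impact function, apparently meant for child hazards to override.
; DelayImpact waits for the predicted hit time, teleports the actor to the hit location, zeroes its sphere's velocity, then calls Impact.
; It swaps fall audio for impact audio, hides itself, and polls until the sound finishes before destroying itself.
; SetSpeedAndSize stores only the size; Speed is unused.
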(event Custom|DelayImpact
  (params (HitLocation :type Vector) (TimeTillHit :type Float%20%28double-precision%29) (Impact%20SW :type Sound%20Wave%20Object%20Reference))
  (bind _hazard_impact_audio (Variables|Default|GetHazard%20Impact%20Audio))
  (Utilities|FlowControl|Delay TimeTillHit) ; Wait till predicted impact time
  (Transformation|SetActorLocation HitLocation false true) ; Teleport to Impact Location
  (Physics|SetPhysicsLinearVelocity (Variables|Default|GetSphereCol) "0, 0, 0" false "None")
  (CallFunction|Impact)
  (Audio|Components|Audio|Stop (Variables|Default|GetHazard%20Fall%20Audio))
  (Audio|Components|Audio|Play _hazard_impact_audio 0.0)
  (Rendering|SetActorHiddenInGame true)
  (Utilities|FlowControl|Delay 0.5 :!label _label)
  (if (Audio|Components|Audio|IsPlaying _hazard_impact_audio)
    (goto _label)
    (else
      (Actor|DestroyActor))))

(event EventBeginPlay)

(event Collision|EventActorBeginOverlap
  (params (OtherActor :type Actor%20Object%20Reference)))

(event EventTick
  (params (DeltaSeconds :type Float%20%28single-precision%29)))

(fn ConstructionScript)

(fn Impact)

(fn SetSpeedandSize
  (params (speed :type Float%20%28double-precision%29) (size :type Float%20%28double-precision%29))
  (Variables|Default|SetHazard%20Size size))