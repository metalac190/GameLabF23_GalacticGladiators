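; Lobby game mode that spawns input pawns on BeginPlay and validates joined players before starting the match.
; TryGameStart counts connected players in the game instance's PlayerData, currently accepting one, and rejects duplicate models through a nested pairwise enum comparison.
; On success, OpenNextLevel always loads the GameMode 2 whitebox level.
; Tournament, random-mode and level-select branching is disconnected, as are several older validation attempts.
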(event Custom|Try%20Game%20Start
  (bind _currentgameinstance (Variables|Default|GetCurrentGameInstance))
  (bind _currentgameinstance_2 (Variables|Default|GetCurrentGameInstance))
  (bind _playerdata (Variables|/Game/Core/Programming/Prototypes/GameData/GI_CORE_GameInstance.GI_CORE_GameInstance_C|GetPlayerData _currentgameinstance))
  (Development|PrintString "GM: Try Game Start")
  ;[0 0 0] Check if more than one player has joined
  (Variables|Local|SetPlayerCount 0)
  (for _array_element (Variables|/Game/Core/Programming/Prototypes/GameData/GI_CORE_GameInstance.GI_CORE_GameInstance_C|GetPlayerData (Variables|Default|GetCurrentGameInstance))
    (if (.PlayerConnected (Utilities|Struct|BreakBP_PlayerData _array_element))
      (Math|Integer|IncrementInt (Variables|Local|GetPlayerCount))))
  (if (> (Variables|Local|GetPlayerCount) 0)
    ;[0 0 0] Check players dont have the same models
    (Variables|Local|SetSameModel false)
    (for (_array_element_2 _array_index) _playerdata
      (for (_array_element_3 _array_index_2) _playerdata
        (bind _int (Default|GetIntfromEnum _currentgameinstance_2 (.PlayerModel (Utilities|Struct|BreakBP_PlayerData _array_element_2))))
        (bind _int_2 (Default|GetIntfromEnum _currentgameinstance_2 (.PlayerModel (Utilities|Struct|BreakBP_PlayerData _array_element_3))))
        (if (Math|Boolean|ANDBoolean (and (.PlayerConnected (Utilities|Struct|BreakBP_PlayerData _array_element_2)) (.PlayerConnected (Utilities|Struct|BreakBP_PlayerData _array_element_3))) (== _int _int_2) (!= _array_index _array_index_2)) ; If any have same model set to true
          (Variables|Local|SetSameModel true))))
    (if (Variables|Local|GetSameModel) ; After loop check if any were same
      (Development|PrintString "players cannot have the same model")
      (else
        (Development|PrintString "CheckSuccessful")
        (CallFunction|OpenNextLevel)))
    (else
      (Development|PrintText "Requires more than one player to start"))))

(event EventBeginPlay
  (CallFunction|SpawnInputPawns))

(fn ConstructionScript)

(fn OpenNextLevel
  ;[1 1 1] Tournament
  ;;[1 1 1] Starts with GameMode 2
  (Development|PrintString "Starting with GameMode 2")
  (Game|OpenLevel(byObjectReference) "/Game/GameMode2/Design/Maps/GM2_LD_Whitebox_CURRENT.GM2_LD_Whitebox_CURRENT"))