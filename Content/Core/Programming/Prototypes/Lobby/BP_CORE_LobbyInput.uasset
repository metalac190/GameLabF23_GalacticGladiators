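; BP_CORE_LobbyInput is a prototype that handles lobby input for the player identified by PlayerID.
; On BeginPlay it caches the first top-level WBP_CORE_LobbyMenu widget and the GM_CORE_Lobby game mode.
; Enhanced Input actions drive the widget to register a join, only once per player, or to select the next option for color changing.
; The start action asks the game mode to attempt starting the game.
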(event Input|EnhancedActionEvents|EnhancedInputActionIA_CORE_Join
  (params (ActionValue :type Boolean) (ElapsedSeconds :type Float%20%28double-precision%29) (TriggeredSeconds :type Float%20%28double-precision%29) (InputAction :type Input%20Action%20Object%20Reference :default "/Game/Core/Programming/Prototypes/Lobby/Input/IA_CORE_Join.IA_CORE_Join"))
  (bind _playerid (Variables|Default|GetPlayerID))
  (:Started
    ;[0 0 0] Player Joining Lobby
    (if (not (Utilities|Array|Get(acopy) (Variables|/Game/Core/Programming/Prototypes/Lobby/WBP_CORE_LobbyMenu.WBP_CORE_LobbyMenu_C|GetPlayerHasJoined (Variables|Default|GetLobbyWidget)) (Variables|Default|GetPlayerID)))
      (Default|PlayerJoinedEvent (Variables|Default|GetLobbyWidget) _playerid)
      (Development|PrintText (Utilities|Text|FormatText "Player Joined: {0}" _playerid)))))

(event Input|EnhancedActionEvents|EnhancedInputActionIA_CORE_Start
  (params (ActionValue :type Boolean) (ElapsedSeconds :type Float%20%28double-precision%29) (TriggeredSeconds :type Float%20%28double-precision%29) (InputAction :type Input%20Action%20Object%20Reference :default "/Game/Core/Programming/Prototypes/Lobby/Input/IA_CORE_Start.IA_CORE_Start"))
  (:Started
    ;[0 0 0] Players Press Enter to Continue Game
    (Default|TryGameStart (Variables|Default|GetGM))))

(event Input|EnhancedActionEvents|EnhancedInputActionIA_CORE_NextSelect
  (params (ActionValue :type Boolean) (ElapsedSeconds :type Float%20%28double-precision%29) (TriggeredSeconds :type Float%20%28double-precision%29) (InputAction :type Input%20Action%20Object%20Reference :default "/Game/Core/Programming/Prototypes/Lobby/Input/IA_CORE_NextSelect.IA_CORE_NextSelect"))
  (:Started
    ;[0 0 0] Changing Color
    (Default|SelectNextEvent (Variables|Default|GetLobbyWidget) (Variables|Default|GetPlayerID))))

(event EventBeginPlay
  ;[1 1 1] Get Lobby Widget
  (bind _foundwidgets (Widget|GetAllWidgetsOfClass "/Game/Core/Programming/Prototypes/Lobby/WBP_CORE_LobbyMenu.WBP_CORE_LobbyMenu_C" true))
  (Variables|Default|SetLobbyWidget (Utilities|Array|Get(acopy) _foundwidgets))
  ;[1 1 1] Set GameMode Variable
  (bind _asgm_core_lobby (Utilities|Casting|CastToGM_CORE_Lobby (Game|GetGameMode)))
  (Variables|Default|SetGM _asgm_core_lobby))

(fn ConstructionScript)