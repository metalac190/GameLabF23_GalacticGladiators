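; Prototype announcer Blueprint for the GM2 game mode that plays voice-over lines at match start, match end and on player kills.
; On BeginPlay it caches the game instance and game mode, then binds to start and end events, hooking each player's kill event once the match starts.
; Cues come from the game instance's audio atlas and play in 2D, with the victory line chosen by winner index.
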(event Custom|OnStartGameVO
  (CallFunction|OnStartGame)
  (for _array_element (Variables|/Game/GameMode2/Programming/Gamemode/GM_GM2.GM_GM2_C|GetPlayers (Variables|Default|GetGameMode))
    (EventDispatchers|BindEventtoOnPlayerKill _array_element (delegate Custom|OnPlayerKillVO))))

(event Custom|OnEndGameVO
  (CallFunction|OnEndGame))

(event Custom|OnPlayerKillVO
  (CallFunction|OnPlayerKill (stale Custom|OnStartGameVO _array_element)))

(event EventBeginPlay
  (CallFunction|GatherVariables)
  (EventDispatchers|BindEventtoOnStartGame (Variables|Default|GetGameMode) (delegate Custom|OnStartGameVO))
  (EventDispatchers|BindEventtoOnEndGame (Variables|Default|GetGameMode) (delegate Custom|OnEndGameVO)))

(fn ConstructionScript)

(fn GatherVariables
  (bind _asgi_core_game_instance (Utilities|Casting|CastToGI_CORE_GameInstance (Game|GetGameInstance)))
  (Variables|Default|SetGameInstance _asgi_core_game_instance)
  (bind _asgm_gm2 (Utilities|Casting|CastToGM_GM2 (Game|GetGameMode)))
  (Variables|Default|SetGameMode _asgm_gm2))

(fn OnStartGame
  (bind _soundcue (Default|GetSoundCue (Variables|/Game/Core/Programming/Prototypes/GameData/GI_CORE_GameInstance.GI_CORE_GameInstance_C|GetCoreAudioAtlas (Variables|Default|GetGameInstance)) "NewEnumerator18"))
  (Audio|PlaySound2D _soundcue 1.0 1.0 0.0 0 0)
  (Development|PrintString "VO: Played Match Start VO"))

(fn OnEndGame
  (LocalVariables|SetAudioAtlas (Variables|/Game/Core/Programming/Prototypes/GameData/GI_CORE_GameInstance.GI_CORE_GameInstance_C|GetCoreAudioAtlas (Variables|Default|GetGameInstance)))
  ;[1 1 1] Will Play Victory VO based on Winner
  (bind _playerscore (Default|GetCurrentWinner (Variables|Default|GetGameInstance)))
  (switch int (.playerindex _playerscore)
    (:0
      (bind _soundcue (Default|GetSoundCue (LocalVariables|GetAudioAtlas) "NewEnumerator19"))
      (LocalVariables|SetPlayedSC _soundcue))
    (:1
      (bind _soundcue_2 (Default|GetSoundCue (LocalVariables|GetAudioAtlas) "NewEnumerator20"))
      (LocalVariables|SetPlayedSC _soundcue_2))
    (:2
      (bind _soundcue_3 (Default|GetSoundCue (LocalVariables|GetAudioAtlas) "NewEnumerator21"))
      (LocalVariables|SetPlayedSC _soundcue_3))
    (:3
      (bind _soundcue_4 (Default|GetSoundCue (LocalVariables|GetAudioAtlas) "NewEnumerator22"))
      (LocalVariables|SetPlayedSC _soundcue_4)))
  (Audio|PlaySound2D (LocalVariables|GetPlayedSC) 1.0 1.0 0.0 0 0))

(fn OnPlayerKill
  (params (KilledPlayer :type PC%20GM2%20Player%20Object%20Reference))
  (bind _soundcue (Default|GetSoundCue (Variables|/Game/Core/Programming/Prototypes/GameData/GI_CORE_GameInstance.GI_CORE_GameInstance_C|GetCoreAudioAtlas (Variables|Default|GetGameInstance)) "NewEnumerator23"))
  (Audio|PlaySound2D _soundcue 1.0 1.0 0.0 0 0))