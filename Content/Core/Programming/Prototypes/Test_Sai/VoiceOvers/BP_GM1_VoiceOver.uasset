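; Prototype voice-over manager for the GM1 game mode, playing 2D announcer cues from the game instance's audio atlas.
; It binds to game start and end, then to each player's hit and death events at start.
; Tick latches a flag once any player is on ice, and a looping timer, randomised once, plays the ice line while set.
; The random-VO pause is unwired, and its flag is never read.
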(event Custom|OnHitVO
  (params (hitBy :type Actor%20Object%20Reference))
  ;[1 1 1] Bind to Player Events
  (CallFunction|OnHit hitBy (stale Custom|OnStartGameVO _array_element)))

(event Custom|OnDieVO
  (params (player :type Actor%20Object%20Reference))
  ;[1 1 1] Bind to Player Events
  (CallFunction|OnDie player))

(event Custom|OnStartGameVO
  (bind _gameinstance (Variables|Default|GetGameInstance))
  (bind _gameinstancevariables (Variables|/Game/Core/Programming/Prototypes/GameData/GI_CORE_GameInstance.GI_CORE_GameInstance_C|GetGameInstanceVariables _gameinstance))
  (bind _timebetweenvo (Variables|/Game/Core/Programming/Prototypes/Test_Sai/PDA_GameInstanceSettings.PDA_GameInstanceSettings_C|GetTimeBetweenVO _gameinstancevariables))
  ;[1 1 1] Bind to GameMode Events
  (CallFunction|OnStartGame)
  ;[1 1 1] Get Players
  (Variables|Default|SetPlayers (Variables|/Game/Systems/Blueprints/GM1/Systems/GM_GM1.GM_GM1_C|GetPlayers (Variables|Default|GetGameMode)))
  ;[1 1 1] Bind to Player Events
  (for _array_element (Variables|Default|GetPlayers)
    (EventDispatchers|BindEventtoOnHit _array_element (delegate Custom|OnHitVO))
    (Development|PrintString "VO: Bound to On Hit")
    (EventDispatchers|BindEventtoOnDie _array_element (delegate Custom|OnDieVO))
    (Development|PrintString "VO: Bound to On Die"))
  ;[1 1 1] On Ice VO
  (Utilities|Time|SetTimerbyEvent (delegate Custom|OnIceVO) (Math|Random|RandomFloatinRange (.x _timebetweenvo) (.y _timebetweenvo)) true))

(event Custom|OnEndGameVO
  ;[1 1 1] Bind to GameMode Events
  (CallFunction|OnEndGame))

(event Custom|PauseRandomVO
  (params (Duration :type Float%20%28single-precision%29))
  ;[1 1 1] Pause the Random Voice Lines
  (Variables|Default|SetAllowRandomVO false)
  (Utilities|FlowControl|Delay Duration)
  (Variables|Default|SetAllowRandomVO true))

(event Custom|OnIceVO
  ;[1 1 1] On Ice VO
  (if (Variables|Default|GetPlayerOnIce)
    (CallFunction|OnIce)))

(event EventBeginPlay
  ;[1 1 1] Gather Variables
  (bind _asgi_core_game_instance (Utilities|Casting|CastToGI_CORE_GameInstance (Game|GetGameInstance))
    (:then
      (Variables|Default|SetGameInstance _asgi_core_game_instance)
      (bind _asgm_gm1 (Utilities|Casting|CastToGM_GM1 (Game|GetGameMode))
        (:then
          (Variables|Default|SetGameMode _asgm_gm1)
          ;[1 1 1] Bind to GameMode Events
          (EventDispatchers|BindEventtoOnStartGame (Variables|Default|GetGameMode) (delegate Custom|OnStartGameVO))
          (EventDispatchers|BindEventtoOnEndGame (Variables|Default|GetGameMode) (delegate Custom|OnEndGameVO)))
        (:CastFailed
          (Development|PrintString "VO: Cannot find GM_GM1"))))
    (:CastFailed
      (Development|PrintString "VO: cannot find game instance"))))

(event EventTick
  (params (DeltaSeconds :type Float%20%28single-precision%29))
  (if (not (Variables|Default|GetPlayerOnIce))
    ;[1 1 1] check if any player is on ice
    (bind _array_element (Utilities|Array|ForEachLoopwithBreak (Variables|Default|GetPlayers) :!label _label)
      (:LoopBody
        (bind _result (Default|IsonSurfaceType _array_element "SurfaceType1"))
        (if _result
          (Variables|Default|SetPlayerOnIce true)
          (goto _label Break))))))

(fn ConstructionScript)

(fn OnHit
  (params (HitBy :type Actor%20Object%20Reference) (HitPlayer :type Actor%20Object%20Reference))
  (Development|PrintString "VO: On Player Hit")
  (bind _soundcue (Default|GetSoundCue (Variables|/Game/Core/Programming/Prototypes/GameData/GI_CORE_GameInstance.GI_CORE_GameInstance_C|GetCoreAudioAtlas (Variables|Default|GetGameInstance)) "NewEnumerator0"))
  (Audio|PlaySound2D _soundcue 1.0 1.0 0.0 0 0))

(fn OnDie
  (params (Player :type Actor%20Object%20Reference))
  (Development|PrintString "VO: On Player Die")
  (bind _soundcue (Default|GetSoundCue (Variables|/Game/Core/Programming/Prototypes/GameData/GI_CORE_GameInstance.GI_CORE_GameInstance_C|GetCoreAudioAtlas (Variables|Default|GetGameInstance)) "NewEnumerator9"))
  (Audio|PlaySound2D _soundcue 1.0 1.0 0.0 0 0))

(fn OnStartGame
  (Development|PrintString "VO: On Start Game")
  (Variables|Default|SetAllowRandomVO true)
  (bind _soundcue (Default|GetSoundCue (Variables|/Game/Core/Programming/Prototypes/GameData/GI_CORE_GameInstance.GI_CORE_GameInstance_C|GetCoreAudioAtlas (Variables|Default|GetGameInstance)) "NewEnumerator18"))
  (Audio|PlaySound2D _soundcue 1.0 1.0 0.0 0 0))

(fn OnEndGame
  (Development|PrintString "VO: On End Game")
  (Variables|Default|SetAllowRandomVO false)
  (bind _soundcue (Default|GetSoundCue (Variables|/Game/Core/Programming/Prototypes/GameData/GI_CORE_GameInstance.GI_CORE_GameInstance_C|GetCoreAudioAtlas (Variables|Default|GetGameInstance)) "NewEnumerator16"))
  (Audio|PlaySound2D _soundcue 1.0 1.0 0.0 0 0))

(fn OnIce
  (Development|PrintString "VO: On Player Ice")
  (bind _soundcue (Default|GetSoundCue (Variables|/Game/Core/Programming/Prototypes/GameData/GI_CORE_GameInstance.GI_CORE_GameInstance_C|GetCoreAudioAtlas (Variables|Default|GetGameInstance)) "NewEnumerator10"))
  (Audio|PlaySound2D _soundcue 1.0 1.0 0.0 0 0))