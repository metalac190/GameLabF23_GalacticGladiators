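; Sound effects manager for the GM2 game mode that plays one-shot positional sounds for player and star gameplay events.
; On BeginPlay it gets the FXManager from GM_GM2 and the audio atlas from the game instance, then binds to the FXManager's collision, dash, death, steal and star lifecycle events.
; Each handler looks up a cue in the atlas by enum and plays it at the relevant location.
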(event Custom|GatherVariables
  (bind _asgm_gm2 (Utilities|Casting|CastToGM_GM2 (Game|GetGameMode)))
  (Variables|PlayerEvents|SetFXManager (Variables|/Game/GameMode2/Programming/Gamemode/GM_GM2.GM_GM2_C|GetFXManager _asgm_gm2))
  (bind _asgi_core_game_instance (Utilities|Casting|CastToGI_CORE_GameInstance (Game|GetGameInstance)))
  (Variables|PlayerEvents|SetAudioAtlas (Variables|/Game/Core/Programming/Prototypes/GameData/GI_CORE_GameInstance.GI_CORE_GameInstance_C|GetSFXGM2AudioAtlas _asgi_core_game_instance)))

(event Custom|PlayerEventBindings
  (EventDispatchers|BindEventtoGM2PlayerCollision (Variables|PlayerEvents|GetFXManager) (delegate Custom|OnPlayerCollision))
  (EventDispatchers|BindEventtoGM2PlayerDashEngaged (Variables|PlayerEvents|GetFXManager) (delegate Custom|OnPlayerDashEngaged))
  (EventDispatchers|BindEventtoGM2PlayerDashCollision (Variables|PlayerEvents|GetFXManager) (delegate Custom|OnPlayerDashCollision))
  (EventDispatchers|BindEventtoGM2PlayerDualDashCollision (Variables|PlayerEvents|GetFXManager) (delegate Custom|OnPlayerDualDashCollision))
  (EventDispatchers|BindEventtoGM2PlayerGroundCollision (Variables|PlayerEvents|GetFXManager) (delegate Custom|OnPlayerGroundCollision))
  (EventDispatchers|BindEventtoGM2PlayerDeath (Variables|PlayerEvents|GetFXManager) (delegate Custom|OnPlayerDeath))
  (EventDispatchers|BindEventtoGM2PlayerStarSteal (Variables|PlayerEvents|GetFXManager) (delegate Custom|OnStarStolen)))

(event Custom|OnStarSpawn
  (params (Star :type BP%20GM2%20Collectible%20Object%20Reference))
  (StarEvents|StarSpawn Star))

(event Custom|OnStarCollected
  (params (Star :type BP%20GM2%20Collectible%20Object%20Reference) (Player :type PC%20GM2%20Player%20Object%20Reference))
  (StarEvents|StarCollected Star Player))

(event Custom|OnLargeStarPreSpawn
  (params (Star :type BP%20GM2%20Big%20Star%20Object%20Reference))
  (StarEvents|LargeStarPreSpawn Star))

(event Custom|OnLargeStarSpawn
  (params (Star :type BP%20GM2%20Big%20Star%20Object%20Reference))
  (StarEvents|LargeStarSpawn Star))

(event Custom|OnLargeStarCollected
  (params (Star :type BP%20GM2%20Big%20Star%20Object%20Reference))
  (StarEvents|LargeStarCollected Star))

(event Custom|OnStarStolen
  (params (OldOwner :type PC%20GM2%20Player%20Object%20Reference) (NewOwner :type PC%20GM2%20Player%20Object%20Reference))
  (PlayerEvents|PlayerStarStolen OldOwner NewOwner))

(event Custom|OnPlayerCollision
  (params (Location :type Vector))
  (PlayerEvents|PlayerCollision Location))

(event Custom|OnPlayerDashEngaged
  (params (Player :type PC%20GM2%20Player%20Object%20Reference))
  (PlayerEvents|PlayerDashEngaged Player))

(event Custom|OnPlayerDashCollision
  (params (Player :type PC%20GM2%20Player%20Object%20Reference))
  (PlayerEvents|PlayerDashCollision Player))

(event Custom|OnPlayerDualDashCollision
  (params (Player1 :type PC%20GM2%20Player%20Object%20Reference) (Player2 :type PC%20GM2%20Player%20Object%20Reference))
  (PlayerEvents|PlayerDualDashCollision Player1 Player2))

(event Custom|OnPlayerGroundCollision
  (params (Player :type PC%20GM2%20Player%20Object%20Reference) (Location :type Vector))
  (PlayerEvents|PlayerGroundCollision Player Location))

(event Custom|OnPlayerDeath
  (params (Player :type PC%20GM2%20Player%20Object%20Reference))
  (PlayerEvents|PlayerDeath Player))

(event Custom|StarEventBindings
  (EventDispatchers|BindEventtoGM2StarPreSpawn (Variables|PlayerEvents|GetFXManager) (delegate Custom|OnStarPreSpawn))
  (EventDispatchers|BindEventtoGM2StarSpawn (Variables|PlayerEvents|GetFXManager) (delegate Custom|OnStarSpawn))
  (EventDispatchers|BindEventtoGM2StarCollected (Variables|PlayerEvents|GetFXManager) (delegate Custom|OnStarCollected))
  (EventDispatchers|BindEventtoGM2LargeStarPreSpawn (Variables|PlayerEvents|GetFXManager) (delegate Custom|OnLargeStarPreSpawn))
  (EventDispatchers|BindEventtoGM2LargeStarSpawn (Variables|PlayerEvents|GetFXManager) (delegate Custom|OnLargeStarSpawn))
  (EventDispatchers|BindEventtoGM2LargeStarCollected (Variables|PlayerEvents|GetFXManager) (delegate Custom|OnLargeStarCollected)))

(event Custom|OnStarPreSpawn
  (params (Star :type BP%20GM2%20Collectible%20Object%20Reference))
  (StarEvents|StarPreSpawn Star))

(event EventBeginPlay
  (CallFunction|GatherVariables)
  (CallFunction|PlayerEventBindings)
  (CallFunction|StarEventBindings))

(fn ConstructionScript)

(fn PlayerCollision
  (params (Location :type Vector))
  (bind _soundcue (Default|GetSoundCue (Variables|PlayerEvents|GetAudioAtlas) "NewEnumerator2" true))
  (Audio|PlaySoundatLocation _soundcue Location "0, 0, 0" 1.0 1.0 0.0 0 0 0 0))

(fn PlayerDashEngaged
  (params (Player :type PC%20GM2%20Player%20Object%20Reference))
  (bind _soundcue (Default|GetSoundCue (Variables|PlayerEvents|GetAudioAtlas) "NewEnumerator14" true))
  (Audio|PlaySoundatLocation _soundcue (Transformation|GetActorLocation Player) "0, 0, 0" 1.0 1.0 0.0 0 0 0 0))

(fn PlayerDashCollision
  (params (Player :type PC%20GM2%20Player%20Object%20Reference))
  (bind _soundcue (Default|GetSoundCue (Variables|PlayerEvents|GetAudioAtlas) "NewEnumerator12" true))
  (Audio|PlaySoundatLocation _soundcue (Transformation|GetActorLocation Player) "0, 0, 0" 1.0 1.0 0.0 0 0 0 0))

(fn PlayerDualDashCollision
  (params (Player1 :type PC%20GM2%20Player%20Object%20Reference) (Player2 :type PC%20GM2%20Player%20Object%20Reference))
  (bind _soundcue (Default|GetSoundCue (Variables|PlayerEvents|GetAudioAtlas) "NewEnumerator33" true))
  (Audio|PlaySoundatLocation _soundcue (Transformation|GetActorLocation Player1) "0, 0, 0" 1.0 1.0 0.0 0 0 0 0))

(fn PlayerGroundCollision
  (params (Player :type PC%20GM2%20Player%20Object%20Reference) (Location :type Vector))
  (bind _soundcue (Default|GetSoundCue (Variables|PlayerEvents|GetAudioAtlas) "NewEnumerator15" true))
  (Audio|PlaySoundatLocation _soundcue Location "0, 0, 0" 1.0 1.0 0.0 0 0 0 0))

(fn PlayerDeath
  (params (Player :type PC%20GM2%20Player%20Object%20Reference))
  (bind _soundcue (Default|GetSoundCue (Variables|PlayerEvents|GetAudioAtlas) "NewEnumerator31" true))
  (Audio|PlaySoundatLocation _soundcue (Transformation|GetActorLocation Player) "0, 0, 0" 1.0 1.0 0.0 0 0 0 0))

(fn StarPreSpawn
  (params (Star :type BP%20GM2%20Collectible%20Object%20Reference))
  (bind _soundcue (Default|GetSoundCue (Variables|PlayerEvents|GetAudioAtlas) "NewEnumerator20" true))
  (Audio|PlaySoundatLocation _soundcue (Transformation|GetActorLocation Star) "0, 0, 0" 1.0 1.0 0.0 0 0 0 0))

(fn StarSpawn
  (params (Star :type BP%20GM2%20Collectible%20Object%20Reference))
  (bind _soundcue (Default|GetSoundCue (Variables|PlayerEvents|GetAudioAtlas) "NewEnumerator21" true))
  (Audio|PlaySoundatLocation _soundcue (Transformation|GetActorLocation Star) "0, 0, 0" 1.0 1.0 0.0 0 0 0 0))

(fn StarCollected
  (params (Star :type BP%20GM2%20Collectible%20Object%20Reference) (Player :type PC%20GM2%20Player%20Object%20Reference))
  (bind _soundcue (Default|GetSoundCue (Variables|PlayerEvents|GetAudioAtlas) "NewEnumerator24" true))
  (Audio|PlaySoundatLocation _soundcue (Transformation|GetActorLocation Player) "0, 0, 0" 1.0 1.0 0.0 0 0 0 0))

(fn LargeStarPreSpawn
  (params (Star :type BP%20GM2%20Big%20Star%20Object%20Reference))
  (bind _soundcue (Default|GetSoundCue (Variables|PlayerEvents|GetAudioAtlas) "NewEnumerator22" true))
  (Audio|PlaySoundatLocation _soundcue (Transformation|GetActorLocation Star) "0, 0, 0" 1.0 1.0 0.0 0 0 0 0))

(fn LargeStarSpawn
  (params (Star :type BP%20GM2%20Big%20Star%20Object%20Reference))
  (bind _soundcue (Default|GetSoundCue (Variables|PlayerEvents|GetAudioAtlas) "NewEnumerator23" true))
  (Audio|PlaySoundatLocation _soundcue (Transformation|GetActorLocation Star) "0, 0, 0" 1.0 1.0 0.0 0 0 0 0))

(fn LargeStarCollected
  (params (Star :type BP%20GM2%20Big%20Star%20Object%20Reference))
  (bind _soundcue (Default|GetSoundCue (Variables|PlayerEvents|GetAudioAtlas) "NewEnumerator25" true))
  (Audio|PlaySoundatLocation _soundcue (Transformation|GetActorLocation Star) "0, 0, 0" 1.0 1.0 0.0 0 0 0 0))

(fn PlayerStarStolen
  (params (OldOwner :type PC%20GM2%20Player%20Object%20Reference) (NewOwner :type PC%20GM2%20Player%20Object%20Reference))
  (bind _soundcue (Default|GetSoundCue (Variables|PlayerEvents|GetAudioAtlas) "NewEnumerator26" true))
  (Audio|PlaySoundatLocation _soundcue (Transformation|GetActorLocation NewOwner) "0, 0, 0" 1.0 1.0 0.0 0 0 0 0))