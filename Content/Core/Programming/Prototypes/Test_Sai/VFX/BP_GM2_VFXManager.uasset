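; VFX manager for the GM2 game mode that spawns one-shot effects for player dash, death and star events.
; Half a second after BeginPlay, it caches the game mode's FXManager and the game instance's GM2 VFX atlas, then binds to the manager's events.
; Each handler fetches its system from the atlas by enum and spawns it at the actor's location, using Player1 for dual impacts and NewOwner for steals.
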(event Custom|Gather%20Variables
  (bind _asgm_gm2 (Utilities|Casting|CastToGM_GM2 (Game|GetGameMode)))
  (bind _output_get (Variables|Default|SetGameMode _asgm_gm2))
  (Variables|Default|SetFXManager (Variables|/Game/GameMode2/Programming/Gamemode/GM_GM2.GM_GM2_C|GetFXManager _output_get))
  (bind _asgi_core_game_instance (Utilities|Casting|CastToGI_CORE_GameInstance (Game|GetGameInstance)))
  (Variables|Default|SetVFXAtlas (Variables|/Game/Core/Programming/Prototypes/GameData/GI_CORE_GameInstance.GI_CORE_GameInstance_C|GetGM2VFXAtlas _asgi_core_game_instance)))

(event Custom|PlayerEventBinding
  (EventDispatchers|BindEventtoGM2PlayerDashEngaged (Variables|Default|GetFXManager) (delegate Custom|OnPlayerDashEngaged))
  (EventDispatchers|BindEventtoGM2PlayerDashCollision (Variables|Default|GetFXManager) (delegate Custom|OnPlayerDashCollision))
  (EventDispatchers|BindEventtoGM2PlayerDualDashCollision (Variables|Default|GetFXManager) (delegate Custom|OnPlayerDualDashCollision))
  (EventDispatchers|BindEventtoGM2PlayerDeath (Variables|Default|GetFXManager) (delegate Custom|OnPlayerDeath))
  (EventDispatchers|BindEventtoGM2PlayerStarSteal (Variables|Default|GetFXManager) (delegate Custom|OnPlayerStarSteal)))

(event Custom|OnPlayerStarSteal
  (params (OldOwner :type PC%20GM2%20Player%20Object%20Reference) (NewOwner :type PC%20GM2%20Player%20Object%20Reference))
  (PlayerEvents|PlayerStarSteal OldOwner NewOwner))

(event Custom|OnLargeStarPreSpawn
  (params (Star :type BP%20GM2%20Big%20Star%20Object%20Reference))
  (StarEvents|LargeStarPreSpawn Star))

(event Custom|OnLargeStarSpawn
  (params (Star :type BP%20GM2%20Big%20Star%20Object%20Reference))
  (StarEvents|LargeStarSpawn Star))

(event Custom|OnLargeStarCollected
  (params (Star :type BP%20GM2%20Big%20Star%20Object%20Reference))
  (StarEvents|LargeStarCollected Star))

(event Custom|OnPlayerDashEngaged
  (params (Player :type PC%20GM2%20Player%20Object%20Reference))
  (PlayerEvents|PlayerDashEngaged Player))

(event Custom|OnPlayerDashCollision
  (params (Player :type PC%20GM2%20Player%20Object%20Reference))
  (PlayerEvents|PlayerDashCollision Player))

(event Custom|OnPlayerDualDashCollision
  (params (Player1 :type PC%20GM2%20Player%20Object%20Reference) (Player2 :type PC%20GM2%20Player%20Object%20Reference))
  (PlayerEvents|PlayerDashDualImpact Player1 Player2))

(event Custom|OnPlayerDeath
  (params (Player :type PC%20GM2%20Player%20Object%20Reference))
  (PlayerEvents|PlayerDeath Player))

(event Custom|StarEventBinding
  (EventDispatchers|BindEventtoGM2StarCollected (Variables|Default|GetFXManager) (delegate Custom|OnStarCollected))
  (EventDispatchers|BindEventtoGM2StarSpawn (Variables|Default|GetFXManager) (delegate Custom|OnStarSpawn))
  (EventDispatchers|BindEventtoGM2StarPreSpawn (Variables|Default|GetFXManager) (delegate Custom|OnStarPreSpawn))
  (EventDispatchers|BindEventtoGM2LargeStarSpawn (Variables|Default|GetFXManager) (delegate Custom|OnLargeStarSpawn))
  (EventDispatchers|AssignGM2LargeStarPreSpawn (Variables|Default|GetFXManager) (delegate Custom|OnLargeStarPreSpawn))
  (EventDispatchers|BindEventtoGM2LargeStarCollected (Variables|Default|GetFXManager) (delegate Custom|OnLargeStarCollected)))

(event Custom|OnStarCollected
  (params (Star :type BP%20GM2%20Collectible%20Object%20Reference) (Player :type PC%20GM2%20Player%20Object%20Reference))
  (StarEvents|StarCollected Star Player))

(event Custom|OnStarSpawn
  (params (Star :type BP%20GM2%20Collectible%20Object%20Reference))
  (StarEvents|StarSpawn Star))

(event Custom|OnStarPreSpawn
  (params (Star :type BP%20GM2%20Collectible%20Object%20Reference))
  (StarEvents|StarPreSpawn Star))

(event EventBeginPlay
  (Utilities|FlowControl|Delay 0.5)
  (CallFunction|GatherVariables)
  (CallFunction|PlayerEventBinding)
  (CallFunction|StarEventBinding))

(fn ConstructionScript)

(fn PlayerDashEngaged
  (params (Player :type PC%20GM2%20Player%20Object%20Reference))
  (bind _vfxasset (Default|GetVFX (Variables|Default|GetVFXAtlas) "NewEnumerator3" false))
  (Niagara|SpawnSystematLocation _vfxasset (Transformation|GetActorLocation Player)))

(fn PlayerDashCollision
  (params (Player :type PC%20GM2%20Player%20Object%20Reference))
  (bind _vfxasset (Default|GetVFX (Variables|Default|GetVFXAtlas) "NewEnumerator4" false))
  (Niagara|SpawnSystematLocation _vfxasset (Transformation|GetActorLocation Player)))

(fn PlayerDashDualImpact
  (params (Player1 :type PC%20GM2%20Player%20Object%20Reference) (Player2 :type PC%20GM2%20Player%20Object%20Reference))
  (bind _vfxasset (Default|GetVFX (Variables|Default|GetVFXAtlas) "NewEnumerator14" false))
  (Niagara|SpawnSystematLocation _vfxasset (Transformation|GetActorLocation Player1)))

(fn PlayerDeath
  (params (Player :type PC%20GM2%20Player%20Object%20Reference))
  (bind _vfxasset (Default|GetVFX (Variables|Default|GetVFXAtlas) "NewEnumerator13" false))
  (Niagara|SpawnSystematLocation _vfxasset (Transformation|GetActorLocation Player)))

(fn PlayerStarSteal
  (params (OldOwner :type PC%20GM2%20Player%20Object%20Reference) (NewOwner :type PC%20GM2%20Player%20Object%20Reference))
  (bind _vfxasset (Default|GetVFX (Variables|Default|GetVFXAtlas) "NewEnumerator11" false))
  (Niagara|SpawnSystematLocation _vfxasset (Transformation|GetActorLocation NewOwner)))

(fn StarCollected
  (params (Star :type BP%20GM2%20Collectible%20Object%20Reference) (Player :type PC%20GM2%20Player%20Object%20Reference))
  (bind _vfxasset (Default|GetVFX (Variables|Default|GetVFXAtlas) "NewEnumerator7" false))
  (Niagara|SpawnSystematLocation _vfxasset (Transformation|GetActorLocation Star)))

(fn StarSpawn
  (params (Star :type BP%20GM2%20Collectible%20Object%20Reference))
  (bind _vfxasset (Default|GetVFX (Variables|Default|GetVFXAtlas) "NewEnumerator6" false))
  (Niagara|SpawnSystematLocation _vfxasset (Transformation|GetActorLocation Star)))

(fn StarPreSpawn
  (params (Star :type BP%20GM2%20Collectible%20Object%20Reference))
  (bind _vfxasset (Default|GetVFX (Variables|Default|GetVFXAtlas) "NewEnumerator5" false))
  (Niagara|SpawnSystematLocation _vfxasset (Transformation|GetActorLocation Star)))

(fn LargeStarCollected
  (params (Star :type BP%20GM2%20Big%20Star%20Object%20Reference))
  (bind _vfxasset (Default|GetVFX (Variables|Default|GetVFXAtlas) "NewEnumerator10" false))
  (Niagara|SpawnSystematLocation _vfxasset (Transformation|GetActorLocation Star)))

(fn LargeStarSpawn
  (params (Star :type BP%20GM2%20Big%20Star%20Object%20Reference))
  (bind _vfxasset (Default|GetVFX (Variables|Default|GetVFXAtlas) "NewEnumerator9" false))
  (Niagara|SpawnSystematLocation _vfxasset (Transformation|GetActorLocation Star)))

(fn LargeStarPreSpawn
  (params (Star :type BP%20GM2%20Big%20Star%20Object%20Reference))
  (bind _vfxasset (Default|GetVFX (Variables|Default|GetVFXAtlas) "NewEnumerator8" false))
  (Niagara|SpawnSystematLocation _vfxasset (Transformation|GetActorLocation Star)))