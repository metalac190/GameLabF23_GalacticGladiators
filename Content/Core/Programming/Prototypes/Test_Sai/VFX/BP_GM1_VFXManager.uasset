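; Prototype VFX manager for GM1 that spawns one-shot Niagara effects for player, bumper hazard and crown events.
; After a short BeginPlay delay it gets the FXManager from GM_GM1 and the GM1 VFX atlas from the game instance, then binds to the FXManager's events.
; Handlers look up effects in the atlas and spawn them at actor locations.
; Running players are tracked in an array, with a running effect spawned at each every Tick.
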(event Custom|PlayerEventBinding
  ;[1 0.6623 0.1292] All the Event Bindings
  (EventDispatchers|BindEventtoGM1PlayerRocketBurstStarted (Variables|References|GetFXManager) (delegate Custom|OnRocketBurstStarted))
  (EventDispatchers|BindEventtoGM1PlayerRocketBurstImpact (Variables|References|GetFXManager) (delegate Custom|OnRocketBurstImpact))
  (EventDispatchers|BindEventtoGM1PlayerRocketBurstRecharged (Variables|References|GetFXManager) (delegate Custom|OnRocketBurstRecharged))
  (EventDispatchers|BindEventtoGM1PlayerDeath (Variables|References|GetFXManager) (delegate Custom|OnPlayerDeath))
  (EventDispatchers|BindEventtoGM1PlayerSpawn (Variables|References|GetFXManager) (delegate Custom|OnPlayerSpawn))
  (EventDispatchers|BindEventtoGM1PlayerRunning (Variables|References|GetFXManager) (delegate Custom|OnPlayerRunning)))

(event Custom|HazardEventBinding
  ;[1 0.6623 0.1292] All the Event Bindings
  (EventDispatchers|BindEventtoGM1HazardBumpersCollision (Variables|References|GetFXManager) (delegate Custom|OnHazardBumpersCollision)))

(event Custom|OnHazardBumpersCollision
  (params (bumper :type BP%20Bumper%20Object%20Reference) (player :type BP%20Player%20GM1%20Object%20Reference))
  ;[1 0.6623 0.1292] All the Event Bindings
  (HazardFX|HazardBumpersCollision bumper player))

(event Custom|OnCrownPreSpawn
  (params (crown :type BP%20Crown%20Object%20Reference))
  ;[1 0.6623 0.1292] All the Event Bindings
  (CrownFX|CrownPreSpawn crown))

(event Custom|OnCrownSpawn
  (params (crown :type BP%20Crown%20Object%20Reference))
  ;[1 0.6623 0.1292] All the Event Bindings
  (CrownFX|CrownSpawn crown))

(event Custom|OnCrownPickup
  (params (crown :type BP%20Crown%20Object%20Reference) (newOwner :type BP%20Player%20GM1%20Object%20Reference))
  ;[1 0.6623 0.1292] All the Event Bindings
  (CrownFX|CrownPickup crown newOwner))

(event Custom|OnCrownStolen
  (params (crown :type BP%20Crown%20Object%20Reference) (newOwner :type BP%20Player%20GM1%20Object%20Reference) (oldOwner :type BP%20Player%20GM1%20Object%20Reference))
  ;[1 0.6623 0.1292] All the Event Bindings
  (CrownFX|CrownStolen crown newOwner oldOwner))

(event Custom|CrownEventBinding
  ;[1 0.6623 0.1292] All the Event Bindings
  (EventDispatchers|BindEventtoGM1CrownPreSpawn (Variables|References|GetFXManager) (delegate Custom|OnCrownPreSpawn))
  (EventDispatchers|BindEventtoGM1CrownSpawn (Variables|References|GetFXManager) (delegate Custom|OnCrownSpawn))
  (EventDispatchers|BindEventtoGM1CrownPickedUp (Variables|References|GetFXManager) (delegate Custom|OnCrownPickup))
  (EventDispatchers|BindEventtoGM1CrownStolen (Variables|References|GetFXManager) (delegate Custom|OnCrownStolen)))

(event Custom|OnRocketBurstStarted
  (params (player :type BP%20Player%20GM1%20Object%20Reference))
  ;[1 0.6623 0.1292] All the Event Bindings
  (PlayerFX|RocketBurstStarted player))

(event Custom|OnRocketBurstImpact
  (params (player :type BP%20Player%20GM1%20Object%20Reference))
  ;[1 0.6623 0.1292] All the Event Bindings
  (PlayerFX|RocketBurstImpact player))

(event Custom|OnRocketBurstRecharged
  (params (player :type BP%20Player%20GM1%20Object%20Reference))
  ;[1 0.6623 0.1292] All the Event Bindings
  (PlayerFX|RocketBurstRecharged player))

(event Custom|OnPlayerDeath
  (params (player :type BP%20Player%20GM1%20Object%20Reference))
  ;[1 0.6623 0.1292] All the Event Bindings
  (PlayerFX|PlayerDeath player))

(event Custom|OnPlayerSpawn
  (params (player :type BP%20Player%20GM1%20Object%20Reference))
  ;[1 0.6623 0.1292] All the Event Bindings
  (PlayerFX|PlayerSpawn player))

(event Custom|OnPlayerRunning
  (params (state :type Boolean) (player :type BP%20Player%20GM1%20Object%20Reference))
  ;[1 0.6623 0.1292] All the Event Bindings
  (PlayerFX|PlayerRunning state player))

(event EventBeginPlay
  (Utilities|FlowControl|Delay 0.5)
  ;[0.2789 1 0.1912] Get Variables
  (bind _asgm_gm1 (Utilities|Casting|CastToGM_GM1 (Game|GetGameMode)))
  (bind _output_get (Variables|References|SetGameMode _asgm_gm1))
  (Variables|References|SetFXManager (Variables|/Game/Systems/Blueprints/GM1/Systems/GM_GM1.GM_GM1_C|GetFXManager _output_get))
  (bind _asgi_core_game_instance (Utilities|Casting|CastToGI_CORE_GameInstance (Game|GetGameInstance)))
  (Variables|References|SetVFX%20Atlas (Variables|/Game/Core/Programming/Prototypes/GameData/GI_CORE_GameInstance.GI_CORE_GameInstance_C|GetGM1VFXAtlas _asgi_core_game_instance))
  ;[0.2789 1 0.1912] Binding to events
  (CallFunction|PlayerEventBinding)
  (CallFunction|HazardEventBinding)
  (CallFunction|CrownEventBinding))

(event EventTick
  (params (DeltaSeconds :type Float%20%28single-precision%29))
  ;[0.2789 1 0.1912] Spawn PlayerRunning NS at the location of Running Players
  (if (Utilities|Array|IsNotEmpty (Variables|Default|GetRunningPlayers))
    (for _array_element (Variables|Default|GetRunningPlayers)
      (bind _vfxasset (Default|GetVFX (Variables|References|GetVFX%20Atlas) "NewEnumerator14" false))
      (Niagara|SpawnSystematLocation _vfxasset (Transformation|GetActorLocation _array_element)))))

(fn ConstructionScript)

(fn RocketBurstStarted
  (params (Player :type BP%20Player%20GM1%20Object%20Reference))
  (bind _vfxasset (Default|GetVFX (Variables|References|GetVFX%20Atlas) "NewEnumerator0" true))
  (Niagara|SpawnSystematLocation _vfxasset (Transformation|GetActorLocation Player)))

(fn RocketBurstImpact
  (params (Player :type BP%20Player%20GM1%20Object%20Reference))
  (bind _vfxasset (Default|GetVFX (Variables|References|GetVFX%20Atlas) "NewEnumerator2" true))
  (Niagara|SpawnSystematLocation _vfxasset (Transformation|GetActorLocation Player)))

(fn RocketBurstRecharged
  (params (Player :type BP%20Player%20GM1%20Object%20Reference))
  (bind _vfxasset (Default|GetVFX (Variables|References|GetVFX%20Atlas) "NewEnumerator3" true))
  (Niagara|SpawnSystematLocation _vfxasset (Transformation|GetActorLocation Player)))

(fn PlayerDeath
  (params (Player :type BP%20Player%20GM1%20Object%20Reference))
  (bind _vfxasset (Default|GetVFX (Variables|References|GetVFX%20Atlas) "NewEnumerator5" true))
  (Niagara|SpawnSystematLocation _vfxasset (Transformation|GetActorLocation Player)))

(fn PlayerSpawn
  (params (Player :type BP%20Player%20GM1%20Object%20Reference))
  (bind _vfxasset (Default|GetVFX (Variables|References|GetVFX%20Atlas) "NewEnumerator4" true))
  (Niagara|SpawnSystematLocation _vfxasset (Transformation|GetActorLocation Player)))

(fn PlayerRunning
  (params (State :type Boolean) (Player :type BP%20Player%20GM1%20Object%20Reference))
  (LocalVariables|SetPlayerGM1 Player)
  (if State
    (Utilities|Array|AddUnique (Variables|Default|GetRunningPlayers) (LocalVariables|GetPlayerGM1))
    (else
      (Utilities|Array|RemoveItem (Variables|Default|GetRunningPlayers) (LocalVariables|GetPlayerGM1)))))

(fn HazardBumpersCollision
  (params (Bumper :type BP%20Bumper%20Object%20Reference) (Player :type BP%20Player%20GM1%20Object%20Reference))
  (bind _vfxasset (Default|GetVFX (Variables|References|GetVFX%20Atlas) "NewEnumerator9" true))
  (Niagara|SpawnSystematLocation _vfxasset (Transformation|GetActorLocation Bumper)))

(fn CrownPreSpawn
  (params (Crown :type BP%20Crown%20Object%20Reference))
  (bind _vfxasset (Default|GetVFX (Variables|References|GetVFX%20Atlas) "NewEnumerator11" true))
  (Niagara|SpawnSystematLocation _vfxasset (Transformation|GetActorLocation Crown)))

(fn CrownSpawn
  (params (Crown :type BP%20Crown%20Object%20Reference))
  (bind _vfxasset (Default|GetVFX (Variables|References|GetVFX%20Atlas) "NewEnumerator10" true))
  (Niagara|SpawnSystematLocation _vfxasset (Transformation|GetActorLocation Crown)))

(fn CrownPickup
  (params (Crown :type BP%20Crown%20Object%20Reference) (NewOwner :type BP%20Player%20GM1%20Object%20Reference))
  (bind _vfxasset (Default|GetVFX (Variables|References|GetVFX%20Atlas) "NewEnumerator13" true))
  (Niagara|SpawnSystematLocation _vfxasset (Transformation|GetActorLocation NewOwner)))

(fn CrownStolen
  (params (Crown :type BP%20Crown%20Object%20Reference) (NewOwner :type BP%20Player%20GM1%20Object%20Reference) (OldOwner :type BP%20Player%20GM1%20Object%20Reference))
  (bind _vfxasset (Default|GetVFX (Variables|References|GetVFX%20Atlas) "NewEnumerator12" true))
  (Niagara|SpawnSystematLocation _vfxasset (Transformation|GetActorLocation NewOwner)))