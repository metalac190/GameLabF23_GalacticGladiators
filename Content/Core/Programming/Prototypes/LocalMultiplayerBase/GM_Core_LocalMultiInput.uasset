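; Prototype local multiplayer game mode that gives each BP_Core_LocalMultiInput in the level its own local player for lobby input.
; On BeginPlay it gathers those actors and calls CreatePlayer per array index, using that index as controller ID and PlayerID.
; Each player gets the IMC_LobbyInput Enhanced Input context and possesses the matching actor, with index 0 using the primary controller.
; It also collects the player controllers and prints each index for debugging.
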(event EventBeginPlay
  (Variables|Default|SetCurrentGameInstance (Game|GetGameInstance))
  (bind _outactors (Actor|GetAllActorsOfClass "/Game/Core/Programming/Prototypes/LocalMultiplayerBase/BP_Core_LocalMultiInput.BP_Core_LocalMultiInput_C"))
  (bind _output_get (Variables|Default|SetLocalInputs _outactors))
  (for (_ _array_index) _output_get
    (bind _output_get_2 (Variables|Default|SetArrayIndex _array_index))
    (bind _returnvalue (Class|GameplayStatics|CreatePlayer _output_get_2))
    (if (> (Variables|Default|GetArrayIndex) 0)
      (Input|AddMappingContext (PlayerController|LocalPlayerSubsystems|GetEnhancedInputLocalPlayerSubsystem _returnvalue) "/Game/Freelance/Programming/Input/IMC_LobbyInput.IMC_LobbyInput" 0 "(bIgnoreAllPressedKeysUntilRelease=True,bForceImmediately=False)")
      (Pawn|Possess (Class|GameplayStatics|GetPlayerControllerfromID (Variables|Default|GetArrayIndex)) (Utilities|Array|Get(acopy) (Variables|Default|GetLocalInputs) (Variables|Default|GetArrayIndex)))
      (Utilities|Array|AddUnique (Variables|Default|GetPlayerControllers) 0)
      (Variables|/Game/Core/Programming/Prototypes/LocalMultiplayerBase/BP_Core_LocalMultiInput.BP_Core_LocalMultiInput_C|SetPlayerID (Utilities|Array|Get(acopy) (Variables|Default|GetLocalInputs) (Variables|Default|GetArrayIndex)) (Variables|Default|GetArrayIndex))
      (Development|PrintText (Utilities|Text|FormatText "Array Index: {0}" (Variables|Default|GetArrayIndex)))
      (else
        (Input|AddMappingContext (PlayerController|LocalPlayerSubsystems|GetEnhancedInputLocalPlayerSubsystem (Game|GetPlayerController 0)) "/Game/Freelance/Programming/Input/IMC_LobbyInput.IMC_LobbyInput" 0 "(bIgnoreAllPressedKeysUntilRelease=True,bForceImmediately=False)")
        (Pawn|Possess (Class|GameplayStatics|GetPlayerControllerfromID) (Utilities|Array|Get(acopy) (Variables|Default|GetLocalInputs) (Variables|Default|GetArrayIndex)))
        (Utilities|Array|AddUnique (Variables|Default|GetPlayerControllers) 0)
        (Variables|/Game/Core/Programming/Prototypes/LocalMultiplayerBase/BP_Core_LocalMultiInput.BP_Core_LocalMultiInput_C|SetPlayerID (Utilities|Array|Get(acopy) (Variables|Default|GetLocalInputs) (Variables|Default|GetArrayIndex)) (Variables|Default|GetArrayIndex))
        (Development|PrintText (Utilities|Text|FormatText "Array Index: {0}" (Variables|Default|GetArrayIndex)))))))

(fn ConstructionScript)