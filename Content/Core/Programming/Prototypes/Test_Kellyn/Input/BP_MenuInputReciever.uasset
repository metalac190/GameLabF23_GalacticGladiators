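; Prototype menu input receiver Blueprint that relays Enhanced Input menu actions to a referenced widget.
; SetWidgetReference stores the target widget.
; Select, back and directional Started events call the matching On handler on that widget after a validity check.
; Only Select prints a warning when no widget is set; the other actions do nothing in that case.
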(event Input|EnhancedActionEvents|EnhancedInputActionIA_Core_MenuBack
  (params (ActionValue :type Boolean) (ElapsedSeconds :type Float%20%28double-precision%29) (TriggeredSeconds :type Float%20%28double-precision%29) (InputAction :type Input%20Action%20Object%20Reference :default "/Game/Core/Programming/Prototypes/Test_Kellyn/Input/IA_Core_MenuBack.IA_Core_MenuBack"))
  (bind _widget (Variables|Default|GetWidget))
  (:Started
    (Utilities|IsValid _widget
      (:Is%20Valid
        (Default|OnBack _widget)))))

(event Input|EnhancedActionEvents|EnhancedInputActionIA_Core_MenuSelect
  (params (ActionValue :type Boolean) (ElapsedSeconds :type Float%20%28double-precision%29) (TriggeredSeconds :type Float%20%28double-precision%29) (InputAction :type Input%20Action%20Object%20Reference :default "/Game/Core/Programming/Prototypes/Test_Kellyn/Input/IA_Core_MenuSelect.IA_Core_MenuSelect"))
  (bind _widget (Variables|Default|GetWidget))
  (:Started
    (Utilities|IsValid _widget
      (:Is%20Valid
        (Default|OnSelect _widget))
      (:Is%20Not%20Valid
        (Development|PrintString "No Widget")))))

(event Input|EnhancedActionEvents|EnhancedInputActionIA_Core_MenuDown
  (params (ActionValue :type Boolean) (ElapsedSeconds :type Float%20%28double-precision%29) (TriggeredSeconds :type Float%20%28double-precision%29) (InputAction :type Input%20Action%20Object%20Reference :default "/Game/Core/Programming/Prototypes/Test_Kellyn/Input/IA_Core_MenuDown.IA_Core_MenuDown"))
  (bind _widget (Variables|Default|GetWidget))
  (:Started
    (Utilities|IsValid _widget
      (:Is%20Valid
        (Default|OnDown _widget)))))

(event Input|EnhancedActionEvents|EnhancedInputActionIA_Core_MenuUp
  (params (ActionValue :type Boolean) (ElapsedSeconds :type Float%20%28double-precision%29) (TriggeredSeconds :type Float%20%28double-precision%29) (InputAction :type Input%20Action%20Object%20Reference :default "/Game/Core/Programming/Prototypes/Test_Kellyn/Input/IA_Core_MenuUp.IA_Core_MenuUp"))
  (bind _widget (Variables|Default|GetWidget))
  (:Started
    (Utilities|IsValid _widget
      (:Is%20Valid
        (Default|OnUp _widget)))))

(event Input|EnhancedActionEvents|EnhancedInputActionIA_Core_MenuLeft
  (params (ActionValue :type Boolean) (ElapsedSeconds :type Float%20%28double-precision%29) (TriggeredSeconds :type Float%20%28double-precision%29) (InputAction :type Input%20Action%20Object%20Reference :default "/Game/Core/Programming/Prototypes/Test_Kellyn/Input/IA_Core_MenuLeft.IA_Core_MenuLeft"))
  (bind _widget (Variables|Default|GetWidget))
  (:Started
    (Utilities|IsValid _widget
      (:Is%20Valid
        (Default|OnLeft _widget)))))

(event Input|EnhancedActionEvents|EnhancedInputActionIA_Core_MenuRight
  (params (ActionValue :type Boolean) (ElapsedSeconds :type Float%20%28double-precision%29) (TriggeredSeconds :type Float%20%28double-precision%29) (InputAction :type Input%20Action%20Object%20Reference :default "/Game/Core/Programming/Prototypes/Test_Kellyn/Input/IA_Core_MenuRight.IA_Core_MenuRight"))
  (bind _widget (Variables|Default|GetWidget))
  (:Started
    (Utilities|IsValid _widget
      (:Is%20Valid
        (Default|OnRight _widget)))))

(event EventBeginPlay)

(event Collision|EventActorBeginOverlap
  (params (OtherActor :type Actor%20Object%20Reference)))

(event EventTick
  (params (DeltaSeconds :type Float%20%28single-precision%29)))

(fn ConstructionScript)

(fn SetWidgetReference
  (params (Widget :type WBP%20GG%20Widge%20Base%20Object%20Reference))
  (Variables|Default|SetWidget Widget))