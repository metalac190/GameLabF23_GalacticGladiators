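; Prototype menu game mode that sets up the main menu when play begins.
; It clears player data on the core game instance, sets the default menu input mapping context and spawns input pawns.
; It then creates the main menu widget, adds it to the viewport, and passes a reference to each local menu input receiver so they can drive the UI.
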(event EventBeginPlay
  (bind _asgi_core_game_instance (Utilities|Casting|CastToGI_CORE_GameInstance (Game|GetGameInstance)))
  (Default|ClearPlayerData _asgi_core_game_instance)
  (Variables|Default|SetDefaultIMC "/Game/Core/Programming/Prototypes/Test_Kellyn/Input/IMC_Core_MenuDefault.IMC_Core_MenuDefault")
  (CallFunction|SpawnInputPawns)
  (bind _returnvalue (UserInterface|CreateWidget "/Game/Core/Programming/Prototypes/Test_Kellyn/Widgets/WBP_MainMenu.WBP_MainMenu_C"))
  (bind _output_get (Variables|Default|SetMainMenuWBP _returnvalue))
  (UserInterface|Viewport|AddtoViewport _output_get 0)
  ;[1 1 1] Gives Each Input Reciever a Refernce to Main Menu Widget
  (for _array_element (Variables|Default|GetLocalInputs)
    (bind _asbp_menu_input_reciever (Utilities|Casting|CastToBP_MenuInputReciever _array_element))
    (Default|SetWidgetReference _asbp_menu_input_reciever (Variables|Default|GetMainMenuWBP))))

(event EventTick
  (params (DeltaSeconds :type Float%20%28single-precision%29)))

(fn ConstructionScript)