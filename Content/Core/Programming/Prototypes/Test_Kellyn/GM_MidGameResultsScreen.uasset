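; Game mode prototype for the mid-game results screen, which displays a menu widget and hooks local inputs up to it.
; On BeginPlay it sets the core menu input mapping context, spawns input pawns, then creates the mid-game menu widget and adds it to the viewport.
; It then passes the widget to each local menu input receiver, stopping at any input that fails the cast.
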(event EventBeginPlay
  (Variables|Default|SetDefaultIMC "/Game/Core/Programming/Prototypes/Test_Kellyn/Input/IMC_Core_MenuDefault.IMC_Core_MenuDefault")
  (CallFunction|SpawnInputPawns)
  (bind _returnvalue (UserInterface|CreateWidget "/Game/Core/Programming/Prototypes/Test_Kellyn/Widgets/WBP_MidGameMenu.WBP_MidGameMenu_C"))
  (bind _output_get (Variables|Default|SetCurrentWidget _returnvalue))
  (UserInterface|Viewport|AddtoViewport _output_get 0)
  (for _array_element (Variables|Default|GetLocalInputs)
    (bind _asbp_menu_input_reciever (Utilities|Casting|CastToBP_MenuInputReciever _array_element))
    (Default|SetWidgetReference _asbp_menu_input_reciever (Variables|Default|GetCurrentWidget))))

(event EventTick
  (params (DeltaSeconds :type Float%20%28single-precision%29)))

(fn ConstructionScript
  (|CallParentFunction))