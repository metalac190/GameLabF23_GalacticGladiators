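; GM1 stage hazard spawner that drops meteors onto telegraphed AOE zones once the game mode signals hazard start.
; A data-driven timer loop spawns a random warning zone, waits, then launches a meteor from above with impact timed by distance over speed.
; Line, ring and burst functions compute points within the arena radius for SpawnPattern, which telegraphs all zones before dropping meteors together.
; The construction script previews spawn range with debug circles and a decal.
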(event Custom|Spawn%20AOE%20Zone%20and%20Meteor
  (bind (_zone _size) (CallFunction|SpawnAOEZone :randomSpawn true))
  (Utilities|FlowControl|Delay (Variables|/Game/Systems/Blueprints/GM1/Hazards/Data/PDA_MeteorSpawner.PDA_MeteorSpawner_C|GetHeads-up%20Time (Variables|Default|GetData)))
  (CallFunction|SpawnMeteor _zone (Utilities|RandomfromRange (Variables|/Game/Systems/Blueprints/GM1/Hazards/Data/PDA_MeteorSpawner.PDA_MeteorSpawner_C|GetMeteor%20Speed (Variables|Default|GetData))) _size)
  (if (Variables|Default|GetbContinueSpawn)
    (Utilities|Time|SetTimerbyEvent (delegate Custom|Spawn%20AOE%20Zone%20and%20Meteor) (Utilities|RandomfromRange (Variables|/Game/Systems/Blueprints/GM1/Hazards/Data/PDA_MeteorSpawner.PDA_MeteorSpawner_C|GetTarget%20Timer (Variables|Default|GetData))))))

(event Custom|Start%20Spawn
  (Utilities|FlowControl|Delay (Variables|/Game/Systems/Blueprints/GM1/Hazards/Data/PDA_MeteorSpawner.PDA_MeteorSpawner_C|GetInitial%20Delay (Variables|Default|GetData)))
  (if (Variables|/Game/Systems/Blueprints/GM1/Hazards/Data/PDA_MeteorSpawner.PDA_MeteorSpawner_C|GetAuto%20Start (Variables|Default|GetData))
    (CallFunction|SpawnAOEZoneandMeteor)))

(event Custom|Spawn%20Pattern
  (params (patternPoints :type Array%20of%20Vector%202D%20Structures) (meteorSize :type Float%20%28double-precision%29) (timer :type Float%20%28double-precision%29) (speed :type Float%20%28double-precision%29))
  (Utilities|Array|Clear (Variables|Default|GetpatternZones))
  (for _array_element patternPoints
    (bind _zone (CallFunction|SpawnAOEZone false _array_element meteorSize))
    (Utilities|Array|AddUnique (Variables|Default|GetpatternZones) _zone))
  (Utilities|FlowControl|Delay timer)
  (for _array_element_2 (Variables|Default|GetpatternZones)
    (CallFunction|SpawnMeteor _array_element_2 speed meteorSize)))

(event EventBeginPlay
  (bind _asgm_gm1 (Utilities|Casting|CastToGM_GM1 (Game|GetGameMode)))
  (EventDispatchers|BindEventtoOnStageHazardStart _asgm_gm1 (delegate Custom|Start%20Spawn)))

(fn ConstructionScript
  (bind _returnvalue (Transformation|GetActorLocation))
  (bind _visual__editor_only_ (Variables|Default|GetVisual%20%28EDITOR%20ONLY%29))
  (bind _data (Variables|Default|GetData))
  (bind _data_2 (Variables|Default|GetData))
  (bind _aoe_range (Variables|/Game/Systems/Blueprints/GM1/Hazards/Data/PDA_MeteorSpawner.PDA_MeteorSpawner_C|GetAOE%20Range _data_2))
  (bind _debug_color (Variables|/Game/Systems/Blueprints/GM1/Hazards/Data/PDA_MeteorSpawner.PDA_MeteorSpawner_C|GetDebug%20Color _data))
  (bind (_lowerbound _upperbound) (Utilities|Struct|BreakFloatRange _aoe_range))
  (Transformation|SetWorldScale3D _visual__editor_only_ (Math|Conversions|ToVector(Float) (.Value (Utilities|Struct|BreakFloatRangeBound (.LowerBound (Utilities|Struct|BreakFloatRange (Variables|/Game/Systems/Blueprints/GM1/Hazards/Data/PDA_MeteorSpawner.PDA_MeteorSpawner_C|GetMeteor%20Size (Variables|Default|GetData))))))))
  (Rendering|Components|Decal|SetDecalColor _visual__editor_only_ (Variables|/Game/Systems/Blueprints/GM1/Hazards/Data/PDA_MeteorSpawner.PDA_MeteorSpawner_C|GetAOE%20Color _data_2))
  (Rendering|Debug|DrawDebugCircle _returnvalue (.Value (Utilities|Struct|BreakFloatRangeBound _lowerbound)) 32 _debug_color 1.0 5.0 "0.000000,1.000000,0.000000" "1.000000,0.000000,0.000000")
  (Rendering|Debug|DrawDebugCircle _returnvalue (.Value (Utilities|Struct|BreakFloatRangeBound _upperbound)) 32 _debug_color 1.0 5.0 "0.000000,1.000000,0.000000" "1.000000,0.000000,0.000000"))

(fn SpawnAOEZone
  (params (randomSpawn :type Boolean) (setPosition :type Vector%202D%20Structure) (setSize :type Float%20%28double-precision%29))
  (bind _returnvalue (Game|SpawnActorfromClass "/Game/Systems/Blueprints/GM1/BP_GM1_AOEZone.BP_GM1_AOEZone_C" (Math|Transform|SelectTransform (Math|Transform|MakeTransform (+ (Transformation|GetActorLocation) (* (Utilities|RandomfromRange (Variables|/Game/Systems/Blueprints/GM1/Hazards/Data/PDA_MeteorSpawner.PDA_MeteorSpawner_C|GetAOE%20Range (Variables|Default|GetData))) (Math|Vector|Normalize (Math|Vector|MakeVector (Math|Random|RandomFloatinRange -1.0 1.0) (Math|Random|RandomFloatinRange -1.0 1.0) 0.0)))) "0, 0, 0" (Math|Conversions|ToVector(Float) (Utilities|RandomfromRange (Variables|/Game/Systems/Blueprints/GM1/Hazards/Data/PDA_MeteorSpawner.PDA_MeteorSpawner_C|GetMeteor%20Size (Variables|Default|GetData))))) (Math|Transform|MakeTransform (+ (Transformation|GetActorLocation) setPosition) "0, 0, 0" (Math|Conversions|ToVector(Float) setSize)) randomSpawn) "AlwaysSpawn" "MultiplyWithRoot" 0 0))
  (Rendering|Components|Decal|SetDecalColor (Variables|/Game/Systems/Blueprints/GM1/BP_GM1_AOEZone.BP_GM1_AOEZone_C|GetAOE%20Zone%20Decal _returnvalue) (Variables|/Game/Systems/Blueprints/GM1/Hazards/Data/PDA_MeteorSpawner.PDA_MeteorSpawner_C|GetAOE%20Color (Variables|Default|GetData)))
  (return _returnvalue (Variables|/Game/Systems/Blueprints/GM1/BP_GM1_AOEZone.BP_GM1_AOEZone_C|GettargetSize _returnvalue)))

(fn SpawnMeteor
  (params (AOE%20Zone :type BP%20GM1%20AOE%20Zone%20Object%20Reference) (Speed :type Float%20%28double-precision%29) (Size :type Float%20%28double-precision%29))
  (bind _returnvalue (Math|Conversions|ToVector(Float) Size))
  (bind _returnvalue_2 (Transformation|GetActorLocation AOE%20Zone))
  (bind _returnvalue_3 (Transformation|GetActorLocation AOE%20Zone))
  (bind _returnvalue_4 (+ _returnvalue_2 "0.000000,0.000000,2000.000000"))
  (bind _returnvalue_5 (Math|Transform|MakeTransform _returnvalue_4 "0, 0, 0" _returnvalue))
  (bind _returnvalue_6 (Class|KismetAnimationLibrary|Lookat _returnvalue_5 _returnvalue_2 "1.000000,0.000000,0.000000" false "0, 0, 0" 0.0))
  (bind _returnvalue_7 (Game|SpawnActorfromClass (Variables|/Game/Systems/Blueprints/GM1/Hazards/Data/PDA_MeteorSpawner.PDA_MeteorSpawner_C|GetMeteor%20Type (Variables|Default|GetData)) _returnvalue_6 "AlwaysSpawn" "MultiplyWithRoot" 0 0))
  (Variables|/Game/Systems/Blueprints/GM1/BP_GM1_AOEZone.BP_GM1_AOEZone_C|SetwatchingHazard AOE%20Zone _returnvalue_7)
  (Default|SetHazardSettings _returnvalue_7 Speed Size (Utilities|GetMeteorForcefromSize Size) (Variables|/Game/Systems/Blueprints/GM1/Hazards/Data/PDA_MeteorSpawner.PDA_MeteorSpawner_C|GetHorizontal%20Impulse%20Only (Variables|Default|GetData)))
  (Physics|AddImpulse (Variables|/Game/Systems/Blueprints/GM1/BP_GM1_Meteor.BP_GM1_Meteor_C|GetSphereCol _returnvalue_7) (* "0.000000,0.000000,-1.000000" Speed) "None" true)
  (Default|DelayImpact _returnvalue_7 _returnvalue_3 (/ (Math|Vector|Distance(Vector) (.Location (Math|Transform|BreakTransform _returnvalue_6)) _returnvalue_3) Speed) "/Game/Audio/SFX/GM1/Waves/sfx_env_Hazard_Impact_2.sfx_env_Hazard_Impact_2")
  (return _returnvalue_7))

(fn CalculateLine
  (params (offset :type Vector%202D%20Structure) (rotation :type Float%20%28double-precision%29) (width :type Float%20%28double-precision%29) (spacing :type Float%20%28double-precision%29))
  (bind _returnvalue (Math|Trig|Sin(Degrees) rotation))
  (bind _returnvalue_2 (Math|Trig|Cos(Degrees) rotation))
  (bind _returnvalue_3 (* width 5e+01 spacing))
  (bind _returnvalue_4 (Math|Vector2D|MakeVector2D _returnvalue_2 _returnvalue))
  (bind _returnvalue_5 (* _returnvalue_4 _returnvalue_3))
  (bind _returnvalue_6 (Actor|GetActorOfClass "/Game/Systems/Blueprints/GM1/Hazards/BP_Arena.BP_Arena_C"))
  (bind _output_get (LocalVariables|Setarena _returnvalue_6))
  (bind _x (Default|GetRadiusinUnits _output_get))
  (LocalVariables|SetarenaRadius _x)
  (LocalVariables|Setcurrent offset)
  (while (< (Math|Vector2D|Vector2DLength (LocalVariables|Getcurrent)) (- (LocalVariables|GetarenaRadius) (* width 5e+01 spacing)))
    (LocalVariables|Setcurrent (+ (LocalVariables|Getcurrent) _returnvalue_5)))
  (while (< (Math|Vector2D|Vector2DLength (LocalVariables|Getcurrent)) (LocalVariables|GetarenaRadius))
    (Utilities|Array|AddUnique (LocalVariables|GetlinePoints) (LocalVariables|Getcurrent))
    (LocalVariables|Setcurrent (- (LocalVariables|Getcurrent) _returnvalue_5)))
  (return (LocalVariables|GetlinePoints)))

(fn CalculateRing
  (params (center :type Vector%202D%20Structure) (radius :type Float%20%28double-precision%29) (numPoints :type Integer))
  (bind _returnvalue (Actor|GetActorOfClass "/Game/Systems/Blueprints/GM1/Hazards/BP_Arena.BP_Arena_C"))
  (bind _output_get (LocalVariables|Setarena _returnvalue))
  (bind _x (Default|GetRadiusinUnits _output_get))
  (LocalVariables|SetarenaRadius _x)
  (for _index (range 0 (- numPoints 1))
    (bind _output_get_2 (LocalVariables|Setcurrent (+ center (* (Math|Vector2D|MakeVector2D (Math|Trig|Cos(Degrees) (* _index (/ 3.6e+02 (Math|Conversions|ToFloat(Integer) numPoints)))) (Math|Trig|Sin(Degrees) (* _index (/ 3.6e+02 (Math|Conversions|ToFloat(Integer) numPoints))))) radius))))
    (if (< (Math|Vector2D|Vector2DLength _output_get_2) (LocalVariables|GetarenaRadius))
      (Utilities|Array|AddUnique (LocalVariables|GetringPoints) (LocalVariables|Getcurrent))))
  (return (LocalVariables|GetringPoints)))

(fn CalculateBurst
  (params (center :type Vector%202D%20Structure) (radius :type Float%20%28double-precision%29) (numPoints :type Integer))
  (bind _returnvalue (Actor|GetActorOfClass "/Game/Systems/Blueprints/GM1/Hazards/BP_Arena.BP_Arena_C"))
  (bind _output_get (LocalVariables|Setarena _returnvalue))
  (bind _x (Default|GetRadiusinUnits _output_get))
  (LocalVariables|SetarenaRadius _x)
  (for _index (range 0 (- numPoints 1))
    (bind _output_get_2 (LocalVariables|Setcurrent (+ center (* (Math|Vector2D|MakeVector2D (Math|Trig|Cos(Degrees) (* _index (/ 3.6e+02 (Math|Conversions|ToFloat(Integer) numPoints)))) (Math|Trig|Sin(Degrees) (* _index (/ 3.6e+02 (Math|Conversions|ToFloat(Integer) numPoints))))) (Math|Random|RandomFloatinRange 0.0 radius)))))
    (if (< (Math|Vector2D|Vector2DLength _output_get_2) (LocalVariables|GetarenaRadius))
      (Utilities|Array|AddUnique (LocalVariables|GetburstPoints) (LocalVariables|Getcurrent))))
  (return (LocalVariables|GetburstPoints)))

(fn SpawnMeteorLine
  (params (position :type Vector%202D%20Structure) (rotation :type Float%20%28double-precision%29) (size :type Float%20%28double-precision%29) (spacing :type Float%20%28double-precision%29) (timer :type Float%20%28double-precision%29) (speed :type Float%20%28double-precision%29))
  (bind _points (CallFunction|CalculateLine position rotation size spacing))
  (CallFunction|SpawnPattern _points size timer speed))

(fn SpawnMeteorRing
  (params (position :type Vector%202D%20Structure) (radius :type Float%20%28double-precision%29) (points :type Integer) (width :type Float%20%28double-precision%29) (timer :type Float%20%28double-precision%29) (speed :type Float%20%28double-precision%29))
  (bind _points (CallFunction|CalculateRing position radius points))
  (CallFunction|SpawnPattern _points width timer speed))

(fn SpawnMeteorBurst
  (params (position :type Vector%202D%20Structure) (radius :type Float%20%28double-precision%29) (count :type Integer) (meteorSize :type Float%20%28double-precision%29) (timer :type Float%20%28double-precision%29) (speed :type Float%20%28double-precision%29))
  (bind _points (CallFunction|CalculateBurst position radius count))
  (CallFunction|SpawnPattern _points meteorSize timer speed))