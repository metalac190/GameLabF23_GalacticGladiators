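; Player block ability component for GM1 that toggles the player's blocking state, fires block callbacks and plays ability effects.
; TryAbilityBlock starts a block if no cooldown timer exists, and that timer's expiry ends the block, so Cooldown also caps its duration.
; Tick shows the player's sphere while blocking and ramps HeldProgress up, decaying it otherwise; EndBlock resets it.
; The looping UpdateBlock timer is disconnected and its function is empty.
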(event Custom|TryAbilityBlock
  (if (CallFunction|CheckCanBlock)
    (CallFunction|StartBlock)
    (bind _returnvalue (Utilities|Time|SetTimerbyEvent (delegate Custom|CooldownTimerExpired) (Variables|Default|GetCooldown)))
    (Variables|Default|SetCooldownTimerHandle _returnvalue)))

(event Custom|CooldownTimerExpired
  (bind _data (Variables|Default|GetData))
  (CallFunction|EndBlock)
  (CallFunction|PlayAbilityEffects (Variables|/Game/Systems/Blueprints/GM1/Player/Systems/Data/PDA_Block.PDA_Block_C|GetSFX _data) (Variables|/Game/Systems/Blueprints/GM1/Player/Systems/Data/PDA_Block.PDA_Block_C|GetVFX _data)))

(event EventTick
  (params (DeltaSeconds :type Float%20%28single-precision%29))
  (bind _player (Variables|Default|GetPlayer))
  (Rendering|SetVisibility (Variables|/Game/Systems/Blueprints/GM1/Player/Blueprints/BP_Player_GM1.BP_Player_GM1_C|GetSphere _player) (select (Variables|/Game/Systems/Blueprints/GM1/Player/Blueprints/BP_Player_GM1.BP_Player_GM1_C|GetbIsBlocking _player) true false) false)
  (if (not (and (Variables|/Game/Systems/Blueprints/GM1/Player/Blueprints/BP_Player_GM1.BP_Player_GM1_C|GetbIsBlocking (Variables|Default|GetPlayer)) (>= (Variables|Default|GetHeldProgress) 1.0)))
    (Variables|Default|SetHeldProgress (Math|Float|Max(Float) (+ (Variables|Default|GetHeldProgress) (* (Variables|Default|GetHeldDelta) DeltaSeconds (select (Variables|/Game/Systems/Blueprints/GM1/Player/Blueprints/BP_Player_GM1.BP_Player_GM1_C|GetbIsBlocking (Variables|Default|GetPlayer)) 1.8 -3.0))) 0.0))))

(fn TrytoBlock
  (if (not (Class|KismetSystemLibrary|TimerExistsHandle (Variables|Default|GetCooldownTimerHandle)))
    (CallFunction|StartBlock)))

(fn StartBlock
  (Variables|/Game/Systems/Blueprints/GM1/Player/Blueprints/BP_Player_GM1.BP_Player_GM1_C|SetbIsBlocking (Variables|Default|GetPlayer) true)
  (Default|CallOnBlock)
  (CallFunction|PlayAbilityEffects (Variables|/Game/Systems/Blueprints/GM1/Player/Systems/Data/PDA_Block.PDA_Block_C|GetSFX (Variables|Default|GetData))))

(fn EndBlock
  (Variables|/Game/Systems/Blueprints/GM1/Player/Blueprints/BP_Player_GM1.BP_Player_GM1_C|SetbIsBlocking (Variables|Default|GetPlayer) false)
  (Default|CallOnEndBlock)
  (Utilities|Time|ClearandInvalidateTimerbyHandle (Variables|Default|GetCooldownTimerHandle))
  (Utilities|Time|ClearandInvalidateTimerbyHandle (Variables|Default|GetBlockTimer))
  (Variables|Default|SetHeldProgress 0.0))

(fn CheckCanBlock
  (bind _output_get (Variables|/Game/Systems/Blueprints/GM1/Player/Blueprints/BP_Player_GM1.BP_Player_GM1_C|SetcanBlock (Variables|Default|GetPlayer) (not (Class|KismetSystemLibrary|TimerExistsHandle (Variables|Default|GetCooldownTimerHandle)))))
  (return _output_get))

(fn UpdateBlock)