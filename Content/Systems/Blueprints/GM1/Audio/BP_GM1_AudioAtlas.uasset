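; BP_GM1_AudioAtlas is a lookup for GM1 audio that maps clip-name enum values to Sound Cues.
; GetSoundCue searches the AudioClips map for the requested clip and returns its cue, or nothing when no entry exists.
; An optional debug flag prints a green message on a hit and a red one for a clip with no cue implemented.
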(fn GetSoundCue
  (params (Clip%20name :type E_GM1_AudioClips%20Enum :default "E_GM1_AudioClips_MAX") (DebugMessage :type Boolean))
  (bind _audio_clips (Variables|Default|GetAudio%20Clips))
  (bind (_value _returnvalue) (Utilities|Map|Find _audio_clips Clip%20name))
  (LocalVariables|SetDebugMessager DebugMessage)
  (if _returnvalue
    (if (LocalVariables|GetDebugMessager)
      (Development|PrintString 0 (Utilities|String|Append "[BP GM1 Audio Atlas] Event {" (Utilities|String|EnumtoString Clip%20name) "} has accessed the associated Sound Cue") true true "(R=0.136170,G=1.000000,B=0.189297,A=1.000000)"))
    (return _value)
    (else
      (if (LocalVariables|GetDebugMessager)
        (Development|PrintString 0 (Utilities|String|Append "[BP GM1 Audio Atlas] Event {" (Utilities|String|EnumtoString Clip%20name) "} does not have a Sound Cue implemented") true true "(R=1.000000,G=0.166667,B=0.166667,A=1.000000)"))
      (return 0))))