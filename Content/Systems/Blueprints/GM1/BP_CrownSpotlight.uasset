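; BP_CrownSpotlight is an overhead spotlight that highlights the crown in the GM1 game mode.
; On BeginPlay it finds BP_Crown, then shows the light on pickup and hides it on drop.
; Tick keeps the light at a fixed height above the tracked actor, and the construction script applies intensity, color and cone angle.
; An alternative that tracks the top-scoring player exists, but its start binding is disconnected.
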(event Custom|BeginTracking
  (Rendering|SetVisibility (Variables|Default|GetSpotLight) true false))

(event Custom|ScoreChange
  (params (PlayerIndex :type Integer) (Amount :type Integer))
  (bind _spotlight (Variables|Default|GetSpotLight))
  ;[1 0 0] Point-based System. To use, hook the topmost bind event into OnBeginPlay
  ;;[0 0 0] Sets Tracked Actor When New Player Has Highest Score
  (for (_array_element _array_index) (Variables|/Game/Systems/Widgets/GM1/WBP_GM1_CrownMode.WBP_GM1_CrownMode_C|GetScoreArray (Variables|/Game/Systems/Blueprints/GM1/Systems/GM_GM1.GM_GM1_C|GetHUDWidget (.AsGM%20GM1 (Utilities|Casting|CastToGM_GM1 (Game|GetGameMode)))))
    (if (> (Variables|/Game/Systems/Widgets/GM1/WBP_GM1_PlayerScore.WBP_GM1_PlayerScore_C|GetTotal%20Score _array_element) (Variables|DEPRECATED|GetHighestScore))
      (Variables|DEPRECATED|SetHighestScore (Variables|/Game/Systems/Widgets/GM1/WBP_GM1_PlayerScore.WBP_GM1_PlayerScore_C|GetTotal%20Score _array_element))
      (Variables|DEPRECATED|SetIndexOfHighestScore _array_index)))
  (Variables|DEPRECATED|SetHighestScore 0)
  (bind _asbp_player_gm1 (Utilities|Casting|CastToBP_Player_GM1 (Pawn|GetControlledPawn (Class|GameplayStatics|GetPlayerControllerfromID (Variables|DEPRECATED|GetIndexOfHighestScore)))))
  (bind _output_get (Variables|Default|SetTrackedActor _asbp_player_gm1))
  ;;[0 0 0] Initial Setup
  (Utilities|FlowControl|DoOnce false
    (:Completed
      (Transformation|SetWorldLocation _spotlight (Math|Vector|MakeVector (.x (Transformation|GetActorLocation _output_get)) (.y (Transformation|GetActorLocation _output_get)) (+ (.z (Transformation|GetActorLocation _output_get)) 1.25e+03)) false false)
      (Rendering|SetVisibility _spotlight true false))))

(event Custom|Start%20Game
  ;[1 0 0] Point-based System. To use, hook the topmost bind event into OnBeginPlay
  (EventDispatchers|BindEventtoOnScoreChange (Variables|/Game/Systems/Blueprints/GM1/Systems/GM_GM1.GM_GM1_C|GetHUDWidget (.AsGM%20GM1 (Utilities|Casting|CastToGM_GM1 (Game|GetGameMode)))) (delegate Custom|ScoreChange)))

(event Custom|PauseTracking
  (Rendering|SetVisibility (Variables|Default|GetSpotLight) false false))

(event EventBeginPlay
  ;[0 0 0] Event Bindings
  (Rendering|SetVisibility (Variables|Default|GetSpotLight) false false)
  (bind _returnvalue (Actor|GetActorOfClass "/Game/Systems/Blueprints/GM1/BP_Crown.BP_Crown_C"))
  (Variables|Default|SetTrackedActor _returnvalue)
  (EventDispatchers|BindEventtoOnPickup _returnvalue (delegate Custom|BeginTracking))
  (EventDispatchers|BindEventtoOnDrop _returnvalue (delegate Custom|PauseTracking)))

(event Collision|EventActorBeginOverlap
  (params (OtherActor :type Actor%20Object%20Reference)))

(event EventTick
  (params (DeltaSeconds :type Float%20%28single-precision%29))
  (bind _trackedactor (Variables|Default|GetTrackedActor))
  (bind _returnvalue (Transformation|GetActorLocation _trackedactor))
  ;[0 0 0] Set Position
  (Utilities|IsValid _trackedactor
    (:Is%20Valid
      (Transformation|SetWorldLocation (Variables|Default|GetSpotLight) (Math|Vector|MakeVector (.x _returnvalue) (.y _returnvalue) (+ (.z _returnvalue) 1.25e+03)) false false))))

(fn ConstructionScript
  (bind _spotlight (Variables|Default|GetSpotLight))
  (Rendering|Components|Light|SetIntensity _spotlight (Variables|Default|GetSpotlightIntensity))
  (Rendering|Components|Light|SetLightColor _spotlight (Variables|Default|GetSpotlightColor) true)
  (Rendering|Lighting|SetOuterConeAngle _spotlight (Variables|Default|GetSpotlightOuterConeAngle)))