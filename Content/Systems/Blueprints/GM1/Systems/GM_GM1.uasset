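; Game mode for GM1, a timed multiplayer crown minigame with pregame countdown, per-player score HUD and tournament progression.
; Setup spawns and possesses a pawn per connected player on a shared camera, then starts the round after the countdown if enough players exist.
; A timer ends the game, then opens the GM2 pregame screen or results map.
; Separate functions configure meteor, bumper, shrinking-ice or random stage hazards and broadcast their start.
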(event Custom|Begin%20Round
  (CallFunction|StartGame))

(event EventBeginPlay
  (CallFunction|DoSetupGame)
  (bind _returnvalue (UserInterface|CreateWidget "/Game/Core/Programming/Prototypes/Test_Ryan/Widgets/WBP_Core_PregameCountdown.WBP_Core_PregameCountdown_C" 0 (Math|Float|Truncate (Variables|Default|GetPregameTimer))))
  (UserInterface|Viewport|AddtoViewport _returnvalue 0)
  (Utilities|FlowControl|Delay (Variables|Default|GetPregameTimer))
  (Class|KismetSystemLibrary|SetTimerforNextTickDelegate (delegate Custom|Begin%20Round)))

(event EventHandleStartingNewPlayer
  (params (NewPlayer :type Player%20Controller%20Object%20Reference))
  ;[1 1 1] Possible Work Around
  (|CallParentFunction NewPlayer)
  (Input|AddMappingContext (PlayerController|LocalPlayerSubsystems|GetEnhancedInputLocalPlayerSubsystem NewPlayer) "/Game/Systems/Blueprints/GM1/Player/Input/IMC_GM1.IMC_GM1" 0 "(bIgnoreAllPressedKeysUntilRelease=True,bForceImmediately=False)"))

(event EventOnRestartPlayer
  (params (NewPlayer :type Controller%20Object%20Reference))
  (|CallParentFunction NewPlayer))

(fn ConstructionScript)

(fn GetPlayerStartPoints
  (bind _outactors (Actor|GetAllActorsOfClass "/Game/Systems/Blueprints/GM1/Systems/BP_GM1_PlayerStart.BP_GM1_PlayerStart_C"))
  (Variables|Player|SetPlayerStarts _outactors))

(fn GameStarted
  (Variables|Player|SetisInGame true)
  (Default|GameStarted (Variables|Camera|GetCameraRef) (Variables|Player|GetPlayers))
  (bind _returnvalue (Actor|GetActorOfClass "/Game/Systems/Blueprints/GM1/BP_Crown.BP_Crown_C"))
  (bind _returnvalue_2 (UserInterface|CreateWidget "/Game/Systems/Widgets/GM1/WBP_GM1_CrownMode.WBP_GM1_CrownMode_C" 0 _returnvalue))
  (bind _output_get (Variables|Default|SetHUDWidget _returnvalue_2))
  (UserInterface|Viewport|AddtoViewport _output_get 0)
  (for _array_element (Variables|Player|GetPlayers)
    (EventDispatchers|BindEventtoOnAdjustPlayerScore _array_element (EventDispatchers|CreateEvent :!event AdjustPlayerScore)))
  (Utilities|Time|SetTimerbyFunctionName 0 "GameEnded" (Math|Conversions|ToFloat(Integer) (Variables|/Game/Systems/Blueprints/GM1/Gameplay/Data/PDA_Gameplay.PDA_Gameplay_C|GetgameDurationInSeconds (Variables|Default|GetGameplayData))))
  (Development|PrintString "GameStarted")
  (Default|IncrementNumGamesPlayed (Variables|Default|GetGame%20Instance)))

(fn GameEnded
  (Variables|Player|SetisInGame false)
  (Default|CallOnEndGame)
  (Development|PrintString "GameEnded")
  ;[1 0.6825 0.1248] Will Wait before going to next level (Sai)
  (Utilities|Time|SetTimerbyFunctionName 0 "GoToNextLevel" 3.0))

(fn RemoveUnusedCameras
  (bind _outactors (Actor|GetAllActorsOfClass "/Script/Engine.CameraActor"))
  (for _array_element _outactors
    (Actor|DestroyActor _array_element)))

(fn DoSetupGame
  ;[0 0 0 0.5] Get Camera Ref
  (bind _outactors (Actor|GetAllActorsOfClass "/Game/Systems/Blueprints/GM1/Camera/CM_GM1.CM_GM1_C"))
  (Variables|Camera|SetCameraRef (Utilities|Array|Get(acopy) _outactors))
  (CallFunction|GetPlayerStartPoints)
  ;[0 0 0 0.5] Game Instance
  (bind _asgi_core_game_instance (Utilities|Casting|CastToGI_CORE_GameInstance (Game|GetGameInstance)))
  (bind _output_get (Variables|Default|SetGame%20Instance _asgi_core_game_instance))
  (for (_ _array_index) (Variables|/Game/Core/Programming/Prototypes/GameData/GI_CORE_GameInstance.GI_CORE_GameInstance_C|GetPlayerData _output_get)
    (bind _connected (Default|GetPlayerConnected (Variables|Default|GetGame%20Instance) _array_index))
    (if _connected
      (CallFunction|SpawnPlayer _array_index (Utilities|Array|Get(acopy) (Variables|Player|GetPlayerStarts) _array_index)))
    (Game|Player|SetViewTargetwithBlend (Game|GetPlayerController _array_index) (Variables|Camera|GetCameraRef) 0.0 "VTBlend_Linear" 0.0 false))
  (return false))

(fn ShouldReset
  (params (ActorToReset :type Actor%20Object%20Reference))
  (return false))

(fn GetActivePlayers
  (bind _players (Variables|Player|GetPlayers))
  (return _players (Utilities|Array|Length _players)))

(fn SelectStageHazard
  (bind _returnvalue (Math|Transform|MakeTransform "0.000000,0.000000,25.000000"))
  (bind _output_get (Variables|Default|SetCurrentStageHazard (Variables|/Game/Systems/Blueprints/GM1/Gameplay/Data/PDA_Gameplay.PDA_Gameplay_C|GetstageHazard (Variables|Default|GetGameplayData))))
  (switch Utilities|FlowControl|Switch|SwitchonE_StageHazardType _output_get :!label _label
    (:NewEnumerator1
      (Game|SpawnActorfromClass "/Game/Systems/Blueprints/GM1/Hazards/Meteors/BP_GM1_MeteorSpawner.BP_GM1_MeteorSpawner_C" _returnvalue "Undefined" "MultiplyWithRoot" 0 (Variables|StageHazardData|GetIceMeteorData) 0))
    (:NewEnumerator2
      (Game|SpawnActorfromClass "/Game/Systems/Blueprints/GM1/Hazards/Meteors/BP_GM1_MeteorSpawner.BP_GM1_MeteorSpawner_C" _returnvalue "Undefined" "MultiplyWithRoot" 0 (Variables|StageHazardData|GetKnockbackMeteorData) 0))
    (:NewEnumerator4
      (bind _outactors (Actor|GetAllActorsOfClass "/Game/Systems/Blueprints/GM1/Hazards/BP_Bumper1.BP_Bumper1_C"))
      (for _array_element _outactors
        (Actor|DestroyActor _array_element))
      (for _array_element_2 (Variables|/Game/Systems/Blueprints/GM1/Hazards/Data/PDA_BumperHazard.PDA_BumperHazard_C|GetBumperLocations (Variables|StageHazardData|GetBumperHazardData))
        (bind _returnvalue_2 (Game|SpawnActorfromClass "/Game/Systems/Blueprints/GM1/Hazards/BP_Bumper1.BP_Bumper1_C" (Math|Conversions|ToTransform(Vector) _array_element_2) "AlwaysSpawn" "MultiplyWithRoot" 0 0 0))
        (Default|RegisterasStageHazard _returnvalue_2)))
    (:NewEnumerator5
      (bind _returnvalue_3 (Actor|GetActorOfClass "/Game/Systems/Blueprints/GM1/Hazards/BP_Arena.BP_Arena_C"))
      (Default|RegisterasStageHazard _returnvalue_3))
    (:NewEnumerator3
      ;[0 0 0] If stage hazard is set to random, get a random stage hazard and then go back through the switch to finish any set up.
      (Variables|Default|SetCurrentStageHazard (Utilities|Select :Index (Math|Random|RandomIntegerinRange 0 3) :Option%200 "NewEnumerator1" :Option%201 "NewEnumerator2" :Option%202 "NewEnumerator4" :Option%203 "NewEnumerator5"))
      (goto _label))))

(fn StartStageHazard
  (Default|CallOnStageHazardStart))

(fn AdjustPlayerScore
  (params (player :type BP%20Player%20GM1%20Object%20Reference) (amount :type Integer))
  (Default|AdjustPlayerScore (Variables|Default|GetHUDWidget) (Variables|/Game/Systems/Blueprints/GM1/Player/Blueprints/BP_Player_GM1.BP_Player_GM1_C|GetIndex player) amount))

(fn GotoNextLevel
  ;[1 0.5556 0.07462] For Tournament Mode, will go to GM2 if TournamentMode is enabled (Sai)
  (bind _canmovetonextlevel (Default|CanGotoNextTournamentLevel (Variables|Default|GetGame%20Instance)))
  (if _canmovetonextlevel
    (Game|OpenLevel(byObjectReference) "/Game/Core/Programming/Prototypes/Test_Sai/PreGameScreens/GM2_PreGameScreen.GM2_PreGameScreen")
    (else
      (Default|ClearPlayerData (Variables|Default|GetGame%20Instance))
      (Game|OpenLevel(byObjectReference) "/Game/Core/Programming/Prototypes/Test_Sai/ResultsScreenMap.ResultsScreenMap"))))

(fn FreePlayerCast
  (return 0))

(fn GetIsinGame
  (return (Variables|Player|GetisInGame)))

(fn RemovePlayer
  (params (PlayerToRemove :type BP%20Player%20GM1%20Object%20Reference))
  (Default|RemoveTrackedTarget (Variables|Camera|GetCameraRef) PlayerToRemove)
  (return false))

(fn ResetGame
  (bind _playerstarts (Variables|Player|GetPlayerStarts))
  (bind _playercontrollers (Variables|Player|GetPlayerControllers))
  (bind _players (Variables|Player|GetPlayers))
  (bind _returnvalue (Utilities|Array|Length _playerstarts))
  (bind _returnvalue_2 (Utilities|Array|Length _players))
  (bind _returnvalue_3 (Utilities|Array|Length _playercontrollers))
  (bind _result (Utilities|Text|FormatText "starts {s} 
players {p}controllers {c}" _returnvalue _returnvalue_2 _returnvalue_3))
  (Utilities|FlowControl|DoOnce false
    (:Completed
      (Development|PrintText _result)
      (Class|GameMode|RestartGame)
      (CallFunction|DoSetupGame)
      (Development|PrintText _result)
      (return true))))

(fn SpawnPlayer
  (params (CurrentPlayerIndex :type Integer) (PlayerStart :type BP%20GM1%20Player%20Start%20Object%20Reference))
  ;[0 0 0 0.5] Spawn Player Pawn and Possess
  (bind _returnvalue (Game|SpawnActorfromClass "/Game/Systems/Blueprints/GM1/Player/Blueprints/BP_Player_GM1.BP_Player_GM1_C" (Transformation|GetActorTransform PlayerStart) "Undefined" "MultiplyWithRoot" 0 CurrentPlayerIndex 0))
  (Utilities|Array|Add (Variables|Player|GetPlayers) _returnvalue)
  (Pawn|Possess (Game|GetPlayerController CurrentPlayerIndex) _returnvalue)
  (return true))

(fn StartGame
  (if (>= (Utilities|Array|Length (Variables|Player|GetPlayers)) (Variables|Player|GetMinPlayers))
    (CallFunction|GameStarted)
    (Default|CallOnStartGame)
    (return false)))