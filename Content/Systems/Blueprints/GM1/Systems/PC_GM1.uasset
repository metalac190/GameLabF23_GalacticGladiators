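; PC_GM1 is a player controller for GM1 that provides debug shortcuts for level reloading and input-device diagnostics.
; Up and D-pad Up debug keys reopen the current level by name, while D-pad Left prints the platform user ID.
; PrintInputDeviceInfo shows controller ID, primary device hardware, connection state and pawn on a keyed per-controller screen message.
; Its looping timer setup is disconnected, so that readout never starts here.
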(event Custom|ReloadLevel
  (bind _returnvalue (Game|GetCurrentLevelName true))
  (Game|OpenLevel(byName) (Utilities|String|StringToName _returnvalue)))

(event EventBeginPlay)

(event Input|GamepadEvents|DebugKeyGamepadDPadLeft
  (params (Key :type Key%20Structure) (ActionValue :type Input%20Action%20Value%20Structure))
  (:Pressed
    (Development|PrintString (Utilities|String|ToString(Integer) (Class|PlayerController|GetPlatformUserId)))))

(event Input|GamepadEvents|DebugKeyGamepadDPadUp
  (params (Key :type Key%20Structure) (ActionValue :type Input%20Action%20Value%20Structure))
  (:Pressed
    (CallFunction|ReloadLevel)))

(event Input|KeyboardEvents|DebugKeyUp
  (params (Key :type Key%20Structure) (ActionValue :type Input%20Action%20Value%20Structure))
  (:Pressed
    (CallFunction|ReloadLevel)))

(fn ConstructionScript)

(fn PrintInputDeviceInfo
  (bind _self self)
  (bind _returnvalue (Utilities|GetDisplayName _self))
  (bind _returnvalue_2 (Class|InputDeviceLibrary|GetPrimaryInputDeviceforUser (Class|PlayerController|GetPlatformUserId)))
  (if (!= _returnvalue_2 (Class|InputDeviceLibrary|InputDeviceIdNone))
    (bind _returnvalue_3 (Class|InputDeviceLibrary|GetInputDeviceConnectionState _returnvalue_2))
    (Development|PrintText (Utilities|Text|FormatText "{pc} ({id}) 
    {device} -- {status} 
    {pawn}" _returnvalue (Class|GameplayStatics|GetPlayerControllerID self) (.HardwareDeviceIdentifier (Utilities|Struct|BreakHardwareDeviceIdentifier (Class|InputDeviceSubsystem|GetInputDeviceHardwareIdentifier (|InputDeviceSubsystem) _returnvalue_2))) (Utilities|String|EnumtoString _returnvalue_3) (Utilities|GetDisplayName (Pawn|GetControlledPawn _self))) true true "(R=0.000000,G=0.660000,B=1.000000,A=1.000000)" 2.0 (Utilities|String|StringToName _returnvalue))))