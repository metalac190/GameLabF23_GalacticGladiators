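; BP_GM1_AOEZone is a meteor hazard warning zone that marks an area of effect with a decal.
; On BeginPlay a timeline scales it in to its placed size.
; While the watched meteor is visible, Tick starts warning audio and a timeline that pulses the decal color toward transparent white.
; When the meteor becomes hidden, it stops the flash and fades the decal out, destroying the actor afterward.
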(event EventBeginPlay
  ;[0 0 0] Animate Scale Intro
  (Variables|Default|SettargetSize (.X (Math|Vector|BreakVector (Transformation|GetActorScale3D))))
  (bind _scale (Timeline|SizeAnim PlayFromStart)
    (:Update
      (Transformation|SetActorScale3D (Math|Conversions|ToVector(Float) (* _scale (Variables|Default|GettargetSize)))))))

(event EventTick
  (params (DeltaSeconds :type Float%20%28single-precision%29))
  (Utilities|IsValid (Variables|Default|GetwatchMeteor)
    (:Is%20Valid
      (if (Variables|/Script/Engine.Actor|GetbHidden (Variables|Default|GetwatchMeteor))
        ;[0 0 0] Hazard was destroyed, setup Fade Out auto destroy
        (Variables|Default|SetcheckingForHazard false)
        (Rendering|Components|Decal|SetFadeOut (Variables|Default|GetAOE%20Zone%20Decal) 0.01 0.4 true)
        (Variables|Default|SetwatchMeteor 0)
        ;[0 0 0] Pulse/Flash Animation
        (bind _pulseflash (Timeline|FlashAnim Stop)
          (:Update
            (Rendering|Components|Decal|SetDecalColor (Variables|Default|GetAOE%20Zone%20Decal) (Math|Color|Lerp(LinearColor) (Variables|Default|GetorigColor) "(R=1.000000,G=1.000000,B=1.000000,A=0.000000)" _pulseflash))))
        (elif (not (Variables|Default|GetisFlashing))
          ;[0 0 0] Set Original Color
          (Variables|Default|SetorigColor (Variables|/Script/Engine.DecalComponent|GetDecalColor (Variables|Default|GetAOE%20Zone%20Decal)))
          (Variables|Default|SetisFlashing true)
          (Components|Activation|Activate (Variables|Default|GetAOE%20Warning%20Audio) false)
          (Timeline|FlashAnim PlayFromStart))))))

(fn ConstructionScript)