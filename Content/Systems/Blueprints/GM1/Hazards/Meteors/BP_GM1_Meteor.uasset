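; BP_GM1_Meteor is the meteor hazard for GM1, configured with settings and a target zone that determines its blast radius.
; On overlapping the arena it stops, plays impact audio and hides, destroying itself once the sound ends.
; Impact uses a sphere overlap as a custom radial force with optional horizontal-only impulse, knocking back players and static mesh actors.
; Hit players also drop the crown and get stunned.
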(event Collision|EventActorBeginOverlap
  (params (OtherActor :type Actor%20Object%20Reference))
  (bind _hazard_impact_audio (Variables|Default|GetHazard%20Impact%20Audio))
  (Utilities|Casting|CastToBP_Arena OtherActor)
  (Physics|SetPhysicsLinearVelocity (Variables|Default|GetSphereCol) "0, 0, 0" false "None")
  (CallFunction|Impact)
  ;[0 0 0] Hide the meteor, then destroy it once the impact SFX have stopped playing
  (Audio|Components|Audio|Stop (Variables|Default|GetHazard%20Fall%20Audio))
  (Audio|Components|Audio|Play _hazard_impact_audio 0.0)
  (Rendering|SetActorHiddenInGame true)
  (Utilities|FlowControl|Delay 0.5 :!label _label)
  (if (Audio|Components|Audio|IsPlaying _hazard_impact_audio)
    (goto _label)
    (else
      (Actor|DestroyActor))))

(fn ConstructionScript)

(fn Impact
  (bind _returnvalue (Transformation|GetActorLocation))
  ;[0 0 0] Knock back each actor in the radius of effect. Effectively apes a RadialForceComponent except that we can fix the impulse to the horizontal.
  (bind _outactors (Collision|SphereOverlapActors _returnvalue (Variables|Default|GetRadius) (Variables|Default|GetAffect%20Channels) 0))
  (for _array_element _outactors
    (bind _asbp_player_gm1 (Utilities|Casting|CastToBP_Player_GM1 _array_element)
      (:then
        (Default|AddImpulse _asbp_player_gm1 (* (Math|Vector|SelectVector (Class|KismetMathLibrary|VectorNormal2D (- (Transformation|GetActorLocation _array_element) _returnvalue) 0.0001) (Math|Vector|Normalize (- (Transformation|GetActorLocation _array_element) _returnvalue)) (Variables|/Game/Systems/Blueprints/GM1/Hazards/Meteors/Data/PDA_Meteor.PDA_Meteor_C|GetHorizontal%20Impulse%20Only (Variables|Default|GetSettings))) (Utilities|GetMeteorForcefromSize (Variables|Default|GetRadius))) false)
        (Default|DropCrown _asbp_player_gm1 self)
        (Default|ApplyStun _asbp_player_gm1 (Variables|/Game/Systems/Blueprints/GM1/Hazards/Meteors/Data/PDA_Meteor.PDA_Meteor_C|GetStun%20Time (Variables|Default|GetSettings))))
      (:CastFailed
        (bind _asstatic_mesh_actor (Utilities|Casting|CastToStaticMeshActor _array_element))
        (Physics|AddImpulse (Variables|/Script/Engine.StaticMeshActor|GetStaticMeshComponent _asstatic_mesh_actor) (* (Math|Vector|SelectVector (Class|KismetMathLibrary|VectorNormal2D (- (Transformation|GetActorLocation _array_element) _returnvalue) 0.0001) (Math|Vector|Normalize (- (Transformation|GetActorLocation _array_element) _returnvalue)) (Variables|/Game/Systems/Blueprints/GM1/Hazards/Meteors/Data/PDA_Meteor.PDA_Meteor_C|GetHorizontal%20Impulse%20Only (Variables|Default|GetSettings))) (Utilities|GetMeteorForcefromSize (Variables|Default|GetRadius))) "None" false)))))

(fn ApplyMeteorSettings
  (params (settings :type PDA%20Meteor%20Object%20Reference) (targetZone :type BP%20GM1%20AOE%20Zone%20Object%20Reference))
  (Variables|Default|SetSettings settings)
  (Variables|Default|Settarget targetZone)
  (Variables|Default|SetRadius (* (Variables|/Game/Systems/Blueprints/GM1/Hazards/Meteors/BP_GM1_AOEZone.BP_GM1_AOEZone_C|GettargetSize targetZone) 5e+01)))