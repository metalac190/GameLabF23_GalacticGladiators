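; BP_IceMeteor is a meteor hazard variant that leaves an ice patch on the arena when it hits.
; Its Impact override runs the parent logic, then spawns BP_IcePatch at the meteor's location, scaled by Radius.
; It converts the spawn transform into BP_Arena's space and attaches the patch with relative rules, then pins it to a fixed local height with random yaw.
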(event EventBeginPlay
  (|CallParentFunction) ; This node is disabled and will not be called.\nDrag off pins to build functionality.
)

(event Collision|EventActorBeginOverlap
  (params (OtherActor :type Actor%20Object%20Reference))
  (|CallParentFunction OtherActor) ; This node is disabled and will not be called.\nDrag off pins to build functionality.
)

(event EventTick
  (params (DeltaSeconds :type Float%20%28single-precision%29))
  (|CallParentFunction DeltaSeconds) ; This node is disabled and will not be called.\nDrag off pins to build functionality.
)

(fn ConstructionScript
  (|CallParentFunction))

(fn Impact
  (|CallParentFunction)
  ;[0 0 0] Spawn an ice patch at the meteor's transform, making sure it is parented to the arena floor correctly
  (bind _returnvalue (Actor|GetActorOfClass "/Game/Systems/Blueprints/GM1/Hazards/BP_Arena.BP_Arena_C"))
  (bind _returnvalue_2 (Game|SpawnActorfromClass "/Game/Systems/Blueprints/GM1/Hazards/BP_IcePatch.BP_IcePatch_C" (Math|Transform|MakeRelativeTransform (Math|Transform|MakeTransform (Transformation|GetActorLocation) "0, 0, 0" (Math|Conversions|ToVector(Float) (/ (Variables|Default|GetRadius) 5e+01))) (Transformation|GetActorTransform _returnvalue)) "Undefined" "MultiplyWithRoot" 0 0))
  (Transformation|AttachActorToActor _returnvalue_2 _returnvalue "None" "KeepRelative" "KeepRelative" "KeepRelative" true)
  (Transformation|SetRelativeLocationAndRotation (Variables|/Game/Systems/Blueprints/GM1/Hazards/BP_IcePatch.BP_IcePatch_C|GetDefaultSceneRoot _returnvalue_2) (Math|Vector|MakeVector (.x (Variables|/Script/Engine.SceneComponent|GetRelativeLocation (Variables|/Game/Systems/Blueprints/GM1/Hazards/BP_IcePatch.BP_IcePatch_C|GetDefaultSceneRoot _returnvalue_2))) (.y (Variables|/Script/Engine.SceneComponent|GetRelativeLocation (Variables|/Game/Systems/Blueprints/GM1/Hazards/BP_IcePatch.BP_IcePatch_C|GetDefaultSceneRoot _returnvalue_2))) 46.0) (Math|Rotator|MakeRotator 0.0 0.0 (Math|Random|RandomFloatinRange 0.0 3.6e+02)) false false))